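; Mordhau Dogpit deathmatch game mode that runs first-to-N duels in numbered rooms.
; Kills increment the killer's score in their room, with a room-ID queue and delay blocking repeat counts.
; Matches reaching their limit are broadcast, announced and removed, and room changes are pushed through the custom GameState.
; On login, admins and PlayFab IDs in the Refs list, loadable from custom config, are flagged as referees.
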(event `self.OnKilled`
  (params (Killer :type "Controller Object Reference") (KilledPlayer :type "Controller Object Reference") (KilledPawn :type "Pawn Object Reference") (Type :type "EMordhauDamageType Enum" :default "Generic") (SubType :type Byte) (DamageSource :type "Actor Object Reference") (DamageAgent :type "Actor Object Reference"))
  (bind _inque (`self.InQue`))
  (`parent.OnKilled` Killer KilledPlayer KilledPawn Type SubType DamageSource DamageAgent)
  (bind _asbp_mordhau_player_controller_dogpit (cast `/CustomMenus/BP_MordhauPlayerController_Dogpit` Killer))
  (bind _currentroomid (`/CustomMenus/BP_MordhauPlayerController_Dogpit.CurrentRoomID` _asbp_mordhau_player_controller_dogpit))
  (if (== (`KismetArrayLibrary.Array_Find` _inque _currentroomid) -1)
    (bind _returnvalue (`KismetArrayLibrary.Array_AddUnique` _inque _currentroomid))
    (bind _done (`self.GetTrackedFight_THIRDATTEMPT` _asbp_mordhau_player_controller_dogpit))
    (if _done
      (`KismetSystemLibrary.Delay` 6.0)
      (`KismetArrayLibrary.Array_Remove` _inque _returnvalue))))

(event `self.K2_PostLogin`
  (params (NewPlayer :type "PlayerController Object Reference"))
  (`parent.K2_PostLogin` NewPlayer)
  (`self.OnPostLogin` NewPlayer))

(fn `AddFT10`
  (params (RoomID :type String) (Controllers :type "Array of /CustomMenus/BP_MordhauPlayerController_Dogpit Object Reference") (ScoreLimit :type Integer))
  (bind _roomsnew (`self.RoomsNEW`))
  (`KismetArrayLibrary.Array_AddUnique` _roomsnew (make `/CustomMenus/FT10/STRUCT_FT10_Room` Controllers (`|MakeArray` 0 0) "NewEnumerator0" RoomID ScoreLimit))
  (set `self.RoomsNEW` _roomsnew)
  (`self.UpdateRooms`))

(fn `AnnounceResults`
  (params (Results :type Text))
  (bind _asbp_deathmatch_game_state_custom (cast `/CustomMenus/BP_DeathmatchGameStateCustom` (`GameplayStatics.GetGameState`)))
  (`/CustomMenus/BP_DeathmatchGameStateCustom.DisplayAnnouncments` _asbp_deathmatch_game_state_custom (`KismetTextLibrary.Conv_TextToString` Results)))

(fn `AnnounceRoomScore`
  (params (Subtext :type String))
  (for _array_element (`self.RoomsNEW`)
    (bind (_players _scores _state _roomid) (break `/CustomMenus/FT10/STRUCT_FT10_Room` _array_element))
    (if (`KismetStringLibrary.EqualEqual_StrStr` _roomid Subtext)
      (bind _asbp_deathmatch_game_state_custom (cast `/CustomMenus/BP_DeathmatchGameStateCustom` (`GameplayStatics.GetGameState`)))
      (`/CustomMenus/BP_DeathmatchGameStateCustom.DisplayAnnouncments` _asbp_deathmatch_game_state_custom (`KismetTextLibrary.Conv_TextToString` (`|FormatText` "{Player1} {Score1} - {Score2} {Player2} " (`PlayerState.GetPlayerName` (`Controller.PlayerState` (`|GetArrayItem` _players))) (`|GetArrayItem` _scores) (`|GetArrayItem` _scores 1) (`PlayerState.GetPlayerName` (`Controller.PlayerState` (`|GetArrayItem` _players 1)))))))))

(fn `Debug`
  (params (NewParam :type String))
  (`self.Broadcast` self NewParam "ServerSay"))

(fn `GetConfig`
  (bind (_arraysize _returnvalue) (`MordhauUtilityLibrary.GetCustomConfigVar_Array` "dogpit" "Refs"))
  (if (> _arraysize 0)
    (set `self.Refs` _returnvalue)))

(fn `GetNewRoomID`
  (returns (ReturnValue :type Integer))
  (return (+ (`KismetArrayLibrary.Array_Length` (`self.RoomsNEW`)) 1)))

(fn `GetTrackedFight_THIRDATTEMPT`
  (params (Killer :type "/CustomMenus/BP_MordhauPlayerController_Dogpit Object Reference"))
  (returns (Done :type Boolean))
  (locals (NewLocalVar_1 :type "Array of Integer"))
  (bind _roomsnew (`self.RoomsNEW`))
  (for (_array_element _array_index) _roomsnew
    (bind (_players _scores _state _roomid _scorelimit) (break `/CustomMenus/FT10/STRUCT_FT10_Room` _array_element))
    (if (`KismetStringLibrary.EqualEqual_StrStr` _roomid (`/CustomMenus/BP_MordhauPlayerController_Dogpit.CurrentRoomID` Killer))
      (bind _returnvalue (`KismetArrayLibrary.Array_Find` _players Killer))
      (if (not (== _returnvalue -1))
        (bind _output_get (set `local.NewLocalVar_1` _scores))
        (bind _returnvalue_2 (+ (`|GetArrayItem` _output_get _returnvalue) 1))
        (if (>= _returnvalue_2 _scorelimit)
          (bind _returnvalue_3 (`KismetMathLibrary.SelectInt` 0 1 (== _returnvalue 1)))
          (bind _result (`|FormatText` "{Winner} has defeated {loser} in a match. {Score1} to {Score2}" (`PlayerState.GetPlayerName` (`Controller.PlayerState` (`|GetArrayItem` _players _returnvalue))) (`PlayerState.GetPlayerName` (`Controller.PlayerState` (`|GetArrayItem` _players _returnvalue_3))) _returnvalue_2 (`|GetArrayItem` _output_get _returnvalue_3)))
          (`self.Broadcast` self (`KismetTextLibrary.Conv_TextToString` _result) "ServerSay")
          (`self.AnnounceResults` _result)
          (`KismetArrayLibrary.Array_RemoveItem` _roomsnew _array_element)
          (else
            (`KismetArrayLibrary.Array_Set` _output_get _returnvalue _returnvalue_2)
            (`KismetArrayLibrary.Array_Set` _roomsnew _array_index (make `/CustomMenus/FT10/STRUCT_FT10_Room` _players (`local.NewLocalVar_1`) _state _roomid _scorelimit))))
        (set `self.RoomsNEW` _roomsnew)
        (`self.UpdateRooms`)
        (return true))))
  (return true))

(fn `OnPostLogin`
  (params (Controller :type "Controller Object Reference"))
  (bind _asbp_mordhau_player_controller_dogpit (cast `/CustomMenus/BP_MordhauPlayerController_Dogpit` Controller))
  (if (`MordhauPlayerController.IsAdmin` _asbp_mordhau_player_controller_dogpit)
    (set `/CustomMenus/BP_MordhauPlayerController_Dogpit.IsRef` true _asbp_mordhau_player_controller_dogpit)
    (elif (not (== (`KismetArrayLibrary.Array_Find` (`self.Refs`) (`MordhauPlayerController.GetPlayFabID` _asbp_mordhau_player_controller_dogpit)) -1))
      (set `/CustomMenus/BP_MordhauPlayerController_Dogpit.IsRef` true _asbp_mordhau_player_controller_dogpit))))

(fn `UpdateRooms`
  (bind _asbp_deathmatch_game_state_custom (cast `/CustomMenus/BP_DeathmatchGameStateCustom` (`GameplayStatics.GetGameState`)))
  (`/CustomMenus/BP_DeathmatchGameStateCustom.OnStructsUpdated` _asbp_deathmatch_game_state_custom)
  (`self.ForceNetUpdate` _asbp_deathmatch_game_state_custom))

(fn `UserConstructionScript`
  (`parent.UserConstructionScript`))