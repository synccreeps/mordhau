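; Custom deathmatch game state for the Dogpit mode, publishing first-to-score duel room standings and driving interactable button visuals.
; OnStructsUpdated rebuilds FT10s from the game mode's rooms with names and scores; its OnRep refreshes the Dogpit menu if visible.
; Cosmetic Tick updates Buttons round-robin, three per frame, to spread the cost.
; DisplayAnnouncments relays announcements to every Dogpit player controller.
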(event `self.ReceiveTick`
  (params (DeltaSeconds :type "Float (single-precision)"))
  (`parent.ReceiveTick` DeltaSeconds)
  (`/Engine/EditorBlueprintResources/StandardMacros.Can Execute Cosmetic Events`
    (:`True`
      (if (> (`KismetArrayLibrary.Array_Length` (`self.Buttons`)) 0)
        (for _ (range 1 4)
          (`self.UpdateVisuals`))))))

(event `DisplayAnnouncments`
  (params (NewParam :type String))
  (bind _outactors (`GameplayStatics.GetAllActorsOfClass` "/CustomMenus/BP_MordhauPlayerController_Dogpit.BP_MordhauPlayerController_Dogpit_C"))
  (for _array_element _outactors
    (`/CustomMenus/BP_MordhauPlayerController_Dogpit.Client_DisplayAnnouncement` _array_element NewParam)))

(fn `OnRep_FT10s`
  (bind _asbp_mordhau_hud_dogpit (cast `/CustomMenus/BP_MordhauHUD_dogpit` (`MordhauUtilityLibrary.GetMordhauHUD`)))
  (bind _dogpitmenu (`/CustomMenus/BP_MordhauHUD_dogpit.Dogpitmenu` _asbp_mordhau_hud_dogpit))
  (if (`Widget.IsVisible` _dogpitmenu)
    (`/CustomMenus/FT10/BP_AdminMenuWidget.CreateEntries` _dogpitmenu)))

(fn `OnStructsUpdated`
  (bind _ft10s (`self.FT10s`))
  (`KismetArrayLibrary.Array_Clear` (`self.FT10s`))
  (bind _asbp_deathmatch_game_mode_custom (cast `/CustomMenus/BP_DeathmatchGameModeCustom` (`GameplayStatics.GetGameMode`)))
  (for _array_element (`/CustomMenus/BP_DeathmatchGameModeCustom.RoomsNEW` _asbp_deathmatch_game_mode_custom)
    (bind (_players _scores _state _roomid _scorelimit) (break `/CustomMenus/FT10/STRUCT_FT10_Room` _array_element))
    (`KismetArrayLibrary.Array_AddUnique` _ft10s (make `/CustomMenus/FT10/STRUCT_Ft10` (`KismetTextLibrary.Conv_StringToText` (`PlayerState.GetPlayerName` (`Controller.PlayerState` (`|GetArrayItem` _players)))) (`KismetTextLibrary.Conv_StringToText` (`PlayerState.GetPlayerName` (`Controller.PlayerState` (`|GetArrayItem` _players 1)))) (`|GetArrayItem` _scores) (`|GetArrayItem` _scores 1) _roomid _scorelimit)))
  (set `self.FT10s` _ft10s))

(fn `UpdateVisuals`
  (bind _buttons (`self.Buttons`))
  (bind _buttonindex (`self.ButtonIndex`))
  (bind _output (`|GetArrayItem` _buttons _buttonindex))
  (`|ExecutionSequence`
    (:`then_0`
      (if (not (`KismetArrayLibrary.Array_IsValidIndex` _buttons _buttonindex))
        (set `self.ButtonIndex` 0)))
    (:`then_1`
      (`/Engine/EditorBlueprintResources/StandardMacros.IsValid` _output
        (:`Is Valid`
          (bind _asbp_base_interactable_actor (cast `/CustomMenus/CustomInteract/BP_BaseInteractableActor` _output))
          (`/CustomMenus/CustomInteract/BP_BaseInteractableActor.UpdateVisuals` _asbp_base_interactable_actor))))
    (:`then_2`
      (set `self.ButtonIndex` (+ (`self.ButtonIndex`) 1)))))

(fn `UserConstructionScript`
  (`parent.UserConstructionScript`))