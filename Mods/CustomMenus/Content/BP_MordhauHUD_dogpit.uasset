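; BP_MordhauHUD_dogpit is a Mordhau HUD Blueprint that adds an admin menu widget for Dogpit.
; When the game state replicates, it constructs BP_AdminMenuWidget on the first player controller, adds it to the viewport and leaves it collapsed.
; ShowMenuWidget reveals the widget through its Show function, and opening the main menu collapses it again after running the parent behavior.
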(event `self.OnGameStateReplicated`
  (`parent.OnGameStateReplicated`)
  (`self.CreateMenuWidget`))

(event `self.HideMainMenu`
  (`parent.HideMainMenu`))

(event `self.Show Main Menu`
  (bind _dogpitmenu (`self.Dogpitmenu`))
  (`parent.Show Main Menu`)
  (`/Engine/EditorBlueprintResources/StandardMacros.IsValid` _dogpitmenu
    (:`Is Valid`
      (`Widget.SetVisibility` _dogpitmenu "Collapsed"))))

(fn `CreateMenuWidget`
  (bind _returnvalue (`GameplayStatics.GetPlayerController` 0))
  (`/Engine/EditorBlueprintResources/StandardMacros.IsValid` _returnvalue
    (:`Is Valid`
      (bind _returnvalue_2 (`|GenericCreateObject` "/CustomMenus/FT10/BP_AdminMenuWidget.BP_AdminMenuWidget_C" _returnvalue))
      (bind _output_get (set `self.Dogpitmenu` _returnvalue_2))
      (`UserWidget.AddToViewport` _output_get 2)
      (`Widget.SetVisibility` _output_get "Collapsed"))))

(fn `ShowMenuWidget`
  (`/CustomMenus/FT10/BP_AdminMenuWidget.Show` (`self.Dogpitmenu`)))

(fn `UserConstructionScript`
  (`parent.UserConstructionScript`))