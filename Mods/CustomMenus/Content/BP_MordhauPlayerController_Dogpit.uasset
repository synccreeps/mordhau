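; Mordhau player controller for the Dogpit mode, letting admins and referees run FT10 score-limited matches between two players.
; Gated events find players by name and add, remove, reset, rescore or announce rooms held in the custom deathmatch game mode.
; It registers an F3 input mapping at runtime to open the HUD menu, whose options come from a player-name array via OnRep.
; It also displays announcements and runs console commands.
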(event `AddFT10`
  (params (Player1 :type Text) (Player2 :type Text) (ScoreLimit :type Integer))
  (bind _returnvalue (`KismetStringLibrary.Conv_IntToString` (`self.NewVar_1`)))
  (`self.SwitchIsRef`
    (:`true`
      (bind (_player_controller _found) (`self.FindPlayer` Player1))
      (if _found
        (bind (_player_controller_2 _found_2) (`self.FindPlayer` Player2))
        (if _found_2
          (bind _asbp_deathmatch_game_mode_custom (cast `/CustomMenus/BP_DeathmatchGameModeCustom` (`GameplayStatics.GetGameMode`)))
          (set `self.NewVar_1` (`/CustomMenus/BP_DeathmatchGameModeCustom.GetNewRoomID` _asbp_deathmatch_game_mode_custom))
          (`/CustomMenus/BP_DeathmatchGameModeCustom.AddFT10` _asbp_deathmatch_game_mode_custom _returnvalue (`|MakeArray` _player_controller _player_controller_2) ScoreLimit)
          (set `/Game/BP_MordhauPlayerController_Dogpit.CurrentRoomID` _returnvalue _player_controller_2)
          (set `/Game/BP_MordhauPlayerController_Dogpit.CurrentRoomID` _returnvalue _player_controller))))))

(event `RemoveFT10`
  (params (RoomID :type String))
  (`self.SwitchIsRef`
    (:`true`
      (bind _asbp_deathmatch_game_mode_custom (cast `/CustomMenus/BP_DeathmatchGameModeCustom` (`GameplayStatics.GetGameMode`)))
      (bind _roomsnew (`/CustomMenus/BP_DeathmatchGameModeCustom.RoomsNEW` _asbp_deathmatch_game_mode_custom))
      (for (_array_element _array_index) _roomsnew
        (if (`KismetStringLibrary.EqualEqual_StrStr` (`.RoomID_16_3892361E43D01FCA8274D7B3F9039A17` (break `/CustomMenus/FT10/STRUCT_FT10_Room` _array_element)) RoomID)
          (`KismetArrayLibrary.Array_Remove` _roomsnew _array_index)
          (set `/CustomMenus/BP_DeathmatchGameModeCustom.RoomsNEW` _roomsnew _asbp_deathmatch_game_mode_custom)
          (`/CustomMenus/BP_DeathmatchGameModeCustom.UpdateRooms` _asbp_deathmatch_game_mode_custom))))))

(event `ResetFT10`
  (params (RoomID :type String))
  (`self.SwitchIsRef`
    (:`true`
      (bind _asbp_deathmatch_game_mode_custom (cast `/CustomMenus/BP_DeathmatchGameModeCustom` (`GameplayStatics.GetGameMode`)))
      (bind _roomsnew (`/CustomMenus/BP_DeathmatchGameModeCustom.RoomsNEW` _asbp_deathmatch_game_mode_custom))
      (for (_array_element _array_index) _roomsnew
        (bind (_players _scores _state _roomid _scorelimit) (break `/CustomMenus/FT10/STRUCT_FT10_Room` _array_element))
        (if (`KismetStringLibrary.EqualEqual_StrStr` _roomid RoomID)
          (`KismetArrayLibrary.Array_Set` _roomsnew _array_index (make `/CustomMenus/FT10/STRUCT_FT10_Room` _players (`|MakeArray` 0 0) _state _roomid _scorelimit))
          (set `/CustomMenus/BP_DeathmatchGameModeCustom.RoomsNEW` _roomsnew _asbp_deathmatch_game_mode_custom)
          (`/CustomMenus/BP_DeathmatchGameModeCustom.UpdateRooms` _asbp_deathmatch_game_mode_custom))))))

(event `self.ReceiveBeginPlay`
  (`parent.ReceiveBeginPlay`)
  (`KismetSystemLibrary.Delay` 1.0)
  (`/Engine/EditorBlueprintResources/StandardMacros.IsValid` (`MordhauUtilityLibrary.GetMordhauInput`) :!label _label
    (:`Is Valid`
      (`self.AddMordhauInput` (make `InputActionKeyMapping` "Dogpit Menu" false false false false "F3")))
    (:`Is Not Valid`
      (`KismetSystemLibrary.Delay` 1.0)
      (goto _label))))

(event `ModifyScore`
  (params (RoomID :type String) (Scores :type "Array of Integer"))
  (`self.SwitchIsRef`
    (:`true`
      (bind _asbp_deathmatch_game_mode_custom (cast `/CustomMenus/BP_DeathmatchGameModeCustom` (`GameplayStatics.GetGameMode`)))
      (bind _roomsnew (`/CustomMenus/BP_DeathmatchGameModeCustom.RoomsNEW` _asbp_deathmatch_game_mode_custom))
      (for (_array_element _array_index) _roomsnew
        (bind (_players _scores _state _roomid _scorelimit) (break `/CustomMenus/FT10/STRUCT_FT10_Room` _array_element))
        (if (`KismetStringLibrary.EqualEqual_StrStr` _roomid RoomID)
          (`KismetArrayLibrary.Array_Set` _roomsnew _array_index (make `/CustomMenus/FT10/STRUCT_FT10_Room` _players Scores _state _roomid _scorelimit))
          (set `/CustomMenus/BP_DeathmatchGameModeCustom.RoomsNEW` _roomsnew _asbp_deathmatch_game_mode_custom)
          (`/CustomMenus/BP_DeathmatchGameModeCustom.UpdateRooms` _asbp_deathmatch_game_mode_custom))))))

(event `AnnounceScores`
  (params (RoomID :type String))
  (`self.SwitchIsRef`
    (:`true`
      (bind _asbp_deathmatch_game_mode_custom (cast `/CustomMenus/BP_DeathmatchGameModeCustom` (`GameplayStatics.GetGameMode`)))
      (`/CustomMenus/BP_DeathmatchGameModeCustom.AnnounceRoomScore` _asbp_deathmatch_game_mode_custom RoomID))))

(event `InputAction|Dogpit Menu`
  (params (Key :type "Key Structure"))
  (:`Pressed`
    (`self.SwitchIsRef`
      (:`true`
        (`self.GetPlayers`)
        (bind _asbp_mordhau_hud_dogpit (cast `/CustomMenus/BP_MordhauHUD_dogpit` (`self.GetHUD`)))
        (`/CustomMenus/BP_MordhauHUD_dogpit.ShowMenuWidget` _asbp_mordhau_hud_dogpit)))))

(event `Client_DisplayAnnouncement`
  (params (NewParam :type String))
  (`self.DisplayAnnouncement` "Announcement" NewParam 6.0))

(event `PleaseWork`
  (params (NewParam :type String))
  (`KismetSystemLibrary.ExecuteConsoleCommand` NewParam self))

(fn `AddMordhauInput`
  (params (`Input Action` :type "InputActionKeyMapping Structure"))
  (returns (Success :type Boolean))
  (locals (AlreadyExists :type Boolean))
  (bind _returnvalue (`MordhauUtilityLibrary.GetMordhauInput`))
  (bind _actionmappings (`MordhauInput.ActionMappings` _returnvalue))
  ;[1 1 1] NOTE: You need to make Input action inside Unreal Project settings to be able to get the event for this input action
  (for (_array_element _array_index) _actionmappings
    (bind (_actionname _bshift _bctrl _balt _bcmd _key) (break `InputActionKeyMapping` _array_element))
    (if (== _actionname (`.ActionName` (break `InputActionKeyMapping` `Input Action`)))
      (if (== _key "None")
        (`KismetArrayLibrary.Array_Set` _actionmappings _array_index `Input Action`)
        (`MordhauInput.SaveSettings` _returnvalue :!label _label)
        (`MordhauInput.ApplySettings` _returnvalue)
        (return true)
        (else
          (set `local.AlreadyExists` true)
          (break)))))
  (if (`local.AlreadyExists`)
    (return false)
    (else
      (`KismetArrayLibrary.Array_Add` _actionmappings `Input Action`)
      (goto _label))))

(fn `ExecuteCommand`
  (params (Command :type String))
  (`self.PleaseWork` Command))

(fn `FindPlayer`
  (params (`Player Name` :type Text))
  (returns (`Player Controller` :type "/Game/BP_MordhauPlayerController_Dogpit Object Reference") (Found :type Boolean))
  (locals (NewLocalVar_1 :type "/Game/BP_MordhauPlayerController_Dogpit Object Reference"))
  (bind _returnvalue (`KismetTextLibrary.Conv_TextToString` `Player Name`))
  (bind _newlocalvar_1 (`local.NewLocalVar_1`))
  (bind _asbp_deathmatch_game_state_custom (cast `/CustomMenus/BP_DeathmatchGameStateCustom` (`GameplayStatics.GetGameState`)))
  (for _array_element (`GameStateBase.PlayerArray` _asbp_deathmatch_game_state_custom)
    (bind _returnvalue_2 (`PlayerState.GetPlayerName` _array_element))
    (if (or (`KismetStringLibrary.Contains` _returnvalue_2 _returnvalue) (`KismetStringLibrary.EqualEqual_StrStr` _returnvalue_2 _returnvalue))
      (bind _asbp_mordhau_player_controller_dogpit (cast `/Game/BP_MordhauPlayerController_Dogpit` (`self.GetOwner` _array_element)))
      (set `local.NewLocalVar_1` _asbp_mordhau_player_controller_dogpit)
      (break)))
  (return _newlocalvar_1 (not (== _newlocalvar_1 null))))

(fn `GetPlayers`
  (bind _target_array (`self.Target Array`))
  (bind _asbp_deathmatch_game_state_custom (cast `/CustomMenus/BP_DeathmatchGameStateCustom` (`GameplayStatics.GetGameState`)))
  (for (_array_element _array_index) (`GameStateBase.PlayerArray` _asbp_deathmatch_game_state_custom)
    (`/Engine/EditorBlueprintResources/StandardMacros.IsValid` _array_element
      (:`Is Valid`
        (`KismetArrayLibrary.Array_Set` _target_array _array_index (`PlayerState.GetPlayerName` _array_element) true))))
  (set `self.Target Array` _target_array))

(fn `NewFunction_0`)

(fn `OnRep_CurrentRoomID`)

(fn `OnRep_IsCurrentlyInFT10`)

(fn `OnRep_IsRef`)

(fn `OnRep_Target Array`
  (`self.TargetArray`))

(fn `TargetArray`
  (bind _asbp_mordhau_hud_dogpit (cast `/CustomMenus/BP_MordhauHUD_dogpit` (`self.GetHUD`)))
  (bind _dogpitmenu (`/CustomMenus/BP_MordhauHUD_dogpit.Dogpitmenu` _asbp_mordhau_hud_dogpit))
  (bind _options (`/CustomMenus/FT10/BP_AdminMenuWidget.Options` _dogpitmenu))
  (`KismetArrayLibrary.Array_Clear` _options)
  (for _array_element (`self.Target Array`)
    (`KismetArrayLibrary.Array_AddUnique` _options (`KismetTextLibrary.Conv_StringToText` _array_element)))
  (set `/CustomMenus/FT10/BP_AdminMenuWidget.Options` _options _dogpitmenu))

(fn `UserConstructionScript`
  (`parent.UserConstructionScript`))