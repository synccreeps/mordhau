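; Base interactable button for Mordhau that, by type, teleports the user, gives equipment, runs console commands or calls an overridable CustomFunction.
; Interaction starts a cooldown that Tick counts down and CanInteract checks.
; Spawned items take the player's saved customization, falling back to random, and are equipped if pickup succeeds.
; It registers with the deathmatch game state; UpdateVisuals lazily creates its display, tracks availability and distance-culls the widget with hysteresis.
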(event `self.ReceiveBeginPlay`
  (`parent.ReceiveBeginPlay`)
  (`/Engine/EditorBlueprintResources/StandardMacros.Can Execute Cosmetic Events`
    (:`True`
      (bind _asbp_deathmatch_game_state_custom (cast `/CustomMenus/BP_DeathmatchGameStateCustom` (`GameplayStatics.GetGameState`)))
      (`KismetArrayLibrary.Array_AddUnique` (`/CustomMenus/BP_DeathmatchGameStateCustom.Buttons` _asbp_deathmatch_game_state_custom) self))))

(event `self.OnInteractionStart`
  (params (Character :type "MordhauCharacter Object Reference"))
  (bind _asbp_mordhau_character (cast `/Game/Mordhau/Blueprints/Characters/BP_MordhauCharacter` Character))
  (bind _asbp_mordhau_player_controller_dogpit (cast `/CustomMenus/BP_MordhauPlayerController_Dogpit` (`AdvancedCharacter.GetControllerIncludingVehicle` _asbp_mordhau_character)))
  (set `self.CooldownRemaining` (`self.Cooldown`))
  (switch `/CustomMenus/FT10/ENUM_ButtonType` (`self.ButtonType`)
    (:`NewEnumerator0`
      (`self.K2_TeleportTo` :`self` _asbp_mordhau_character :`DestLocation` (`self.Teleport Location`)))
    (:`NewEnumerator1`
      (`self.SpawnItem` _asbp_mordhau_character))
    (:`NewEnumerator2`
      (for _array_element (`self.ConsoleCommands`)
        (`/CustomMenus/BP_MordhauPlayerController_Dogpit.ExecuteCommand` _asbp_mordhau_player_controller_dogpit _array_element)))
    (:`NewEnumerator3`
      (`self.CustomFunction` _asbp_mordhau_character _asbp_mordhau_player_controller_dogpit))))

(event `self.ReceiveTick`
  (params (DeltaSeconds :type "Float (single-precision)"))
  (bind _cooldownremaining (`self.CooldownRemaining`))
  (if (> _cooldownremaining 0.0)
    (set `self.CooldownRemaining` (- _cooldownremaining DeltaSeconds))))

(fn `CanInteract`
  (params (Character :type "MordhauCharacter Object Reference"))
  (returns (ReturnValue :type Boolean))
  (`/Engine/EditorBlueprintResources/StandardMacros.IsValid` Character
    (:`Is Valid`
      (if (> (`self.CooldownRemaining`) 0.0)
        _
        (else
          (return true))))
    (:`Is Not Valid`
      _))
  (return false))

(fn `CustomFunction`
  (params (Character :type "/Game/Mordhau/Blueprints/Characters/BP_MordhauCharacter Object Reference") (Controller :type "/Game/Mordhau/Blueprints/BP_MordhauPlayerController Object Reference")))

(fn `InitializeDisplay`
  (bind _skeletalmesh (`self.SkeletalMesh`))
  (bind _static_mesh (`self.Static Mesh`))
  (`|ExecutionSequence`
    (:`then_0`
      (`/Engine/EditorBlueprintResources/StandardMacros.IsValid` _skeletalmesh
        (:`Is Valid`
          (`SkinnedMeshComponent.SetSkinnedAssetAndUpdate` (`self.LODSkeletalMesh`) _skeletalmesh true))
        (:`Is Not Valid`
          (`/Engine/EditorBlueprintResources/StandardMacros.IsValid` _static_mesh
            (:`Is Valid`
              (`StaticMeshComponent.SetStaticMesh` (`self.StaticMesh`) _static_mesh))))))
    (:`then_1`
      (bind _returnvalue (`AddComponent|NODE_AddMordhauWidgetComponent-1` :`RelativeTransform` (`KismetMathLibrary.MakeTransform` (`SceneComponent.RelativeLocation` (`self.WidgetLocation`)))))
      (set `self.Widget` _returnvalue))
    (:`then_2`
      (`self.SetAvailability` false)
      (set `self.Initialized` true))))

(fn `OnRep_CooldownRemaining`)

(fn `SetAvailability`
  (params (NewAvailable :type Boolean))
  (set `self.IsAvailable` NewAvailable))

(fn `SpawnItem`
  (params (ForCharacter :type "/Game/Mordhau/Blueprints/Characters/BP_MordhauCharacter Object Reference"))
  (locals (Emblem :type Integer) (EmblemColor1 :type Byte) (EmblemColor2 :type Byte) (Customization :type "EquipmentCustomization Structure"))
  (bind _itemtogive (`self.ItemToGive`))
  (if (`KismetSystemLibrary.IsValidClass` _itemtogive)
    (bind _returnvalue (`|SpawnActorFromClass` _itemtogive (`self.GetTransform`) "Undefined" "OverrideRootScale" null null))
    (bind _asmordhau_equipment (cast `MordhauEquipment` _returnvalue))
    (bind _returnvalue_2 (`MordhauEquipment.GetRandomCustomization` _asmordhau_equipment true))
    (set `local.Customization` _returnvalue_2)
    (`|ExecutionSequence`
      (:`then_0`
        (bind _asmordhau_player_controller (cast `MordhauPlayerController` (`Pawn.GetController` ForCharacter)))
        (bind (_emblem _emblemcolors) (break `AppearanceCustomization` (`.AppearanceCustomization` (break `CharacterProfile` (`MordhauPlayerController.CharacterProfile` _asmordhau_player_controller)))))
        (set `local.Emblem` _emblem)
        (set `local.EmblemColor1` (`|GetArrayItem` _emblemcolors))
        (set `local.EmblemColor2` (`|GetArrayItem` _emblemcolors 1))
        (bind (_outcustomization _returnvalue_3) (`MordhauPlayerController.GetDefaultEquipmentCustomizationFor` _asmordhau_player_controller (`GameplayStatics.GetObjectClass` _asmordhau_equipment)))
        (if _returnvalue_3
          (set `local.Customization` _outcustomization)))
      (:`then_1`
        (`MordhauEquipment.AssignCustomization` _asmordhau_equipment (`local.Customization`) (`KismetMathLibrary.Conv_IntToByte` (`local.Emblem`)) (`local.EmblemColor1`) (`local.EmblemColor2`))
        (`MordhauEquipment.RestockOtherEquipmentOnCharacter` _asmordhau_equipment ForCharacter)
        (if (not (and (`MordhauEquipment.bDestroyIfNoAmmo` _asmordhau_equipment) (== (`MordhauEquipment.GetAmmo` _asmordhau_equipment) 0)))
          (bind _returnvalue_4 (`MordhauCharacter.PickUp` ForCharacter _asmordhau_equipment -1))
          (if _returnvalue_4
            (`MordhauCharacter.SwitchEquipment` ForCharacter _asmordhau_equipment)
            (else
              (set `MordhauEquipment.bCanRagdoll` true _asmordhau_equipment)
              (`MordhauEquipment.UpdateEquipmentState` _asmordhau_equipment))))))))

(fn `UpdateVisuals`
  (bind _returnvalue (`GameplayStatics.GetPlayerController` 0))
  (bind _returnvalue_2 (`KismetSystemLibrary.MakeLiteralDouble` (`self.WidgetViewDistance`)))
  (bind _returnvalue_3 (`KismetMathLibrary.VSize` (- (`self.K2_GetActorLocation`) (`PlayerCameraManager.GetCameraLocation` (`GameplayStatics.GetPlayerCameraManager` 0)))))
  (`|ExecutionSequence`
    (:`then_0`
      (if (not (`self.Initialized`))
        (`self.InitializeDisplay`)))
    (:`then_1`
      (`/Engine/EditorBlueprintResources/StandardMacros.IsValid` _returnvalue
        (:`Is Valid`
          (if (`Controller.IsLocalPlayerController` _returnvalue)
            (`|ExecutionSequence`
              (:`then_0`
                (if (> (`self.CooldownRemaining`) 0.0)
                  (`self.SetAvailability` false)
                  (else
                    (`self.SetAvailability` true))))
              (:`then_1`
                (`|ExecutionSequence`
                  (:`then_0`
                    (set `self.IsValid` true))
                  (:`then_1`
                    (if (!= (`MordhauWidgetComponent.OverrideVisible` (`self.Widget`)) 0)
                      (if (not (< _returnvalue_3 (+ _returnvalue_2 25.0)))
                        (set `MordhauWidgetComponent.OverrideVisible` 0 (`self.Widget`)))
                      (elif (< _returnvalue_3 _returnvalue_2)
                        (set `MordhauWidgetComponent.OverrideVisible` -1 (`self.Widget`))))))))))))))

(fn `UserConstructionScript`
  (bind _skeletalmesh (`self.SkeletalMesh`))
  (bind _static_mesh (`self.Static Mesh`))
  (`parent.UserConstructionScript`)
  (if (or (`MordhauUtilityLibrary.IsEditor`) (`MordhauUtilityLibrary.IsPlayInEditor`))
    (`TextRenderComponent.K2_SetText` (`self.TextRender`) (`self.WidgetText`))
    (`/Engine/EditorBlueprintResources/StandardMacros.IsValid` _skeletalmesh
      (:`Is Valid`
        (`SkinnedMeshComponent.SetSkinnedAssetAndUpdate` (`self.LODSkeletalMesh`) _skeletalmesh true))
      (:`Is Not Valid`
        (`/Engine/EditorBlueprintResources/StandardMacros.IsValid` _static_mesh
          (:`Is Valid`
            (`StaticMeshComponent.SetStaticMesh` (`self.StaticMesh`) _static_mesh)))))))