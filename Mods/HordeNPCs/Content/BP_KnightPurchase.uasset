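; Horde-mode purchase interactable that spends a player's coins to spawn an AI knight bot on team 0.
; Interaction is gated by cost and a cap on living bots; it possesses the bot with a new AI controller, assigns its profile and equips weapons.
; Display setup derives a mesh and adds a widget toggled by camera distance, with availability following coins.
; Optional chest mode breaks on purchase, using a RepNotify for effects, ragdoll and timed respawn.
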(event `self.ReceiveBeginPlay`
  (`parent.ReceiveBeginPlay`)
  (`/Engine/EditorBlueprintResources/StandardMacros.Can Execute Cosmetic Events`
    (:`True`
      (`self.SetAvailability` false))))

(event `self.OnInteractionStart`
  (params (Character :type "MordhauCharacter Object Reference"))
  (bind _spawntransform (`self.SpawnTransform`))
  (bind _asbp_horde_player_state (cast `/Game/Mordhau/Blueprints/GameModes/Horde/BP_HordePlayerState` (`Pawn.PlayerState` Character)))
  (bind _asbp_horde_character (cast `/Game/Mordhau/Blueprints/Characters/BP_HordeCharacter` Character))
  (`|ExecutionSequence`
    (:`then_0`
      (bind _returnvalue (`|SpawnActorFromClass` "/HordeNPCs/BP_KnightAIController.BP_KnightAIController_C" _spawntransform "Undefined" "OverrideRootScale" null null))
      (bind _returnvalue_2 (`|GenericCreateObject` (`self.Behavior Profile`) _returnvalue))
      (set `MordhauAIController.BehaviorProfile` _returnvalue_2 _returnvalue)
      (bind _returnvalue_3 (`|SpawnActorFromClass` (`self.Bot Class`) _spawntransform "Undefined" "OverrideRootScale" _returnvalue null))
      (bind _asmordhau_character (cast `MordhauCharacter` _returnvalue_3))
      (`MordhauCharacter.AssignProfile` _asmordhau_character (`self.New Profile`))
      (`Controller.Possess` _returnvalue _asmordhau_character)
      (set `AdvancedCharacter.Team` 0 _asmordhau_character)
      (for _array_element (`self.Weapons`)
        (bind _returnvalue_4 (`|SpawnActorFromClass` _array_element _spawntransform "Undefined" "OverrideRootScale" _asmordhau_character _asmordhau_character)) ; Name of weapon to spawn in
        (bind _asmordhau_equipment (cast `MordhauEquipment` _returnvalue_4))
        (`MordhauEquipment.AssignCustomization` _asmordhau_equipment (make `EquipmentCustomization` 0 (`|MakeArray` 0 0 0 :!type "Byte") (`|MakeArray` 0 0 0 :!type "Byte")) 0 0 0)
        (`MordhauCharacter.PickUp` _asmordhau_character _asmordhau_equipment 0)))
    (:`then_1`
      (set `/Game/Mordhau/Blueprints/GameModes/Horde/BP_HordePlayerState.Coins` (- (`/Game/Mordhau/Blueprints/GameModes/Horde/BP_HordePlayerState.Coins` _asbp_horde_player_state) (`self.Cost`)) _asbp_horde_player_state)
      (bind _asbp_horde_player_controller (cast `/Game/Mordhau/Blueprints/GameModes/Horde/BP_HordePlayerController` (`Pawn.GetController` _asbp_horde_character)))
      (set `/Game/Mordhau/Blueprints/GameModes/Horde/BP_HordePlayerController.PurchaseTrigger` (+ (`/Game/Mordhau/Blueprints/GameModes/Horde/BP_HordePlayerController.PurchaseTrigger` _asbp_horde_player_controller) 1) _asbp_horde_player_controller))
    (:`then_2`
      (if (`self.UseChests`)
        (bind _asbp_horde_player_controller_2 (cast `/Game/Mordhau/Blueprints/GameModes/Horde/BP_HordePlayerController` (`Pawn.GetController` _asbp_horde_character))
          (:`then`
            (`self.BreakChest` _asbp_horde_player_controller_2))
          (:`CastFailed`
            (`self.BreakChest` null)))))))

(event `RespawnChest`
  (if (`self.UseChests`)
    (`KismetSystemLibrary.Delay` (`self.RespawnTimeChests`))
    (set `self.ChestDestroyed` false)))

(fn `BreakChest`
  (params (DestroyerPlayerController :type "MordhauPlayerController Object Reference"))
  (if (`self.UseChests`)
    (if (not (`self.ChestDestroyed`))
      (`PrimitiveComponent.SetCollisionEnabled` (`self.LODSkeletalMesh`) "NoCollision")
      (`self.SpawnContents` DestroyerPlayerController)
      (set `self.ChestDestroyed` true))))

(fn `CanInteract`
  (params (Character :type "MordhauCharacter Object Reference"))
  (returns (ReturnValue :type Boolean))
  (bind _temp (`self.Temp`))
  (bind _outactors (`GameplayStatics.GetAllActorsOfClass` (`self.Bot Class`)))
  (`KismetArrayLibrary.Array_Clear` _temp)
  (for _array_element _outactors
    (bind _asbp_mordhau_character (cast `/Game/Mordhau/Blueprints/Characters/BP_MordhauCharacter` _array_element))
    (if (not (`AdvancedCharacter.GetIsDead` _asbp_mordhau_character))
      (`KismetArrayLibrary.Array_AddUnique` _temp _asbp_mordhau_character)))
  (if (< (`KismetArrayLibrary.Array_Length` _temp) (`self.MaxAllowedAmmount`))
    (`/Engine/EditorBlueprintResources/StandardMacros.IsValid` Character
      (:`Is Valid`
        (bind _asbp_horde_player_state (cast `/Game/Mordhau/Blueprints/GameModes/Horde/BP_HordePlayerState` (`Pawn.PlayerState` Character))
          (:`then`
            (if (>= (`/Game/Mordhau/Blueprints/GameModes/Horde/BP_HordePlayerState.Coins` _asbp_horde_player_state) (`self.Cost`))
              (return true)
              (else
                _)))
          (:`CastFailed`
            _)))
      (:`Is Not Valid`
        _)))
  (return false))

(fn `GetLocation`
  (returns (ReturnValue :type "Transform Structure"))
  (return (`KismetMathLibrary.Conv_VectorToTransform` (+ (`self.K2_GetActorLocation` self) (`KismetMathLibrary.MakeVector` (`KismetMathLibrary.RandomFloatInRange` -100.0 100.0) (`KismetMathLibrary.RandomFloatInRange` -100.0 100.0) 100.0)))))

(fn `InitializeDisplay`
  (bind _lodskeletalmesh (`self.LODSkeletalMesh`))
  (bind _purchasableclass (`self.PurchasableClass`))
  (bind _newmesh (`self.NewMesh`))
  (bind _lodskeletalmesh_2 (`self.LODSkeletalMesh`))
  (`|ExecutionSequence`
    (:`then_0`
      (`/Engine/EditorBlueprintResources/StandardMacros.IsValid` _newmesh
        (:`Is Valid`
          (`SkinnedMeshComponent.SetSkinnedAssetAndUpdate` _lodskeletalmesh_2 _newmesh true)
          (`StaticMeshComponent.SetStaticMesh` (`self.StaticMesh`) null))
        (:`Is Not Valid`
          (`SkinnedMeshComponent.SetSkinnedAssetAndUpdate` _lodskeletalmesh_2 null true)
          (`StaticMeshComponent.SetStaticMesh` (`self.StaticMesh`) null)
          (if (`KismetSystemLibrary.IsValidClass` _purchasableclass)
            (`|ExecutionSequence`
              (:`then_0`
                (bind _returnvalue (`|SpawnActorFromClass` _purchasableclass (`self.GetTransform`) "Undefined" "OverrideRootScale" null null))
                (bind _asmordhau_equipment (cast `MordhauEquipment` _returnvalue))
                (set `MordhauEquipment.bForceInstantMeshUpdate` true _asmordhau_equipment)
                (bind _returnvalue_2 (`MordhauEquipment.GetRandomCustomization` _asmordhau_equipment true))
                (`MordhauEquipment.AssignCustomization` _asmordhau_equipment _returnvalue_2 0 0 0)
                (bind _skeletalmeshcomponent (`MordhauEquipment.SkeletalMeshComponent` _asmordhau_equipment))
                (`SkinnedMeshComponent.SetSkinnedAssetAndUpdate` _lodskeletalmesh (`SkinnedMeshComponent.SkeletalMesh` _skeletalmeshcomponent) true)
                (`SkinnedMeshComponent.SetPhysicsAsset` _lodskeletalmesh (`MordhauEquipment.PhysicsAsset` _asmordhau_equipment) false)
                (for _index (range (`PrimitiveComponent.GetNumMaterials` _skeletalmeshcomponent))
                  (bind _returnvalue_3 (`PrimitiveComponent.GetMaterial` _skeletalmeshcomponent _index))
                  (`PrimitiveComponent.SetMaterial` _lodskeletalmesh _index _returnvalue_3)
                  (bind _asmaterial_instance_dynamic (cast `MaterialInstanceDynamic` _returnvalue_3))
                  (`MaterialInstanceDynamic.SetScalarParameterValue` _asmaterial_instance_dynamic "ShineIntensity" 1.0)))
              (:`then_1`
                (`self.K2_DestroyActor` _returnvalue)))
            (elif (`self.UseChests`)
              (`SkinnedMeshComponent.SetSkinnedAssetAndUpdate` (`self.LODSkeletalMesh`) (`self.ChestMesh`) true))))))
    (:`then_1`
      (bind _returnvalue_4 (`MordhauUtilityLibrary.GetComponentsBoundingBoxInActorSpace` self))
      (bind _returnvalue_5 (`AddComponent|NODE_AddMordhauWidgetComponent-0` :`RelativeTransform` (`KismetMathLibrary.MakeTransform` _returnvalue_4)))
      (set `self.Widget` _returnvalue_5))
    (:`then_2`
      (`self.SetAvailability` false)
      (set `self.Initialized` true))))

(fn `OnChestDestroyed`)

(fn `OnRep_ChestDestroyed`
  (bind _returnvalue (`self.K2_GetActorLocation`))
  (bind _chestdestroyed (`self.ChestDestroyed`))
  (bind _lodskeletalmesh (`self.LODSkeletalMesh`))
  (bind _returnvalue_2 (`PrimitiveComponent.GetCollisionEnabled` _lodskeletalmesh))
  (if (`self.UseChests`)
    (set `self.bIsInteractable` (not _chestdestroyed))
    (`|ExecutionSequence`
      (:`then_0`
        (`SceneComponent.SetHiddenInGame` (`self.LODSkeletalMesh`) _chestdestroyed false)
        (if _chestdestroyed
          (`|ExecutionSequence`
            (:`then_0`
              (if (`|EnumInequality` _returnvalue_2 "NoCollision")
                (`PrimitiveComponent.SetCollisionEnabled` _lodskeletalmesh "NoCollision")))
            (:`then_1`
              (`/Engine/EditorBlueprintResources/StandardMacros.Can Execute Cosmetic Events`
                (:`True`
                  (`GameplayStatics.SpawnEmitterAtLocation` (`self.DestroyedParticles`) _returnvalue)
                  (`GameplayStatics.PlaySoundAtLocation` "/Game/Mordhau/Audio/Cues/Misc/SC_Chest_Break.SC_Chest_Break" _returnvalue (struct) 1.0 1.0 0.0 null null null)
                  (`/Engine/EditorBlueprintResources/StandardMacros.IsValid` (`self.DestroyedRagdollMesh`)
                    (:`Is Valid`
                      (bind _returnvalue_3 (`|SpawnActorFromClass` "/Game/Mordhau/Blueprints/GameModes/BattleRoyale/BP_BattleRoyaleChestRagdoll.BP_BattleRoyaleChestRagdoll_C" (`self.GetTransform`) "Undefined" "OverrideRootScale" null null))
                      (`SkinnedMeshComponent.SetSkinnedAssetAndUpdate` (`SkeletalMeshActor.SkeletalMeshComponent` _returnvalue_3) (`self.DestroyedRagdollMesh`) true)
                      (bind _skeletalmeshcomponent (`SkeletalMeshActor.SkeletalMeshComponent` _returnvalue_3))
                      (`PrimitiveComponent.SetCollisionEnabled` _skeletalmeshcomponent "QueryAndPhysics")
                      (`PrimitiveComponent.SetSimulatePhysics` _skeletalmeshcomponent true)))))))
          (elif (`|EnumInequality` _returnvalue_2 "QueryAndPhysics")
            (`PrimitiveComponent.SetCollisionEnabled` _lodskeletalmesh "QueryAndPhysics"))))
      (:`then_1`
        (if _chestdestroyed
          (`self.OnChestDestroyed`)
          (`/Engine/EditorBlueprintResources/ActorMacros.Switch Has Authority`
            (:`Authority`
              (if (> (`self.RespawnTimeChests`) 0.0)
                (`self.RespawnChest`)
                (else
                  (`self.SetLifeSpan` 2.0))))))))))

(fn `SetAvailWidget`
  (returns (ReturnValue :type String))
  (locals (Temp :type "Array of Actor Object Reference"))
  (bind _temp (`local.Temp`))
  (bind _outactors (`GameplayStatics.GetAllActorsOfClass` (`self.Bot Class`)))
  (`KismetArrayLibrary.Array_Clear` _temp)
  (for _array_element _outactors
    (bind _asbp_mordhau_character (cast `/Game/Mordhau/Blueprints/Characters/BP_MordhauCharacter` _array_element))
    (if (not (`AdvancedCharacter.GetIsDead` _asbp_mordhau_character))
      (`KismetArrayLibrary.Array_AddUnique` _temp _asbp_mordhau_character)))
  (return (`KismetStringLibrary.Concat_StrStr` (`KismetTextLibrary.Conv_TextToString` (`self.ClassName`)) " \n" "Cost: " (`KismetStringLibrary.Conv_IntToString` (`self.Cost`)) " \n" (`KismetStringLibrary.Conv_IntToString` (`KismetArrayLibrary.Array_Length` _temp)) "/" (`KismetStringLibrary.Conv_IntToString` (`self.MaxAllowedAmmount`)))))

(fn `SpawnContents`
  (params (CustomizeFor :type "MordhauPlayerController Object Reference")))

(fn `UpdateVisuals`
  (bind _returnvalue (`GameplayStatics.GetPlayerController` 0))
  (bind _isavailable (`self.IsAvailable`))
  (bind _returnvalue_2 (`KismetMathLibrary.VSize` (- (`self.K2_GetActorLocation`) (`PlayerCameraManager.GetCameraLocation` (`GameplayStatics.GetPlayerCameraManager` 0)))))
  (`|ExecutionSequence`
    (:`then_0`
      (if (not (`self.Initialized`))
        (`self.InitializeDisplay`)))
    (:`then_1`
      (`/Engine/EditorBlueprintResources/StandardMacros.IsValid` _returnvalue
        (:`Is Valid`
          (if (`Controller.IsLocalPlayerController` _returnvalue)
            (`|ExecutionSequence`
              (:`then_0`
                (bind _asbp_horde_player_state (cast `/Game/Mordhau/Blueprints/GameModes/Horde/BP_HordePlayerState` (`Controller.PlayerState` _returnvalue)))
                (if (`self.ChestDestroyed`)
                  (set `MordhauWidgetComponent.OverrideVisible` 0 (`self.Widget`))
                  (elif (not (== _isavailable (>= (`/Game/Mordhau/Blueprints/GameModes/Horde/BP_HordePlayerState.Coins` _asbp_horde_player_state) (`self.Cost`))))
                    (`self.SetAvailability` (not _isavailable)))))
              (:`then_1`
                (`|ExecutionSequence`
                  (:`then_0`
                    (set `self.IsValid` true))
                  (:`then_1`
                    (if (!= (`MordhauWidgetComponent.OverrideVisible` (`self.Widget`)) 0)
                      (if (not (< _returnvalue_2 (+ 800.0 25.0)))
                        (set `MordhauWidgetComponent.OverrideVisible` 0 (`self.Widget`)))
                      (elif (< _returnvalue_2 800.0)
                        (set `MordhauWidgetComponent.OverrideVisible` -1 (`self.Widget`))))))))))))))

(fn `UserConstructionScript`
  (`parent.UserConstructionScript`))