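; BP_NormalKnight is a knight character, apparently AI-driven, that takes no damage from certain allied pawn types.
; Six seconds after BeginPlay it destroys itself if it has no valid controller.
; On death it removes its MordhauWidget component and destroys its controller.
; ModifyDamage returns zero when the instigator's pawn is a BP_HordeCharacter, BP_NormalKnight or BP_SpecialKnight_2, otherwise the parent's result.
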(event `self.ReceiveBeginPlay`
  (`parent.ReceiveBeginPlay`)
  (`KismetSystemLibrary.Delay` 6.0)
  (`/Engine/EditorBlueprintResources/StandardMacros.IsValid` (`self.GetController`)
    (:`Is Not Valid`
      (`self.K2_DestroyActor`))))

(event `self.OnDied`
  (params (Angle :type "Float (single-precision)") (Type :type "EMordhauDamageType Enum" :default "Generic") (SubType :type Byte) (Bone :type Name) (Point :type "Vector Structure") (Source :type "Actor Object Reference") (Agent :type "Actor Object Reference"))
  (`parent.OnDied` Angle Type SubType Bone Point Source Agent)
  (`|ExecutionSequence`
    (:`then_0`
      (`ActorComponent.K2_DestroyComponent` (`self.MordhauWidget`)))
    (:`then_1`
      (`self.K2_DestroyActor` (`self.GetController`)))))

(fn `ModifyDamage`
  (params (DamageAmount :type "Float (double-precision)") (DamageInfo :type "MordhauDamageInfo Structure (by ref)") (EventInstigator :type "Controller Object Reference"))
  (returns (ReturnValue :type "Float (double-precision)"))
  (bind _returnvalue (`Controller.K2_GetPawn` EventInstigator))
  (bind _returnvalue_2 (`parent.ModifyDamage` DamageAmount DamageInfo EventInstigator))
  (cast `/Game/Mordhau/Blueprints/Characters/BP_HordeCharacter` _returnvalue
    (:`then`
      _)
    (:`CastFailed`
      (cast `/Game/BP_NormalKnight` _returnvalue
        (:`then`
          _)
        (:`CastFailed`
          (cast `/HordeNPCs/BP_SpecialKnight_2` _returnvalue
            (:`then`
              _)
            (:`CastFailed`
              (return _returnvalue_2)))))))
  (return 0.0))

(fn `UserConstructionScript`
  (`parent.UserConstructionScript`))