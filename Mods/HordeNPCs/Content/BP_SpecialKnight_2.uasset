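; Special AI knight character with ability helpers, which ignores damage from horde characters, normal knights and its own class.
; Abilities start as net motions unless one is active, with timing helpers for cooldown and duration.
; Helpers pick reachable teleport points near random spots, trace to ground, and spawn two angled extra projectiles server-side behind a recursion guard.
; It destroys itself if uncontrolled shortly after spawning, and its controller on death.
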(event `self.ReceiveBeginPlay`
  (`parent.ReceiveBeginPlay`)
  (`KismetSystemLibrary.Delay` 6.0)
  (`/Engine/EditorBlueprintResources/StandardMacros.IsValid` (`self.GetController`)
    (:`Is Not Valid`
      (`self.K2_DestroyActor`))))

(event `self.OnDied`
  (params (Angle :type "Float (single-precision)") (Type :type "EMordhauDamageType Enum" :default "Generic") (SubType :type Byte) (Bone :type Name) (Point :type "Vector Structure") (Source :type "Actor Object Reference") (Agent :type "Actor Object Reference"))
  (`parent.OnDied` Angle Type SubType Bone Point Source Agent)
  (`|ExecutionSequence`
    (:`then_0`
      (`ActorComponent.K2_DestroyComponent` (`self.MordhauWidget`)))
    (:`then_1`
      (`self.K2_DestroyActor` (`self.GetController`)))))

(fn `DoSpecialAbility`
  (params (SpecialAbility :type Integer))
  (returns (Success :type Boolean))
  (cast `/Game/Mordhau/Blueprints/Motions/BP_AbilityMotion` (`self.GetMotion`)
    (:`then`
      (`KismetSystemLibrary.PrintString` "Knight Ability Fail")
      (return false))
    (:`CastFailed`
      (`self.AssignNetMotionSimple` (enumliteral `EMotionType` "Ability") (`KismetMathLibrary.Conv_IntToByte` SpecialAbility))
      (`KismetSystemLibrary.PrintString` "Knight Ability used")
      (return true))))

(fn `FindTeleport`
  (returns (TeleportLocation :type "Vector Structure"))
  (locals (NewLocalVar_0 :type "Array of /Game/Mordhau/Blueprints/Characters/BP_MordhauCharacter Object Reference"))
  (bind _teleportspots (`self.TeleportSpots`))
  (`KismetArrayLibrary.Array_Shuffle` _teleportspots)
  (bind _element (`self.Random Element (Ref)` _teleportspots)
    (:`NewParam`
      (return (`NavigationSystemV1.K2_GetRandomReachablePointInRadius` (`KismetMathLibrary.MakeVector` (.x (`self.K2_GetActorLocation` _element)) (.y (`self.K2_GetActorLocation` _element)) (+ (.z (`self.K2_GetActorLocation` _element)) 300.0)) 500.0 null "/Game/Mordhau/AI/Navigation/BP_NavFilter_Default.BP_NavFilter_Default_C")))))

(fn `GetFloorWalkable`
  (returns (`Walkable Floor` :type Boolean))
  (if (`.bWalkableFloor` (break `FindFloorResult` (`CharacterMovementComponent.CurrentFloor` (`self.CharacterMovement`))))
    (return true)
    (else
      (return false))))

(fn `ModifyDamage`
  (params (DamageAmount :type "Float (double-precision)") (DamageInfo :type "MordhauDamageInfo Structure (by ref)") (EventInstigator :type "Controller Object Reference"))
  (returns (ReturnValue :type "Float (double-precision)"))
  (bind _returnvalue (`Controller.K2_GetPawn` EventInstigator))
  (bind _returnvalue_2 (`parent.ModifyDamage` DamageAmount DamageInfo EventInstigator))
  (cast `/Game/Mordhau/Blueprints/Characters/BP_HordeCharacter` _returnvalue
    (:`then`
      _)
    (:`CastFailed`
      (cast `/HordeNPCs/BP_NormalKnight` _returnvalue
        (:`then`
          _)
        (:`CastFailed`
          (cast `/Game/BP_SpecialKnight_2` _returnvalue
            (:`then`
              _)
            (:`CastFailed`
              (return _returnvalue_2)))))))
  (return 0.0))

(fn `RememberStartAbilityTime`
  (params (Duration :type "Float (double-precision)"))
  (returns (OutDuration :type "Float (double-precision)"))
  (set `self.LastAbilityStartTime` (`GameplayStatics.GetTimeSeconds`))
  (bind _output_get (set `self.LastAbilityDuration` Duration))
  (return _output_get))

(fn `SpecialCooldown`
  (params (Duration :type "Float (double-precision)"))
  (`/Engine/EditorBlueprintResources/ActorMacros.Switch Has Authority`
    (:`Authority`
      (bind _output_get (set `self.NextSpecialTime` (+ Duration (`GameplayStatics.GetTimeSeconds`))))
      (`KismetSystemLibrary.PrintString` (`KismetStringLibrary.Concat_StrStr` "Special Cooldown Activated: " (`KismetStringLibrary.Conv_DoubleToString` _output_get))))))

(fn `TraceToGround`
  (params (ActorOr :type "Actor Object Reference") (Location :type "Vector Structure") (TraceComplex :type Boolean) (Type :type "EObjectTypeQuery Enum" :default "ObjectTypeQuery1") (Debug :type Boolean))
  (returns (Hit :type Boolean) (HitResult :type "HitResult Structure"))
  (locals (TraceStart :type "Vector Structure") (ActorsToIgnore :type "Array of Actor Object Reference") (DebugType :type "EDrawDebugTrace Enum"))
  (`/Engine/EditorBlueprintResources/StandardMacros.IsValid` ActorOr
    (:`Is Valid`
      (set `local.TraceStart` (`self.K2_GetActorLocation` ActorOr))
      (set `local.ActorsToIgnore` (`|MakeArray` ActorOr)))
    (:`Is Not Valid`
      (set `local.TraceStart` Location)))
  (if Debug
    (set `local.DebugType` "Persistent"))
  (bind (_outhit _returnvalue) (`KismetSystemLibrary.LineTraceSingleForObjects` null (`local.TraceStart`) (+ (`local.TraceStart`) (0.0 0.0 -999999.0)) (`|MakeArray` Type) TraceComplex (`local.ActorsToIgnore`) (`local.DebugType`)))
  (return _returnvalue _outhit))

(fn `TryScatterShot`
  (params (SourceProjectile :type "MordhauProjectile Object Reference"))
  (bind _returnvalue (`GameplayStatics.GetObjectClass` SourceProjectile))
  (bind _returnvalue_2 (`self.GetTransform` SourceProjectile))
  (bind _returnvalue_3 (`AIBlueprintHelperLibrary.GetAIController` self))
  (bind _rotation (.rotation _returnvalue_2))
  (bind _scale (.scale _returnvalue_2))
  (`/Engine/EditorBlueprintResources/ActorMacros.Switch Has Authority`
    (:`Authority`
      (if (not (`self.AvoidScattershotRecursion`))
        (set `self.AvoidScattershotRecursion` true)
        (`|ExecutionSequence`
          (:`then_0`
            (`|ExecutionSequence`
              (:`then_0`
                (bind _returnvalue_4 (`|SpawnActorFromClass` _returnvalue (`KismetMathLibrary.MakeTransform` (`KismetMathLibrary.TransformLocation` _returnvalue_2 (50.0 100.0 0.0)) (`KismetMathLibrary.MakeRotator` (.roll _rotation) (.pitch _rotation) (+ (.yaw _rotation) 10.0)) _scale) "Undefined" "OverrideRootScale" null null))
                (set `MordhauProjectile.bUsesLocalProjectileBlending` false _returnvalue_4)
                (`MordhauProjectile.InitializeProjectile` _returnvalue_4 _returnvalue_3 false self)
                (`MordhauProjectile.Fire` _returnvalue_4))
              (:`then_1`
                (bind _returnvalue_5 (`|SpawnActorFromClass` _returnvalue (`KismetMathLibrary.MakeTransform` (`KismetMathLibrary.TransformLocation` _returnvalue_2 (50.0 -100.0 0.0)) (`KismetMathLibrary.MakeRotator` (.roll _rotation) (.pitch _rotation) (+ (.yaw _rotation) -10.0)) _scale) "Undefined" "OverrideRootScale" null null))
                (set `MordhauProjectile.bUsesLocalProjectileBlending` false _returnvalue_5)
                (`MordhauProjectile.InitializeProjectile` _returnvalue_5 _returnvalue_3 false self)
                (`MordhauProjectile.Fire` _returnvalue_5))))
          (:`then_1`
            (set `self.AvoidScattershotRecursion` false)))))))

(fn `UserConstructionScript`
  (`parent.UserConstructionScript`))