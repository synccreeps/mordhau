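; BP_BossAbilityMotion is a motion that drives the Yimir boss's eight special abilities, such as Hookshot, Shockwave, Lightning and Downfire.
; On begin it resets the boss's additive override and uses the net motion's first parameter to call the chosen ability's opening function on BP_Yimir.
; Tick counts down a timer, then fires that ability's second stage once.
; An interrupted exit destroys any valid Projectile.
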(event `self.OnBegin`
  (`parent.OnBegin`)
  (bind _asbp_yimir (cast `/HordeNPCs/Boss/BP_Yimir` (`self.GetOwnerMordhauCharacter`)))
  (`AdvancedCharacter.ResetAdditiveOverrideType` _asbp_yimir)
  (switch `int` (`KismetMathLibrary.Conv_ByteToInt` (`.MotionParam0` (break `NetMotion` (`MordhauCharacter.GetCurrentNetMotion` _asbp_yimir))))
    (:`0`
      (`/HordeNPCs/Boss/BP_Yimir.BeginHookshot` _asbp_yimir))
    (:`1`
      (`/HordeNPCs/Boss/BP_Yimir.BeginShockwave` _asbp_yimir))
    (:`2`
      (`/HordeNPCs/Boss/BP_Yimir.BeginImmortality` _asbp_yimir))
    (:`3`
      (`/HordeNPCs/Boss/BP_Yimir.BeginScatter` _asbp_yimir))
    (:`4`
      (`/HordeNPCs/Boss/BP_Yimir.BeginLightning` _asbp_yimir))
    (:`5`
      (`/HordeNPCs/Boss/BP_Yimir.Stage1ReverseShock` _asbp_yimir))
    (:`6`
      (`/HordeNPCs/Boss/BP_Yimir.RandomProjectiles` _asbp_yimir))
    (:`7`
      (`/HordeNPCs/Boss/BP_Yimir.Stage1Downfire` _asbp_yimir))))

(event `self.OnTick`
  (params (DeltaTime :type "Float (single-precision)"))
  (`parent.OnTick` DeltaTime)
  (if (== (`self.CurrentStage`) 0)
    (bind _output_get (set `self.Stage2Time` (- (`self.Stage2Time`) DeltaTime)))
    (if (<= _output_get 0.0)
      (set `self.CurrentStage` 1)
      (bind _asbp_yimir (cast `/HordeNPCs/Boss/BP_Yimir` (`self.GetOwnerMordhauCharacter`)))
      (switch `int` (`KismetMathLibrary.Conv_ByteToInt` (`.MotionParam0` (break `NetMotion` (`MordhauCharacter.GetCurrentNetMotion` _asbp_yimir))))
        (:`0`
          (`/HordeNPCs/Boss/BP_Yimir.Stage2Hookshot` _asbp_yimir))
        (:`1`
          (`/HordeNPCs/Boss/BP_Yimir.Stage2Shockwave` _asbp_yimir))
        (:`2`
          (`/HordeNPCs/Boss/BP_Yimir.Stage2Immortality` _asbp_yimir))
        (:`3`
          (`/HordeNPCs/Boss/BP_Yimir.Stage2Scatter` _asbp_yimir))
        (:`4`
          (`/HordeNPCs/Boss/BP_Yimir.Stage2Lightning` _asbp_yimir))
        (:`5`
          (`/HordeNPCs/Boss/BP_Yimir.Stage2ReverseShock` _asbp_yimir))
        (:`6`
          (`/HordeNPCs/Boss/BP_Yimir.Stage2Projectiles` _asbp_yimir))
        (:`7`
          (`/HordeNPCs/Boss/BP_Yimir.Stage2Downfire` _asbp_yimir))))))

(event `self.OnLeave`
  (params (Interrupted :type Boolean))
  (bind _projectile (`self.Projectile`))
  (`parent.OnLeave` Interrupted)
  (if Interrupted
    (`/Engine/EditorBlueprintResources/StandardMacros.IsValid` _projectile
      (:`Is Valid`
        (`Actor.K2_DestroyActor` _projectile)))))