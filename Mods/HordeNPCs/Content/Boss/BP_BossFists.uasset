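; Boss fists weapon for Mordhau that knocks enemy characters flying on hit.
; After the parent hit logic, characters on another team have an 85% chance to be launched along the fists' forward vector and upward.
; The launch repeats after a short delay, then a replicated knockback trip follows.
; A Yimir random special-ability branch remains disconnected, so attack start only calls the parent.
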(event `self.ReceiveBeginPlay`
  (`parent.ReceiveBeginPlay`))

(event `self.OnAttackStarted`
  (params (Move :type "EAttackMove Enum" :default "RightStrike") (Angle :type "Float (single-precision)"))
  (`parent.OnAttackStarted` Move Angle))

(event `self.OnHit`
  (params (Actor :type "Actor Object Reference") (Move :type "EAttackMove Enum" :default "RightStrike") (Bone :type Name) (WorldLocation :type "Vector Structure (by ref)") (Tier :type Byte) (SurfaceType :type Byte))
  (`parent.OnHit` Actor Move Bone WorldLocation Tier SurfaceType)
  (bind _asbp_mordhau_character (cast `/Game/Mordhau/Blueprints/Characters/BP_MordhauCharacter` Actor))
  (if (== (`AdvancedCharacter.Team` _asbp_mordhau_character) (`AdvancedCharacter.Team` (`self.GetParentCharacter`)))
    _
    (elif (`KismetMathLibrary.RandomBoolWithWeight` 0.85)
      (bind _newparam (`self.LaunchVelocity`))
      (`Character.LaunchCharacter` _asbp_mordhau_character _newparam false false)
      (`KismetSystemLibrary.Delay` 0.1)
      (`Character.LaunchCharacter` _asbp_mordhau_character _newparam false false)
      (`KismetSystemLibrary.Delay` 0.2)
      (`/Game/Mordhau/Blueprints/Characters/BP_MordhauCharacter.ReplicatedTripWithKnockback` _asbp_mordhau_character))))

(fn `LaunchVelocity`
  (returns (NewParam :type "Vector Structure"))
  (return (`KismetMathLibrary.MakeVector` (* (.x (`self.GetActorForwardVector`)) 500.0) (* (.y (`self.GetActorForwardVector`)) 500.0) (+ (.z (`self.GetActorForwardVector`)) 500.0))))

(fn `UserConstructionScript`
  (`parent.UserConstructionScript`))