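; BP_FireSubField_BM is a boss fire sub-field that adds decal timing and fade-out to its parent sub-field behavior.
; On BeginPlay it caches the particle system's world location and creates a dynamic decal material stamped with the current time as HitTime.
; Both deactivation events start a short delayed decal fade without destroying the actor, then call the parent.
; A FadedOutDecal flag keeps DeactivateSubField from restarting a fade already begun.
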(event `self.ReceiveBeginPlay`
  (`parent.ReceiveBeginPlay`)
  (set `self.Sublocation` (`SceneComponent.K2_GetComponentLocation` (`self.ParticleSystem`)))
  (bind _returnvalue (`DecalComponent.CreateDynamicMaterialInstance` (`self.Decal`)))
  (`MaterialInstanceDynamic.SetScalarParameterValue` _returnvalue "HitTime" (`GameplayStatics.GetTimeSeconds`)))

(event `self.BeginSubFieldDeactivation`
  (set `self.FadedOutDecal` true)
  (`DecalComponent.SetFadeOut` (`self.Decal`) 2.0 0.2 false)
  (`parent.BeginSubFieldDeactivation`))

(event `self.DeactivateSubField`
  (`|ExecutionSequence`
    (:`then_0`
      (if (not (`self.FadedOutDecal`))
        (`DecalComponent.SetFadeOut` (`self.Decal`) 2.0 0.2 false)
        (set `self.FadedOutDecal` true)))
    (:`then_1`
      (`parent.DeactivateSubField`))))

(fn `UserConstructionScript`
  (`parent.UserConstructionScript`))