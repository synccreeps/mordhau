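; Boss mage projectile for Mordhau that deals an icy area blast on impact, built on a parent projectile class.
; On hit it plays a world camera shake and ice impact particles, then hides the projectile visual and calls the parent hit handler.
; Only the authority applies radial falloff damage with knockback and structure damage, ignoring the shooter's pawn and friendlies.
; All other events and the construction script add no behavior.
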(event `self.OnProjectileHit`
  (params (HitLocation :type "Vector Structure") (HitNormal :type "Vector Structure") (BounceForce :type "Float (single-precision)") (Surface :type Byte) (bHasHitWorld :type Boolean) (bHasStopped :type Boolean))
  (`|ExecutionSequence`
    (:`then_0`
      (`GameplayStatics.PlayWorldCameraShake` "/Game/Mordhau/Blueprints/CameraShakes/ImpactShake.ImpactShake_C" HitLocation 500.0 900.0 10.0)
      (`GameplayStatics.SpawnEmitterAtLocation` "/HordeNPCs/Boss/Particle/Par_4E_Ice_Impact_01.Par_4E_Ice_Impact_01" HitLocation))
    (:`then_1`
      (`/Engine/EditorBlueprintResources/ActorMacros.Switch Has Authority`
        (:`Authority`
          (bind _returnvalue (`self.GetProjectileOwningController`))
          (`MordhauUtilityLibrary.MordhauApplyRadialDamageWithFalloff` 75.0 65.0 400.0 20.0 HitLocation 200.0 500.0 5.0 (`|MakeArray` (`Controller.K2_GetPawn` _returnvalue) :!type "Actor Object Reference") 500.0 350.0 0.0 self _returnvalue "ECC_Visibility" true))))
    (:`then_2`
      (`SceneComponent.SetHiddenInGame` (`self.NS_Projectile`) true false))
    (:`then_3`
      (`parent.OnProjectileHit` HitLocation HitNormal BounceForce Surface bHasHitWorld bHasStopped))))

(fn `UserConstructionScript`
  (`parent.UserConstructionScript`))