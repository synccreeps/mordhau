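; Boss area attack that, despite its MeteorVolley name, erupts as a one-shot thorn burst after an activation delay, then removes its decal.
; The server traces to ground, spawns thorn Niagara, launches living non-friendly characters in the Box, then expires.
; Victims are launched up and along their own facing twice in quick succession, then tripped with knockback.
; Meteor effects, repeating ticks and line-of-sight damage remain as disconnected nodes.
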(event `self.ReceiveBeginPlay`
  (`KismetSystemLibrary.Delay` (`self.ActivationDelay`))
  (`|ExecutionSequence`
    (:`then_0`
      (`/Engine/EditorBlueprintResources/ActorMacros.Switch Has Authority`
        (:`Authority`
          (`self.DamageTick`)
          (`self.SetLifeSpan` 2.0))))
    (:`then_1`
      (`KismetSystemLibrary.Delay` 1.0)
      (`ActorComponent.K2_DestroyComponent` (`self.Decal`)))))

(event `DamageTick`
  (bind (_hit _hitresult) (`self.TraceToGround` self))
  (`NiagaraFunctionLibrary.SpawnSystemAtLocation` "/HordeNPCs/Boss/Particle/NS_Thorns_1.NS_Thorns_1" (`.Location` (`GameplayStatics.BreakHitResult` _hitresult)))
  (bind _asmordhau_game_state (cast `MordhauGameState` (`GameplayStatics.GetGameState`)))
  (bind _output_get (set `self.Overlaps` (`PrimitiveComponent.GetOverlappingActors` (`self.Box`) "/Script/Mordhau.AdvancedCharacter")))
  (for _array_element _output_get
    (bind _asadvanced_character (cast `AdvancedCharacter` _array_element))
    (if (not (`AdvancedCharacter.GetIsDead` _asadvanced_character))
      (bind _returnvalue (`MordhauGameState.IsFriendly` _asmordhau_game_state _asadvanced_character (`self.InstigatorController`) true))
      (if (not _returnvalue)
        (`self.Launch` _asadvanced_character)))))

(event `Launch`
  (params (Char :type "AdvancedCharacter Object Reference"))
  (bind _asbp_mordhau_character (cast `/Game/Mordhau/Blueprints/Characters/BP_MordhauCharacter` Char))
  (bind _newparam (`self.LaunchVelocity` _asbp_mordhau_character))
  (`Character.LaunchCharacter` _asbp_mordhau_character _newparam false false)
  (`KismetSystemLibrary.Delay` 0.1)
  (`Character.LaunchCharacter` _asbp_mordhau_character _newparam false false)
  (`KismetSystemLibrary.Delay` 0.2)
  (`/Game/Mordhau/Blueprints/Characters/BP_MordhauCharacter.ReplicatedTripWithKnockback` _asbp_mordhau_character))

(fn `LaunchVelocity`
  (params (Char :type "AdvancedCharacter Object Reference"))
  (returns (NewParam :type "Vector Structure"))
  (return (`KismetMathLibrary.MakeVector` (* (.x (`self.GetActorForwardVector` Char)) 1200.0) (* (.y (`self.GetActorForwardVector` Char)) 1200.0) (+ (.z (`self.GetActorForwardVector` Char)) 1200.0))))

(fn `TraceToGround`
  (params (ActorOr :type "Actor Object Reference") (Location :type "Vector Structure") (TraceComplex :type Boolean) (Type :type "EObjectTypeQuery Enum" :default "ObjectTypeQuery1") (Debug :type Boolean))
  (returns (Hit :type Boolean) (HitResult :type "HitResult Structure"))
  (locals (TraceStart :type "Vector Structure") (ActorsToIgnore :type "Array of Actor Object Reference") (DebugType :type "EDrawDebugTrace Enum"))
  (`/Engine/EditorBlueprintResources/StandardMacros.IsValid` ActorOr
    (:`Is Valid`
      (set `local.TraceStart` (`self.K2_GetActorLocation` ActorOr))
      (set `local.ActorsToIgnore` (`|MakeArray` ActorOr)))
    (:`Is Not Valid`
      (set `local.TraceStart` Location)))
  (if Debug
    (set `local.DebugType` "Persistent"))
  (bind (_outhit _returnvalue) (`KismetSystemLibrary.LineTraceSingleForObjects` null (`local.TraceStart`) (+ (`local.TraceStart`) (0.0 0.0 -999999.0)) (`|MakeArray` Type) TraceComplex (`local.ActorsToIgnore`) (`local.DebugType`)))
  (return _returnvalue _outhit))

(fn `UserConstructionScript`)