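; Boss weapon Blueprint for the Ulfberht, built on Mordhau's hit framework, whose live OnHit only passes through to the parent.
; Disconnected nodes hold an unused on-hit effect: a thorn Niagara burst at the traced ground point and authority-only radial damage with knockback that spares friendlies.
; The TraceToGround helper line-traces straight down from an actor or location, with optional debug drawing, and is called only by that unused effect.
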(event `self.OnHit`
  (params (Actor :type "Actor Object Reference") (Move :type "EAttackMove Enum" :default "RightStrike") (Bone :type Name) (WorldLocation :type "Vector Structure (by ref)") (Tier :type Byte) (SurfaceType :type Byte))
  (`parent.OnHit` Actor Move Bone WorldLocation Tier SurfaceType))

(fn `TraceToGround`
  (params (ActorOr :type "Actor Object Reference") (Location :type "Vector Structure") (TraceComplex :type Boolean) (Type :type "EObjectTypeQuery Enum" :default "ObjectTypeQuery1") (Debug :type Boolean))
  (returns (Hit :type Boolean) (HitResult :type "HitResult Structure"))
  (locals (TraceStart :type "Vector Structure") (ActorsToIgnore :type "Array of Actor Object Reference") (DebugType :type "EDrawDebugTrace Enum"))
  (`/Engine/EditorBlueprintResources/StandardMacros.IsValid` ActorOr
    (:`Is Valid`
      (set `local.TraceStart` (`self.K2_GetActorLocation` ActorOr))
      (set `local.ActorsToIgnore` (`|MakeArray` ActorOr)))
    (:`Is Not Valid`
      (set `local.TraceStart` Location)))
  (if Debug
    (set `local.DebugType` "Persistent"))
  (bind (_outhit _returnvalue) (`KismetSystemLibrary.LineTraceSingleForObjects` null (`local.TraceStart`) (+ (`local.TraceStart`) (0.0 0.0 -999999.0)) (`|MakeArray` Type) TraceComplex (`local.ActorsToIgnore`) (`local.DebugType`)))
  (return _returnvalue _outhit))

(fn `UserConstructionScript`
  (`parent.UserConstructionScript`))