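; Yimir is a Horde-mode AI boss caster that drives a HUD health bar and scales incoming damage by attacker class.
; A looping timer starts random specials off cooldown through ability motions, whose Begin/Stage2 functions handle projectiles, scatter shots, meteor and lightning volleys, push/pull shockwaves and brief immortality.
; A second timer teleports it upward for an ability, then to a random BP_BossTeleportActor, where it enrages at the nearest enemy and casts again.
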(event `CustomEvent_1`
  (bind _returnvalue (`self.GetMotion`))
  (bind _asbp_horde_aicontroller (cast `/Game/Mordhau/AI/BP_HordeAIController` (`AIBlueprintHelperLibrary.GetAIController` self)))
  (bind _returnvalue_2 (`MordhauAIController.PerceivesEnemy` _asbp_horde_aicontroller))
  (if _returnvalue_2
    (cast `/Game/Mordhau/Blueprints/Motions/BP_AbilityMotion` _returnvalue
      (:`CastFailed`
        (cast `AttackMotion` _returnvalue
          (:`CastFailed`
            (`self.DoSpecialAbility` 6)
            (bind _returnvalue_3 (`MordhauAIController.GetPerceivedEnemies` _asbp_horde_aicontroller))
            (bind _output_get (set `self.NewVar_4` _returnvalue_3))
            (`KismetArrayLibrary.Array_Shuffle` _output_get)
            (bind _element (`self.Random Element (Ref)` _output_get)
              (:`NewParam`
                (`self.Enrage` _element 4.0)))))))))

(event `self.ReceiveBeginPlay`
  (`parent.ReceiveBeginPlay`)
  (set `self.Scenes` (`|MakeArray` (`self.MordhauScene`) (`self.MordhauScene1`) (`self.MordhauScene2`) (`self.MordhauScene3`) (`self.MordhauScene4`) (`self.MordhauScene5`) (`self.MordhauScene6`) (`self.MordhauScene7`)))
  (bind _outactors (`GameplayStatics.GetAllActorsOfClass` "/HordeNPCs/Boss/BP_BossTeleportActor.BP_BossTeleportActor_C"))
  (bind _output_get (set `self.TeleportSpots` _outactors))
  (if (> (`KismetArrayLibrary.Array_Length` _output_get) 0)
    (bind _returnvalue (`KismetSystemLibrary.K2_SetTimerDelegate` (delegate `TeleportTo`) 15.312 true))
    (set `self.NewVar_0` _returnvalue))
  (bind _returnvalue_2 (`KismetSystemLibrary.K2_SetTimerDelegate` (delegate `CustomEvent_0`) 5.3 true))
  (set `self.NewVar_1` _returnvalue_2))

(event `CustomEvent_0`
  (bind _returnvalue (`GameplayStatics.GetGameState`))
  (`/Engine/EditorBlueprintResources/StandardMacros.IsValid` _returnvalue
    (:`Is Valid`
      (if (>= (`GameStateBase.GetServerWorldTimeSeconds` _returnvalue) (`self.NextSpecialTime`))
        (`self.DoSpecialAbility` (`KismetMathLibrary.RandomIntegerInRange` 0 5))))))

(event `TeleportTo`
  (bind _returnvalue (`self.K2_GetActorLocation`))
  (`GameplayStatics.PlaySoundAtLocation` "/HordeNPCs/Boss/SC/SC_IceProjectile.SC_IceProjectile" _returnvalue (struct) 1.0 1.0 0.0 null null null)
  (`NiagaraFunctionLibrary.SpawnSystemAtLocation` "/HordeNPCs/Boss/Particle/NS_Hit3.NS_Hit3" _returnvalue)
  (`self.K2_TeleportTo` (+ (`self.K2_GetActorLocation`) (0.0 0.0 800.0)))
  (`|ExecutionSequence`
    (:`then_0`
      (`self.DoSpecialAbility` 7))
    (:`then_1`
      (if (`self.GetFloorWalkable`) :!label _label
        (bind _teleportlocation (`self.FindTeleport`))
        (`NiagaraFunctionLibrary.SpawnSystemAtLocation` "/HordeNPCs/Boss/Particle/NS_Hit3.NS_Hit3" (`self.K2_GetActorLocation`))
        (`NiagaraFunctionLibrary.SpawnSystemAtLocation` "/HordeNPCs/Boss/Particle/NS_Hit3.NS_Hit3" _teleportlocation)
        (`self.K2_TeleportTo` _teleportlocation)
        (bind _asbp_horde_aicontroller (cast `/Game/Mordhau/AI/BP_HordeAIController` (`AIBlueprintHelperLibrary.GetAIController` self)))
        (bind _returnvalue_2 (`MordhauAIController.GetClosestEnemy` _asbp_horde_aicontroller))
        (`/Engine/EditorBlueprintResources/StandardMacros.IsValid` _returnvalue_2
          (:`Is Valid`
            (`self.Enrage` _returnvalue_2 4.0))
          (:`Is Not Valid`
            _))
        (if (`self.GetFloorWalkable`) :!label _label_2
          (`self.DoSpecialAbility` 1)
          (else
            (`KismetSystemLibrary.RetriggerableDelay` 0.1)
            (goto _label_2)))
        (else
          (`KismetSystemLibrary.Delay` 1.0)
          (goto _label))))))

(event `self.OnAfterDied`
  (params (Angle :type "Float (single-precision)") (Type :type "EMordhauDamageType Enum" :default "Generic") (SubType :type Byte) (Bone :type Name) (Point :type "Vector Structure") (Source :type "Actor Object Reference") (Agent :type "Actor Object Reference"))
  (`KismetSystemLibrary.K2_ClearAndInvalidateTimerHandle` (`self.NewVar_0`))
  (`KismetSystemLibrary.K2_ClearAndInvalidateTimerHandle` (`self.NewVar_1`))
  (`SceneComponent.SetHiddenInGame` (`self.NS_Snowstorm_Dot`) true true)
  (`parent.OnAfterDied` Angle Type SubType Bone Point Source Agent)
  (bind _asbp_horde_hud_bog (cast `/Jötunheimr/blueprints/BP_HordeHUD_BOG` (`MordhauUtilityLibrary.GetMordhauHUD`)))
  (bind _hudwidgetcustom (`/Jötunheimr/blueprints/BP_HordeHUD_BOG.HudWidgetCustom` _asbp_horde_hud_bog))
  (`/Engine/EditorBlueprintResources/StandardMacros.IsValid` _hudwidgetcustom
    (:`Is Valid`
      (`Widget.RemoveFromParent` (`/Jötunheimr/blueprints/BP_HordeHUDWidget_BOG.BP_BOssHP` _hudwidgetcustom)))))

(event `self.ReceiveTick`
  (params (DeltaSeconds :type "Float (single-precision)"))
  (`parent.ReceiveTick` DeltaSeconds)
  (bind _asbp_horde_hud_bog (cast `/Jötunheimr/blueprints/BP_HordeHUD_BOG` (`MordhauUtilityLibrary.GetMordhauHUD`)))
  (bind _hudwidgetcustom (`/Jötunheimr/blueprints/BP_HordeHUD_BOG.HudWidgetCustom` _asbp_horde_hud_bog))
  (`/Engine/EditorBlueprintResources/StandardMacros.IsValid` _hudwidgetcustom
    (:`Is Valid`
      (set `/Jötunheimr/blueprints/BP_HordeHUDWidget_BOG.BlackMageHealth` (/ (`KismetMathLibrary.Conv_ByteToDouble` (`self.Health`)) 100.0) _hudwidgetcustom))))

(event `self.OnAttackStarted`
  (`parent.OnAttackStarted`))

(event `RequestVolley`
  (params (Location :type "Vector Structure"))
  (bind _returnvalue (`AIBlueprintHelperLibrary.GetAIController` self))
  (`self.SpecialCooldown` 4.0)
  (cast `/HordeNPCs/Boss/BP_BossAbilityMotion` (`self.GetMotion`))
  (bind _returnvalue_2 (`|SpawnActorFromClass` "/HordeNPCs/Boss/BP_MeteorVolley.BP_MeteorVolley_C" (`KismetMathLibrary.MakeTransform` Location) "AlwaysSpawn" "OverrideRootScale" null _returnvalue null))
  (set `/HordeNPCs/Boss/BP_MeteorVolley.DamageMultiplier` 1.0 _returnvalue_2)
  (set `/HordeNPCs/Boss/BP_MeteorVolley.InstigatorController` _returnvalue _returnvalue_2))

(event `TriggerImmortality`
  (set `self.IsImmortal` true)
  (set `self.bIsUnflinchable` true)
  (`KismetSystemLibrary.RetriggerableDelay` (`self.LastAbilityDuration`))
  (set `self.IsImmortal` false)
  (set `self.bIsUnflinchable` false))

(event `RequestLightning`
  (params (Location :type "Vector Structure"))
  (bind _returnvalue (`AIBlueprintHelperLibrary.GetAIController` self))
  (cast `/HordeNPCs/Boss/BP_BossAbilityMotion` (`self.GetMotion`))
  (bind _returnvalue_2 (`|SpawnActorFromClass` "/HordeNPCs/Boss/BP_LightningVolley.BP_LightningVolley_C" (`KismetMathLibrary.MakeTransform` Location) "Undefined" "OverrideRootScale" null _returnvalue self))
  (set `/HordeNPCs/Boss/BP_LightningVolley.DamageMultiplier` 1.0 _returnvalue_2)
  (set `/HordeNPCs/Boss/BP_LightningVolley.InstigatorController` _returnvalue _returnvalue_2))

(fn `BeginHookshot`
  (bind _asbp_boss_ability_motion (cast `/HordeNPCs/Boss/BP_BossAbilityMotion` (`self.GetMotion`)))
  (set `MordhauMotion.EndTime` (+ (`MordhauMotion.StartTime` _asbp_boss_ability_motion) 1.0) _asbp_boss_ability_motion)
  (set `/HordeNPCs/Boss/BP_BossAbilityMotion.Stage2Time` 0.5 _asbp_boss_ability_motion)
  (`self.PlayAnim` "/HordeNPCs/Boss/Anim/MeteorVolley.MeteorVolley"))

(fn `BeginImmortality`
  (bind _asbp_boss_ability_motion (cast `/HordeNPCs/Boss/BP_BossAbilityMotion` (`self.GetMotion`)))
  (set `MordhauMotion.EndTime` (+ (`MordhauMotion.StartTime` _asbp_boss_ability_motion) 1.0) _asbp_boss_ability_motion)
  (set `/HordeNPCs/Boss/BP_BossAbilityMotion.Stage2Time` 0.25 _asbp_boss_ability_motion)
  (`self.PlayAnim` "/HordeNPCs/Boss/Anim/MTG_Immortality_V2.MTG_Immortality_V2"))

(fn `BeginLightning`
  (bind _asbp_boss_ability_motion (cast `/HordeNPCs/Boss/BP_BossAbilityMotion` (`self.GetMotion`)))
  (set `MordhauMotion.EndTime` (+ (`MordhauMotion.StartTime` _asbp_boss_ability_motion) 1.0) _asbp_boss_ability_motion)
  (set `/HordeNPCs/Boss/BP_BossAbilityMotion.Stage2Time` 0.5 _asbp_boss_ability_motion)
  (`self.PlayAnim` "/Game/Mordhau/Animations/Montages/MTG_Horde_Volley_V2.MTG_Horde_Volley_V2"))

(fn `BeginScatter`
  (bind _asbp_boss_ability_motion (cast `/HordeNPCs/Boss/BP_BossAbilityMotion` (`self.GetMotion`)))
  (set `MordhauMotion.EndTime` (+ (`MordhauMotion.StartTime` _asbp_boss_ability_motion) 1.0) _asbp_boss_ability_motion)
  (set `/HordeNPCs/Boss/BP_BossAbilityMotion.Stage2Time` 0.5 _asbp_boss_ability_motion)
  (`self.PlayAnim` "/Game/Mordhau/Animations/Montages/MTG_Horde_Volley_V2.MTG_Horde_Volley_V2"))

(fn `BeginShockwave`
  (bind _asbp_boss_ability_motion (cast `/HordeNPCs/Boss/BP_BossAbilityMotion` (`self.GetMotion`)))
  (set `MordhauMotion.EndTime` (+ (`MordhauMotion.StartTime` _asbp_boss_ability_motion) 1.0) _asbp_boss_ability_motion)
  (set `/HordeNPCs/Boss/BP_BossAbilityMotion.Stage2Time` 0.5 _asbp_boss_ability_motion)
  (`self.PlayAnim` "/HordeNPCs/Boss/Anim/MTG_Shockwave_V2.MTG_Shockwave_V2"))

(fn `DoSpecialAbility`
  (params (SpecialAbility :type Integer))
  (returns (Success :type Boolean))
  (cast `/Game/Mordhau/Blueprints/Motions/BP_AbilityMotion` (`self.GetMotion`)
    (:`then`
      (return false))
    (:`CastFailed`
      (`self.AssignNetMotionSimple` (enumliteral `EMotionType` "Ability") (`KismetMathLibrary.Conv_IntToByte` SpecialAbility))
      (return true))))

(fn `FindTargetsForLightning`
  (params (InRot :type "Rotator Structure") (A :type "Vector Structure"))
  (locals (NewLocalVar_1 :type "Array of HitResult Structure"))
  (for _array_element (`self.Scenes`)
    (bind (_hit _hitresult) (`self.TraceToGround` null (`SceneComponent.K2_GetComponentLocation` _array_element) true))
    (`self.RequestLightning` (`.Location` (`GameplayStatics.BreakHitResult` _hitresult)))))

(fn `FindTeleport`
  (returns (TeleportLocation :type "Vector Structure"))
  (locals (NewLocalVar_0 :type "Array of /Game/Mordhau/Blueprints/Characters/BP_MordhauCharacter Object Reference"))
  (bind _teleportspots (`self.TeleportSpots`))
  (`KismetArrayLibrary.Array_Shuffle` _teleportspots)
  (bind _element (`self.Random Element (Ref)` _teleportspots)
    (:`NewParam`
      (return (`KismetMathLibrary.MakeVector` (.x (`self.K2_GetActorLocation` _element)) (.y (`self.K2_GetActorLocation` _element)) (+ (.z (`self.K2_GetActorLocation` _element)) 300.0))))))

(fn `FindVolleyTarget`
  (params (AimLocation :type "Vector Structure") (AimRotation :type "Rotator Structure"))
  (returns (Success :type Boolean) (Location :type "Vector Structure"))
  (bind (_outhit _returnvalue) (`KismetSystemLibrary.LineTraceSingleForObjects` AimLocation (+ AimLocation (* (`KismetMathLibrary.GetForwardVector` AimRotation) 100000.0)) (`|MakeArray` "ObjectTypeQuery1" :!type "EObjectTypeQuery Enum") true))
  (if _returnvalue
    (return true (`.Location` (`GameplayStatics.BreakHitResult` _outhit)))
    (else
      (return false (0.0 0.0 0.0)))))

(fn `FireProjectile`
  (returns (ReturnValue :type "/HordeNPCs/Boss/BP_MageProjectile2_BOG Object Reference"))
  (bind _camerarotation1p (`self.CameraRotation1P`))
  (bind _camera (`self.Camera`))
  (`GameplayStatics.PlaySoundAtLocation` "/HordeNPCs/Boss/SC/SC_IceProjectile.SC_IceProjectile" (`self.K2_GetActorLocation`) (struct) 1.0 1.0 0.0 null null null)
  (bind _returnvalue (`|SpawnActorFromClass` "/HordeNPCs/Boss/BP_MageProjectile2_BOG.BP_MageProjectile2_BOG_C" (`KismetMathLibrary.MakeTransform` (`KismetMathLibrary.MakeVector` (.x (+ (`SceneComponent.GetSocketLocation` (`self.Mesh`) "RightHand") (* (* (`KismetMathLibrary.GetForwardVector` _camerarotation1p) (`KismetMathLibrary.Normal` (+ (`SceneComponent.GetForwardVector` _camera) (`SceneComponent.GetRightVector` _camera)))) 2.0))) (.y (+ (`SceneComponent.GetSocketLocation` (`self.Mesh`) "RightHand") (* (* (`KismetMathLibrary.GetForwardVector` _camerarotation1p) (`KismetMathLibrary.Normal` (+ (`SceneComponent.GetForwardVector` _camera) (`SceneComponent.GetRightVector` _camera)))) 2.0))) (+ (.z (+ (`SceneComponent.GetSocketLocation` (`self.Mesh`) "RightHand") (* (* (`KismetMathLibrary.GetForwardVector` _camerarotation1p) (`KismetMathLibrary.Normal` (+ (`SceneComponent.GetForwardVector` _camera) (`SceneComponent.GetRightVector` _camera)))) 2.0))) 35.0)) _camerarotation1p) "Undefined" "OverrideRootScale" null null))
  (`MordhauProjectile.InitializeProjectile` _returnvalue (`self.GetControllerIncludingVehicle`) false self)
  (`MordhauProjectile.Fire` _returnvalue)
  (return _returnvalue))

(fn `FireProjectile_0`
  (returns (ReturnValue :type "/HordeNPCs/Boss/BP_MageProjectile2_BOG Object Reference"))
  (`GameplayStatics.PlaySoundAtLocation` "/HordeNPCs/Boss/SC/SC_IceProjectile.SC_IceProjectile" (`self.K2_GetActorLocation`) (struct) 1.0 1.0 0.0 null null null)
  (bind _returnvalue (`|SpawnActorFromClass` "/HordeNPCs/Boss/BP_MageProjectile2_BOG.BP_MageProjectile2_BOG_C" (`KismetMathLibrary.MakeTransform` (`SceneComponent.GetSocketLocation` (`self.Mesh`) "RightFoot") (struct :`Pitch` -90.0)) "Undefined" "OverrideRootScale" null null))
  (`MordhauProjectile.InitializeProjectile` _returnvalue (`self.GetControllerIncludingVehicle`) false self)
  (`MordhauProjectile.Fire` _returnvalue)
  (return _returnvalue))

(fn `GetFloorWalkable`
  (returns (`Walkable Floor` :type Boolean))
  (if (`.bWalkableFloor` (break `FindFloorResult` (`CharacterMovementComponent.CurrentFloor` (`self.CharacterMovement`))))
    (return true)
    (else
      (return false))))

(fn `ModifyDamage`
  (params (DamageAmount :type "Float (double-precision)") (DamageInfo :type "MordhauDamageInfo Structure (by ref)") (EventInstigator :type "Controller Object Reference"))
  (returns (ReturnValue :type "Float (double-precision)"))
  (bind _returnvalue (`Controller.K2_GetPawn` EventInstigator))
  (if (`self.IsImmortal`)
    (return 0.0)
    (else
      (bind _returnvalue_2 (`parent.ModifyDamage` DamageAmount DamageInfo EventInstigator))
      (`/Engine/EditorBlueprintResources/StandardMacros.IsValid` _returnvalue
        (:`Is Valid`
          (cast `/HordeNPCs/Thor/BP_Thor` _returnvalue
            (:`then`
              _)
            (:`CastFailed`
              (cast `/Jötunheimr/blueprints/Npcs/Odin/BP_Odin` _returnvalue
                (:`then`
                  _)
                (:`CastFailed`
                  (cast `/HordeNPCs/BP_SpecialKnight_2` _returnvalue
                    (:`then`
                      _)
                    (:`CastFailed`
                      (cast `/HordeNPCs/BP_NormalKnight` _returnvalue
                        (:`then`
                          _)
                        (:`CastFailed`
                          (return _returnvalue_2)))))
                  (return (* _returnvalue_2 0.6))))))
          (return (* _returnvalue_2 1.6)))
        (:`Is Not Valid`
          (return DamageAmount))))))

(fn `RandomProjectiles`
  (bind _asbp_boss_ability_motion (cast `/HordeNPCs/Boss/BP_BossAbilityMotion` (`self.GetMotion`)))
  (set `MordhauMotion.EndTime` (+ (`MordhauMotion.StartTime` _asbp_boss_ability_motion) 1.0) _asbp_boss_ability_motion)
  (set `/HordeNPCs/Boss/BP_BossAbilityMotion.Stage2Time` 0.5 _asbp_boss_ability_motion)
  (`self.PlayAnim` "/Game/Mordhau/Animations/Montages/MTG_Horde_Volley_V2.MTG_Horde_Volley_V2"))

(fn `RememberStartAbilityTime`
  (params (Duration :type "Float (double-precision)"))
  (returns (OutDuration :type "Float (double-precision)"))
  (set `self.LastAbilityStartTime` (`GameplayStatics.GetTimeSeconds`))
  (bind _output_get (set `self.LastAbilityDuration` Duration))
  (return _output_get))

(fn `SpecialCooldown`
  (params (Duration :type "Float (double-precision)"))
  (`/Engine/EditorBlueprintResources/ActorMacros.Switch Has Authority`
    (:`Authority`
      (bind _output_get (set `self.NextSpecialTime` (+ Duration (`GameplayStatics.GetTimeSeconds`))))
      (`KismetSystemLibrary.PrintString` (`KismetStringLibrary.Concat_StrStr` "Special Cooldown Activated: " (`KismetStringLibrary.Conv_DoubleToString` _output_get))))))

(fn `Stage1Downfire`
  (bind _asbp_boss_ability_motion (cast `/HordeNPCs/Boss/BP_BossAbilityMotion` (`self.GetMotion`)))
  (set `MordhauMotion.EndTime` (+ (`MordhauMotion.StartTime` _asbp_boss_ability_motion) 1.0) _asbp_boss_ability_motion)
  (set `/HordeNPCs/Boss/BP_BossAbilityMotion.Stage2Time` 0.5 _asbp_boss_ability_motion)
  (`self.PlayAnim` "/Game/Mordhau/Animations/Montages/MTG_Horde_Volley_V2.MTG_Horde_Volley_V2"))

(fn `Stage1ReverseShock`
  (bind _asbp_boss_ability_motion (cast `/HordeNPCs/Boss/BP_BossAbilityMotion` (`self.GetMotion`)))
  (set `MordhauMotion.EndTime` (+ (`MordhauMotion.StartTime` _asbp_boss_ability_motion) 1.0) _asbp_boss_ability_motion)
  (set `/HordeNPCs/Boss/BP_BossAbilityMotion.Stage2Time` 0.5 _asbp_boss_ability_motion)
  (`self.PlayAnim` "/HordeNPCs/Boss/Anim/MTG_Shockwave_V2_2.MTG_Shockwave_V2_2"))

(fn `Stage2Downfire`
  (cast `/HordeNPCs/Boss/BP_BossAbilityMotion` (`self.GetMotion`))
  (`|ExecutionSequence`
    (:`then_0`
      (`/Engine/EditorBlueprintResources/ActorMacros.Switch Has Authority`
        (:`Authority`
          (bind _returnvalue (`self.FireProjectile_0`))
          (`self.TryScatterShot` _returnvalue))))))

(fn `Stage2Hookshot`
  (cast `/HordeNPCs/Boss/BP_BossAbilityMotion` (`self.GetMotion`))
  (for _ (range 3)
    (bind (_hit _hitresult) (`self.TraceToGround` null (`SceneComponent.K2_GetComponentLocation` (`|GetArrayItem` (`self.Scenes`) (`KismetMathLibrary.RandomIntegerInRange` 0 6)))))
    (if _hit
      (`self.RequestVolley` (`.Location` (`GameplayStatics.BreakHitResult` _hitresult))))))

(fn `Stage2Immortality`
  (cast `/HordeNPCs/Boss/BP_BossAbilityMotion` (`self.GetMotion`))
  (`self.RememberStartAbilityTime` 7.0)
  (`/Engine/EditorBlueprintResources/ActorMacros.Switch Has Authority`
    (:`Authority`
      (`self.SpecialCooldown` 7.0)
      (`self.TriggerImmortality`))))

(fn `Stage2Lightning`
  (cast `/HordeNPCs/Boss/BP_BossAbilityMotion` (`self.GetMotion`))
  (`|ExecutionSequence`
    (:`then_0`
      (`self.FindTargetsForLightning` (`self.CameraRotation1P`) (`self.CameraLocation1P`)))
    (:`then_1`
      (`self.SpecialCooldown` 4.0))))

(fn `Stage2Projectiles`
  (cast `/HordeNPCs/Boss/BP_BossAbilityMotion` (`self.GetMotion`))
  (`/Engine/EditorBlueprintResources/ActorMacros.Switch Has Authority`
    (:`Authority`
      (`self.FireProjectile`))))

(fn `Stage2ReverseShock`
  (`|ExecutionSequence`
    (:`then_0`
      (`GameplayStatics.PlaySoundAtLocation` "/HordeNPCs/Boss/SC/MMO_Game_Magic_Designed_Dark_Cast_07_Cue.MMO_Game_Magic_Designed_Dark_Cast_07_Cue" (`self.K2_GetActorLocation`) (struct) 1.0 1.0 0.0 null null null))
    (:`then_1`
      (set `self.RagdollForceMultIfDmgAgent` 17.0)
      (set `self.bForceRagdollIfDmgAgent` true)
      (`self.PlayAttackYell`)
      (cast `/HordeNPCs/Boss/BP_BossAbilityMotion` (`self.GetMotion`))
      (`/Engine/EditorBlueprintResources/ActorMacros.Switch Has Authority`
        (:`Authority`
          (`self.SpecialCooldown` 3.0)
          (`MordhauUtilityLibrary.MordhauApplyRadialDamageWithFalloff` 35.0 35.0 150.0 150.0 (`self.K2_GetActorLocation`) 600.0 800.0 1.0 (`|MakeArray` self :!type "Actor Object Reference") -2000.0 -2000.0 0.0 self (`AIBlueprintHelperLibrary.GetAIController` self) "ECC_Visibility" true))))))

(fn `Stage2Scatter`
  (cast `/HordeNPCs/Boss/BP_BossAbilityMotion` (`self.GetMotion`))
  (`|ExecutionSequence`
    (:`then_0`
      (`/Engine/EditorBlueprintResources/ActorMacros.Switch Has Authority`
        (:`Authority`
          (bind _returnvalue (`self.FireProjectile`))
          (`self.TryScatterShot` _returnvalue)
          (`self.SpecialCooldown` 3.0))))))

(fn `Stage2Shockwave`
  (`|ExecutionSequence`
    (:`then_0`
      (`GameplayStatics.PlaySoundAtLocation` "/Game/Mordhau/Audio/Cues/Horde/Abilities/Soundcues/SC_ABL_Shockwave.SC_ABL_Shockwave" (`self.K2_GetActorLocation`) (struct) 1.0 1.0 0.0 null null null))
    (:`then_1`
      (set `self.RagdollForceMultIfDmgAgent` 17.0)
      (set `self.bForceRagdollIfDmgAgent` true)
      (`self.PlayAttackYell`)
      (cast `/HordeNPCs/Boss/BP_BossAbilityMotion` (`self.GetMotion`))
      (`/Engine/EditorBlueprintResources/ActorMacros.Switch Has Authority`
        (:`Authority`
          (`self.SpecialCooldown` 1.0)
          (`MordhauUtilityLibrary.MordhauApplyRadialDamageWithFalloff` 25.0 25.0 150.0 150.0 (`self.K2_GetActorLocation`) 600.0 700.0 1.0 (`|MakeArray` self :!type "Actor Object Reference") 600.0 600.0 150.0 self (`AIBlueprintHelperLibrary.GetAIController` self) "ECC_Visibility" true))))))

(fn `TraceToGround`
  (params (ActorOr :type "Actor Object Reference") (Location :type "Vector Structure") (TraceComplex :type Boolean) (Type :type "EObjectTypeQuery Enum" :default "ObjectTypeQuery1") (Debug :type Boolean))
  (returns (Hit :type Boolean) (HitResult :type "HitResult Structure"))
  (locals (TraceStart :type "Vector Structure") (ActorsToIgnore :type "Array of Actor Object Reference") (DebugType :type "EDrawDebugTrace Enum"))
  (`/Engine/EditorBlueprintResources/StandardMacros.IsValid` ActorOr
    (:`Is Valid`
      (set `local.TraceStart` (`self.K2_GetActorLocation` ActorOr))
      (set `local.ActorsToIgnore` (`|MakeArray` ActorOr)))
    (:`Is Not Valid`
      (set `local.TraceStart` Location)))
  (if Debug
    (set `local.DebugType` "Persistent"))
  (bind (_outhit _returnvalue) (`KismetSystemLibrary.LineTraceSingleForObjects` null (`local.TraceStart`) (+ (`local.TraceStart`) (0.0 0.0 -999999.0)) (`|MakeArray` Type) TraceComplex (`local.ActorsToIgnore`) (`local.DebugType`)))
  (return _returnvalue _outhit))

(fn `TryScatterShot`
  (params (SourceProjectile :type "MordhauProjectile Object Reference"))
  (bind _returnvalue (`GameplayStatics.GetObjectClass` SourceProjectile))
  (bind _returnvalue_2 (`self.GetTransform` SourceProjectile))
  (bind _returnvalue_3 (`AIBlueprintHelperLibrary.GetAIController` self))
  (bind _rotation (.rotation _returnvalue_2))
  (bind _scale (.scale _returnvalue_2))
  (`/Engine/EditorBlueprintResources/ActorMacros.Switch Has Authority`
    (:`Authority`
      (if (not (`self.AvoidScattershotRecursion`))
        (set `self.AvoidScattershotRecursion` true)
        (`|ExecutionSequence`
          (:`then_0`
            (`|ExecutionSequence`
              (:`then_0`
                (bind _returnvalue_4 (`|SpawnActorFromClass` _returnvalue (`KismetMathLibrary.MakeTransform` (`KismetMathLibrary.TransformLocation` _returnvalue_2 (50.0 100.0 0.0)) (`KismetMathLibrary.MakeRotator` (.roll _rotation) (.pitch _rotation) (+ (.yaw _rotation) 10.0)) _scale) "Undefined" "OverrideRootScale" null null))
                (set `MordhauProjectile.bUsesLocalProjectileBlending` false _returnvalue_4)
                (`MordhauProjectile.InitializeProjectile` _returnvalue_4 _returnvalue_3 false self)
                (`MordhauProjectile.Fire` _returnvalue_4))
              (:`then_1`
                (bind _returnvalue_5 (`|SpawnActorFromClass` _returnvalue (`KismetMathLibrary.MakeTransform` (`KismetMathLibrary.TransformLocation` _returnvalue_2 (50.0 -100.0 0.0)) (`KismetMathLibrary.MakeRotator` (.roll _rotation) (.pitch _rotation) (+ (.yaw _rotation) -10.0)) _scale) "Undefined" "OverrideRootScale" null null))
                (set `MordhauProjectile.bUsesLocalProjectileBlending` false _returnvalue_5)
                (`MordhauProjectile.InitializeProjectile` _returnvalue_5 _returnvalue_3 false self)
                (`MordhauProjectile.Fire` _returnvalue_5))))
          (:`then_1`
            (set `self.AvoidScattershotRecursion` false)))))))

(fn `UserConstructionScript`
  (`parent.UserConstructionScript`))