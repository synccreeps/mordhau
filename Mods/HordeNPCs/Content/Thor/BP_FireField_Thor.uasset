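; Thor's fire field, which after a warmup burns actors inside it, skipping horde characters, two knight types and horde kill objectives.
; Burnable actors deep enough inside are burned by the server, with damage and tick curves driven by time spent in the field.
; Other Mordhau actors take damage every other tick, and overlapping subfields from same-age or older fields are deactivated.
; Damage is attributed to BP_Thor's default object, and audio fades out on deactivation.
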(event `self.ReceiveTick`
  (params (DeltaSeconds :type "Float (single-precision)"))
  (bind _actorpresencetickcount (`self.ActorPresenceTickCount`))
  (if (<= (+ (`self.CreatedTime`) (`self.WarmupTime`)) (`GameplayStatics.GetTimeSeconds`))
    (`parent.ReceiveTick` DeltaSeconds)
    (`/Engine/EditorBlueprintResources/StandardMacros.IsValid` self
      (:`Is Valid`
        (bind _keys (`BlueprintMapLibrary.Map_Keys` _actorpresencetickcount))
        (for _array_element _keys
          (cast `/Game/Mordhau/Blueprints/Characters/BP_HordeCharacter` _array_element
            (:`CastFailed`
              (cast `/HordeNPCs/BP_SpecialKnight_2` _array_element
                (:`CastFailed`
                  (cast `/HordeNPCs/BP_NormalKnight` _array_element
                    (:`CastFailed`
                      (cast `/Game/Mordhau/Blueprints/GameModes/Horde/Objectives/BP_HordeKillObjective` _array_element
                        (:`CastFailed`
                          (`|ExecutionSequence`
                            (:`then_0`
                              (bind _returnvalue (`self.GetComponentByClass` _array_element "/Script/Mordhau.BurnableComponent"))
                              (`/Engine/EditorBlueprintResources/StandardMacros.IsValid` _returnvalue
                                (:`Is Valid`
                                  (`BurnableComponent.SetOnFire` _returnvalue self))))
                            (:`then_1`
                              (`/Engine/EditorBlueprintResources/ActorMacros.Switch Has Authority`
                                (:`Authority`
                                  (`/Engine/EditorBlueprintResources/StandardMacros.IsValid` _returnvalue
                                    (:`Is Valid`
                                      (bind _returnvalue_2 (`self.ComputeDistanceIntoField` (`self.K2_GetActorLocation` _array_element)))
                                      (if (>= _returnvalue_2 200.0)
                                        (bind (_value _returnvalue_3) (`BlueprintMapLibrary.Map_Find` _actorpresencetickcount _array_element))
                                        (bind _returnvalue_4 (* (`self.GetActorTickInterval`) (`KismetMathLibrary.Conv_IntToDouble` _value)))
                                        (`BurnableComponent.StartBurning` _returnvalue 0.5 (`CurveFloat.GetFloatValue` (`self.CharFireDmgByTime`) _returnvalue_4) (`CurveFloat.GetFloatValue` (`self.CharFireTickByTime`) _returnvalue_4) (`self.GetAgent`) (`self.InstigatorController`))
                                        (else
                                          (`BlueprintMapLibrary.Map_Remove` _actorpresencetickcount _array_element))))
                                    (:`Is Not Valid`
                                      (bind _asmordhau_actor (cast `MordhauActor` _array_element)
                                        (:`then`
                                          (if _returnvalue_3
                                            (if (== (mod _value 2) 0)
                                              (bind _asbp_destroyable_actor (cast `/Game/Mordhau/Blueprints/Interactables/Environment/BP_DestroyableActor` _asmordhau_actor)
                                                (:`then`
                                                  (bind _returnvalue_5 (`self.ComputeDistanceIntoField` (`PrimitiveComponent.GetClosestPointOnCollision` (`/Game/Mordhau/Blueprints/Interactables/Environment/BP_DestroyableActor.StaticMesh` _asbp_destroyable_actor) (`self.GetFieldBoundsCenter`) "None")))
                                                  (if (>= _returnvalue_5 250.0)
                                                    (`GameplayStatics.ApplyDamage` _asmordhau_actor (`self.OtherDamage`) (`self.InstigatorController`) (`self.GetAgent`) :!label _label)))
                                                (:`CastFailed`
                                                  (bind _returnvalue_6 (`self.ComputeDistanceIntoField` (`self.K2_GetActorLocation` _asmordhau_actor)))
                                                  (if (>= _returnvalue_6 250.0)
                                                    (goto _label)))))))
                                        (:`CastFailed`
                                          (if (== _value 1)
                                            (bind _asbp_fire_sub_field_thor (cast `/HordeNPCs/Thor/BP_FireSubField_Thor` _array_element))
                                            (bind _returnvalue_7 (`self.ComputeDistanceIntoField` (`self.K2_GetActorLocation` _asbp_fire_sub_field_thor)))
                                            (bind _returnvalue_8 (`SubField.GetMaster` _asbp_fire_sub_field_thor))
                                            (if (and (<= (`MasterField.CreatedTime` _returnvalue_8) (`self.CreatedTime`)) (>= _returnvalue_7 225.0))
                                              (`SubField.DeactivateSubField` _asbp_fire_sub_field_thor))))))))))))))))))))))))

(event `self.BeginFieldDeactivation`
  (`parent.BeginFieldDeactivation`)
  (`AudioComponent.FadeOut` (`self.Audio`) 1.5 0.0 "Linear"))

(fn `GetAgent`
  (returns (Agent :type "Actor Object Reference"))
  (return (`MordhauUtilityLibrary.GetDefaultActor` "/HordeNPCs/Thor/BP_Thor.BP_Thor_C")))

(fn `UserConstructionScript`
  (`parent.UserConstructionScript`))