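; Thor lightning strike actor that hits once on BeginPlay, with unused delayed and repeating-volley logic left disconnected.
; On authority it applies radial damage sparing friendlies and the instigator's pawn, spawns a fire field, then expires shortly after.
; A downward trace places the Niagara bolt, also authority-only, and gates passing the instigator controller to the fire field.
; The decal is removed after a short delay.
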(event `self.ReceiveBeginPlay`
  (`|ExecutionSequence`
    (:`then_0`
      (`/Engine/EditorBlueprintResources/ActorMacros.Switch Has Authority`
        (:`Authority`
          (`self.DamageTick`)
          (`self.SetLifeSpan` 2.0))))
    (:`then_1`
      (`KismetSystemLibrary.Delay` 1.0)
      (`ActorComponent.K2_DestroyComponent` (`self.Decal`)))))

(event `DamageTick`
  (bind _instigatorcontroller (`self.InstigatorController`))
  (bind _returnvalue (`SceneComponent.K2_GetComponentLocation` (`self.MordhauScene`)))
  (bind _returnvalue_2 (`Controller.K2_GetPawn` _instigatorcontroller))
  (`MordhauUtilityLibrary.MordhauApplyRadialDamageWithFalloff` 15.0 15.0 200.0 200.0 _returnvalue 350.0 400.0 1.0 (`|MakeArray` _returnvalue_2 :!type "Actor Object Reference") 0.0 0.0 50.0 _returnvalue_2 _instigatorcontroller "ECC_Visibility" true)
  (bind _returnvalue_3 (`|SpawnActorFromClass` "/HordeNPCs/Thor/BP_FireField_Thor.BP_FireField_Thor_C" (`KismetMathLibrary.MakeTransform` _returnvalue) "AlwaysSpawn" "OverrideRootScale" null null))
  (bind (_hit _hitresult) (`self.TraceToGround` self (0.0 0.0 0.0) true))
  (if _hit
    (`NiagaraFunctionLibrary.SpawnSystemAtLocation` "/HordeNPCs/Boss/Particle/NS_Mage_LIghtning_Bolt.NS_Mage_LIghtning_Bolt" (`.Location` (`GameplayStatics.BreakHitResult` _hitresult)))
    (`/Engine/EditorBlueprintResources/StandardMacros.IsValid` _returnvalue_3
      (:`Is Valid`
        (set `/Game/Mordhau/Blueprints/Fields/BP_MasterField.InstigatorController` (`self.InstigatorController`) _returnvalue_3)))))

(fn `TraceToGround`
  (params (ActorOr :type "Actor Object Reference") (Location :type "Vector Structure") (TraceComplex :type Boolean) (Type :type "EObjectTypeQuery Enum" :default "ObjectTypeQuery1") (Debug :type Boolean))
  (returns (Hit :type Boolean) (HitResult :type "HitResult Structure"))
  (locals (TraceStart :type "Vector Structure") (ActorsToIgnore :type "Array of Actor Object Reference") (DebugType :type "EDrawDebugTrace Enum"))
  (`/Engine/EditorBlueprintResources/StandardMacros.IsValid` ActorOr
    (:`Is Valid`
      (set `local.TraceStart` (`self.K2_GetActorLocation` ActorOr))
      (set `local.ActorsToIgnore` (`|MakeArray` ActorOr)))
    (:`Is Not Valid`
      (set `local.TraceStart` Location)))
  (if Debug
    (set `local.DebugType` "Persistent"))
  (bind (_outhit _returnvalue) (`KismetSystemLibrary.LineTraceSingleForObjects` null (`local.TraceStart`) (+ (`local.TraceStart`) (0.0 0.0 -999999.0)) (`|MakeArray` Type) TraceComplex (`local.ActorsToIgnore`) (`local.DebugType`)))
  (return _returnvalue _outhit))

(fn `UserConstructionScript`)