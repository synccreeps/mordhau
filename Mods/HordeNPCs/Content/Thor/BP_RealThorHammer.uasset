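; Thor's hammer weapon Blueprint that adds a lightning impact and knockback to its parent's hit handling.
; OnHit spawns a Niagara lightning effect at the impact point, then calls Launch for non-boss horde enemies on team 1.
; Launch pushes the enemy upward and along its own forward vector, repeats the push after a short delay, then triggers a replicated trip with knockback.
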(event `Launch`
  (params (Char :type "AdvancedCharacter Object Reference"))
  (bind _asbp_horde_enemy (cast `/Game/Mordhau/Blueprints/GameModes/Horde/BP_HordeEnemy` Char))
  (bind _newparam (`self.LaunchVelocity` _asbp_horde_enemy))
  (`Character.LaunchCharacter` _asbp_horde_enemy _newparam false false)
  (`KismetSystemLibrary.Delay` 0.1)
  (`Character.LaunchCharacter` _asbp_horde_enemy _newparam false false)
  (`KismetSystemLibrary.Delay` 0.2)
  (`/Game/Mordhau/Blueprints/Characters/BP_MordhauCharacter.ReplicatedTripWithKnockback` _asbp_horde_enemy))

(event `self.OnHit`
  (params (Actor :type "Actor Object Reference") (Move :type "EAttackMove Enum" :default "RightStrike") (Bone :type Name) (WorldLocation :type "Vector Structure (by ref)") (Tier :type Byte) (SurfaceType :type Byte))
  (`parent.OnHit` Actor Move Bone WorldLocation Tier SurfaceType)
  (`NiagaraFunctionLibrary.SpawnSystemAtLocation` "/HordeNPCs/Thor/NS_LightningShoot_Hit.NS_LightningShoot_Hit" WorldLocation)
  (bind _asbp_horde_enemy (cast `/Game/Mordhau/Blueprints/GameModes/Horde/BP_HordeEnemy` Actor))
  (if (== (`AdvancedCharacter.Team` _asbp_horde_enemy) 1)
    (if (not (`/Game/Mordhau/Blueprints/GameModes/Horde/BP_HordeEnemy.IsBoss` _asbp_horde_enemy))
      (`self.Launch` _asbp_horde_enemy))))

(fn `LaunchVelocity`
  (params (Char :type "AdvancedCharacter Object Reference"))
  (returns (NewParam :type "Vector Structure"))
  (return (`KismetMathLibrary.MakeVector` (* (.x (`self.GetActorForwardVector` Char)) 300.0) (* (.y (`self.GetActorForwardVector` Char)) 300.0) (+ (.z (`self.GetActorForwardVector` Char)) 150.0))))

(fn `UserConstructionScript`
  (`parent.UserConstructionScript`))