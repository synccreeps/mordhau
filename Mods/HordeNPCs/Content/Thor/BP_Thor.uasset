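; Thor, an AI-controlled combat character with three two-stage specials timed through BP_ThorAbilityMotion: ragdolling radial shockwave, lightning volleys and downward scattershot projectile.
; Looping timers trigger two specials while an enemy is perceived, one after teleporting upward, and are cleared on death.
; The TotalHits RepNotify fires another special after enough hits from BP_MordhauAIController sources, then resets.
; Lightning spawns at ground traces beneath five scene components.
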(event `CustomEvent_0`
  (bind _asbp_mordhau_aicontroller (cast `/Game/Mordhau/AI/BP_MordhauAIController` (`self.GetControllerIncludingVehicle`)))
  (bind _returnvalue (`MordhauAIController.PerceivesEnemy` _asbp_mordhau_aicontroller))
  (if _returnvalue
    (`self.K2_TeleportTo` (+ (`self.K2_GetActorLocation`) (0.0 0.0 800.0)))
    (`self.DoSpecialAbility` 2)))

(event `self.ReceiveBeginPlay`
  (`parent.ReceiveBeginPlay`)
  (set `self.Scenes` (`|MakeArray` (`self.MordhauScene1`) (`self.MordhauScene2`) (`self.MordhauScene3`) (`self.MordhauScene4`) (`self.MordhauScene5`)))
  (bind _returnvalue (`KismetSystemLibrary.K2_SetTimerDelegate` (delegate `CustomEvent_0`) 6.235 true))
  (set `self.NewVar_0` _returnvalue)
  (bind _returnvalue_2 (`KismetSystemLibrary.K2_SetTimerDelegate` (delegate `CustomEvent_1`) 10.577 true))
  (set `self.NewVar_1` _returnvalue_2))

(event `CustomEvent_1`
  (bind _asbp_mordhau_aicontroller (cast `/Game/Mordhau/AI/BP_MordhauAIController` (`self.GetControllerIncludingVehicle`)))
  (bind _returnvalue (`MordhauAIController.PerceivesEnemy` _asbp_mordhau_aicontroller))
  (if _returnvalue
    (`self.DoSpecialAbility` 1)))

(event `self.OnTookDamage`
  (params (bWillKill :type Boolean) (Type :type "EMordhauDamageType Enum" :default "Generic") (SubType :type Byte) (Bone :type "Name (by ref)") (Point :type "Vector Structure (by ref)") (Source :type "Actor Object Reference") (Agent :type "Actor Object Reference"))
  (`parent.OnTookDamage` bWillKill Type SubType Bone Point Source Agent)
  (cast `/Game/Mordhau/AI/BP_MordhauAIController` Source)
  (set `self.TotalHits` (+ (`self.TotalHits`) 1)))

(event `RequestLightning`
  (params (Location :type "Vector Structure"))
  (bind _returnvalue (`AIBlueprintHelperLibrary.GetAIController` self))
  (cast `/HordeNPCs/Thor/BP_ThorAbilityMotion` (`self.GetMotion`))
  (bind _returnvalue_2 (`|SpawnActorFromClass` "/HordeNPCs/Thor/BP_LightningVolley_Thor.BP_LightningVolley_Thor_C" (`KismetMathLibrary.MakeTransform` Location) "Undefined" "OverrideRootScale" null _returnvalue self))
  (set `/HordeNPCs/Thor/BP_LightningVolley_Thor.DamageMultiplier` 0.5 _returnvalue_2)
  (set `/HordeNPCs/Thor/BP_LightningVolley_Thor.InstigatorController` _returnvalue _returnvalue_2))

(event `self.OnDied`
  (params (Angle :type "Float (single-precision)") (Type :type "EMordhauDamageType Enum" :default "Generic") (SubType :type Byte) (Bone :type Name) (Point :type "Vector Structure") (Source :type "Actor Object Reference") (Agent :type "Actor Object Reference"))
  (`parent.OnDied` Angle Type SubType Bone Point Source Agent)
  (`KismetSystemLibrary.K2_ClearAndInvalidateTimerHandle` (`self.NewVar_0`))
  (`KismetSystemLibrary.K2_ClearAndInvalidateTimerHandle` (`self.NewVar_1`))
  (`SceneComponent.SetHiddenInGame` (`self.NS_Electrictotem_Aura`) true false))

(fn `BeginLightning`
  (bind _asbp_thor_ability_motion (cast `/HordeNPCs/Thor/BP_ThorAbilityMotion` (`self.GetMotion`)))
  (set `MordhauMotion.EndTime` (+ (`MordhauMotion.StartTime` _asbp_thor_ability_motion) 1.0) _asbp_thor_ability_motion)
  (set `/HordeNPCs/Thor/BP_ThorAbilityMotion.Stage2Time` 0.5 _asbp_thor_ability_motion)
  (`self.PlayAnim` "/Game/Mordhau/Animations/Montages/MTG_Horde_Volley_V2.MTG_Horde_Volley_V2"))

(fn `BeginShockwave`
  (bind _asbp_thor_ability_motion (cast `/HordeNPCs/Thor/BP_ThorAbilityMotion` (`self.GetMotion`)))
  (set `MordhauMotion.EndTime` (+ (`MordhauMotion.StartTime` _asbp_thor_ability_motion) 1.0) _asbp_thor_ability_motion)
  (set `/HordeNPCs/Thor/BP_ThorAbilityMotion.Stage2Time` 0.5 _asbp_thor_ability_motion)
  (`self.PlayAnim` "/HordeNPCs/Thor/ANIM_ThorShockwave.ANIM_ThorShockwave"))

(fn `FindTargetsForLightning`
  (locals (NewLocalVar_1 :type "Array of HitResult Structure"))
  (for _array_element (`self.Scenes`)
    (bind (_hit _hitresult) (`self.TraceToGround` null (`SceneComponent.K2_GetComponentLocation` _array_element) true))
    (`self.RequestLightning` (`.Location` (`GameplayStatics.BreakHitResult` _hitresult)))))

(fn `FireProjectile_Down`
  (returns (ReturnValue :type "MordhauProjectile Object Reference"))
  (bind _returnvalue (`|SpawnActorFromClass` "/HordeNPCs/Thor/BP_ThorProjectile_Down.BP_ThorProjectile_Down_C" (`KismetMathLibrary.MakeTransform` (`SceneComponent.GetSocketLocation` (`self.Mesh`) "RightFoot") (struct :`Pitch` -90.0)) "Undefined" "OverrideRootScale" null null))
  (`MordhauProjectile.InitializeProjectile` _returnvalue (`self.GetControllerIncludingVehicle`) false self)
  (`MordhauProjectile.Fire` _returnvalue)
  (return _returnvalue))

(fn `NewFunction_0`
  (`/Engine/EditorBlueprintResources/ActorMacros.Switch Has Authority`
    (:`Authority`
      (set `self.TotalHits` 0))))

(fn `OnRep_TotalHits`
  (if (>= (`self.TotalHits`) 15)
    (bind _success (`self.DoSpecialAbility` 0))
    (if _success
      (`self.NewFunction_0`))))

(fn `Stage1Downfire`
  (bind _asbp_thor_ability_motion (cast `/HordeNPCs/Thor/BP_ThorAbilityMotion` (`self.GetMotion`)))
  (set `MordhauMotion.EndTime` (+ (`MordhauMotion.StartTime` _asbp_thor_ability_motion) 1.0) _asbp_thor_ability_motion)
  (set `/HordeNPCs/Thor/BP_ThorAbilityMotion.Stage2Time` 0.5 _asbp_thor_ability_motion)
  (`self.PlayAnim` "/Game/Mordhau/Animations/Montages/MTG_Horde_Volley_V2.MTG_Horde_Volley_V2"))

(fn `Stage2Downfire`
  (cast `/HordeNPCs/Thor/BP_ThorAbilityMotion` (`self.GetMotion`))
  (`/Engine/EditorBlueprintResources/ActorMacros.Switch Has Authority`
    (:`Authority`
      (bind _returnvalue (`self.FireProjectile_Down`))
      (`self.TryScatterShot` _returnvalue))))

(fn `Stage2Lightning`
  (cast `/HordeNPCs/Thor/BP_ThorAbilityMotion` (`self.GetMotion`))
  (`|ExecutionSequence`
    (:`then_0`
      (`self.FindTargetsForLightning`))
    (:`then_1`
      (`self.SpecialCooldown` 4.0))))

(fn `Stage2Shockwave`
  (set `self.RagdollForceMultIfDmgAgent` 17.0)
  (set `self.bForceRagdollIfDmgAgent` true)
  (`self.PlayAttackYell`)
  (cast `/HordeNPCs/Thor/BP_ThorAbilityMotion` (`self.GetMotion`))
  (`/Engine/EditorBlueprintResources/ActorMacros.Switch Has Authority`
    (:`Authority`
      (`MordhauUtilityLibrary.MordhauApplyRadialDamageWithFalloff` 15.0 15.0 150.0 150.0 (`self.K2_GetActorLocation`) 600.0 700.0 1.0 (`|MakeArray` self :!type "Actor Object Reference") 600.0 600.0 400.0 self (`AIBlueprintHelperLibrary.GetAIController` self) "ECC_Visibility" true))))

(fn `UserConstructionScript`
  (`parent.UserConstructionScript`))