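; Motion for Thor's abilities in Mordhau, driving a two-stage Shockwave, Lightning or Downfire on the owning BP_Thor.
; On begin it resets the character's additive override type and uses the net motion's MotionParam0 to pick which first-stage function to call.
; Tick counts down Stage2Time, then advances CurrentStage and calls the matching second-stage function once, re-reading the same parameter.
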(event `self.OnBegin`
  (`parent.OnBegin`)
  (bind _asbp_thor (cast `/HordeNPCs/Thor/BP_Thor` (`self.GetOwnerMordhauCharacter`)))
  (`AdvancedCharacter.ResetAdditiveOverrideType` _asbp_thor)
  (switch `int` (`KismetMathLibrary.Conv_ByteToInt` (`.MotionParam0` (break `NetMotion` (`MordhauCharacter.GetCurrentNetMotion` _asbp_thor))))
    (:`0`
      (`/HordeNPCs/Thor/BP_Thor.BeginShockwave` _asbp_thor))
    (:`1`
      (`/HordeNPCs/Thor/BP_Thor.BeginLightning` _asbp_thor))
    (:`2`
      (`/HordeNPCs/Thor/BP_Thor.Stage1Downfire` _asbp_thor))))

(event `self.OnTick`
  (params (DeltaTime :type "Float (single-precision)"))
  (`parent.OnTick` DeltaTime)
  (if (== (`self.CurrentStage`) 0)
    (bind _output_get (set `self.Stage2Time` (- (`self.Stage2Time`) DeltaTime)))
    (if (<= _output_get 0.0)
      (set `self.CurrentStage` 1)
      (bind _asbp_thor (cast `/HordeNPCs/Thor/BP_Thor` (`self.GetOwnerMordhauCharacter`)))
      (switch `int` (`KismetMathLibrary.Conv_ByteToInt` (`.MotionParam0` (break `NetMotion` (`MordhauCharacter.GetCurrentNetMotion` _asbp_thor))))
        (:`0`
          (`/HordeNPCs/Thor/BP_Thor.Stage2Shockwave` _asbp_thor))
        (:`1`
          (`/HordeNPCs/Thor/BP_Thor.Stage2Lightning` _asbp_thor))
        (:`2`
          (`/HordeNPCs/Thor/BP_Thor.Stage2Downfire` _asbp_thor))))))