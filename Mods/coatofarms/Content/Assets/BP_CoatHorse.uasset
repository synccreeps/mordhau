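; BP_CoatHorse is a Blueprint that displays a temporary text message above its head.
; TextAboveHeadClient sets and shows the TextRender text, then hides it after a ten-second delay.
; Every tick, the text's X axis is turned to point directly away from the first player's camera, so it tracks that camera's position.
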(event `TextAboveHeadClient`
  (params (Message :type String))
  (bind _textrender (`self.TextRender`))
  (`SceneComponent.SetVisibility` _textrender true false)
  (`TextRenderComponent.K2_SetText` _textrender (`KismetTextLibrary.Conv_StringToText` Message))
  (`KismetSystemLibrary.Delay` 10.0)
  (`SceneComponent.SetVisibility` _textrender false false))

(event `self.ReceiveTick`
  (params (DeltaSeconds :type "Float (single-precision)"))
  (bind _returnvalue (`GameplayStatics.GetPlayerCameraManager` 0))
  (bind _textrender (`self.TextRender`))
  (`|ExecutionSequence`
    (:`then_0`
      (`/Engine/EditorBlueprintResources/StandardMacros.IsValid` _returnvalue
        (:`Is Valid`
          (`SceneComponent.K2_SetWorldRotation` _textrender (`KismetMathLibrary.MakeRotFromX` (- (`SceneComponent.K2_GetComponentLocation` _textrender) (`self.K2_GetActorLocation` _returnvalue))) false false))))))

(fn `UserConstructionScript`
  (`parent.UserConstructionScript`))