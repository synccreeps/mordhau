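; BP_DestroyableGate is a gate that MC_coatofarms characters can break and repair through damage events.
; While intact, ten hits from such a character destroy it; while destroyed, three left or right BP_SmithHammer strikes restore it.
; The IsDestroyed RepNotify swaps the two meshes' visibility and toggles the main mesh's collision.
; Repair resets TimesHit but not TotalHits, so later repairs need only one hammer strike.
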(event `self.ReceiveAnyDamage`
  (params (Damage :type "Float (single-precision)") (DamageType :type "DamageType Object Reference") (InstigatedBy :type "Controller Object Reference") (DamageCauser :type "Actor Object Reference"))
  (if (`SceneComponent.IsVisible` (`self.StaticMesh`))
    (cast `/coatofarms/Assets/MC_coatofarms` DamageCauser)
    (bind _output_get (set `self.TimesHit` (+ (stale _output_get) 1)))
    (if (>= (`self.TimesHit`) 10)
      (set `self.IsDestroyed` true))
    (else
      (bind _asmc_coatofarms (cast `/coatofarms/Assets/MC_coatofarms` DamageCauser))
      (bind _asattack_motion (cast `AttackMotion` (`MordhauCharacter.Motion` _asmc_coatofarms)))
      (bind _move (`AttackMotion.Move` _asattack_motion))
      (if (or (`|EnumEquality` _move "RightStrike") (`|EnumEquality` _move "LeftStrike"))
        (if (== (`GameplayStatics.GetObjectClass` (`AttackMotion.Weapon` _asattack_motion)) "/Game/Mordhau/Blueprints/Equipment/Weapons/Specific/OneHanded/BP_SmithHammer.BP_SmithHammer_C")
          (bind _output_get_2 (set `self.Total Hits` (+ (`self.Total Hits`) 1)))
          (if (>= _output_get_2 3)
            (set `self.IsDestroyed` false)
            (set `self.TimesHit` 0)))))))

(fn `OnRep_IsDestroyed`
  (bind _staticmesh (`self.StaticMesh`))
  (bind _staticmesh_2 (`self.StaticMesh`))
  (if (`self.IsDestroyed`)
    (`SceneComponent.SetVisibility` _staticmesh_2 false false)
    (`PrimitiveComponent.SetCollisionEnabled` _staticmesh_2 "NoCollision")
    (`SceneComponent.SetVisibility` (`self.StaticMesh1`) true false)
    (else
      (`SceneComponent.SetVisibility` _staticmesh true false)
      (`PrimitiveComponent.SetCollisionEnabled` _staticmesh "QueryAndPhysics")
      (`SceneComponent.SetVisibility` (`self.StaticMesh1`) false false))))

(fn `UserConstructionScript`
  (`parent.UserConstructionScript`))