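; Coat of Arms game mode that manages player factions and persists them with player inventories.
; Faction events create, rename, delete and edit membership in a map, then refresh affected name prefixes through player controllers matched by PlayFab ID.
; BeginPlay loads the CoAData save, then loops an autosave every ten seconds.
; Each save merges inventories from controllers with valid data into stored records, preserving entries for absent players.
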(event `ChangeAllFactionPlayersNamePrefix`
  (params (Faction :type String) (ClearName :type Boolean))
  (bind _keys (`BlueprintMapLibrary.Map_Keys` (`.AllMembers_8_630C94A04817D994D40C6BBC740E7B50` (break `/coatofarms/Assets/FactionsDataStruct` (`BlueprintMapLibrary.Map_Find` (`self.Factions`) Faction)))))
  (for _array_element _keys
    (`self.ChangePlayerNamePrefix` _array_element ClearName)))

(event `LoadData`
  ;[1 1 1] Load data
  (bind _returnvalue (`GameplayStatics.DoesSaveGameExist` "CoAData"))
  (if _returnvalue
    (bind _returnvalue_2 (`GameplayStatics.LoadGameFromSlot` "CoAData"))
    (bind _ascoatsavegame (cast `/coatofarms/Assets/coatsavegame` _returnvalue_2))
    (set `self.PlayerData` (`/coatofarms/Assets/coatsavegame.playerdata` _ascoatsavegame))
    (set `self.Factions` (`/coatofarms/Assets/coatsavegame.Factions` _ascoatsavegame))))

(event `ChangePlayerNamePrefix`
  (params (PlayerID :type String) (ClearName :type Boolean))
  (bind _outactors (`GameplayStatics.GetAllActorsOfClass` "/coatofarms/Assets/PC_coatofarms.PC_coatofarms_C"))
  (for _array_element _outactors
    (if (`KismetStringLibrary.EqualEqual_StrStr` (`MordhauPlayerController.GetPlayFabID` _array_element) PlayerID)
      (`/coatofarms/Assets/PC_coatofarms.ChangeNameFactionPrefix` _array_element ClearName)
      (break))))

(event `CreateFaction`
  (params (FactionName :type String) (FactionOwnerID :type String) (FactionOwnerName :type String))
  ;[1 1 1] Faction Create Rename Delete
  (`BlueprintMapLibrary.Map_Add` (`self.Factions`) FactionName (make `/coatofarms/Assets/FactionsDataStruct` FactionName FactionOwnerID (`|MakeMap` FactionOwnerID FactionOwnerName)))
  (`self.ChangePlayerNamePrefix` FactionOwnerID))

(event `RenameFaction`
  (params (FactionOldName :type String) (FactionNewName :type String))
  (bind _factions (`self.Factions`))
  (bind (_factionname _factionleaderid _allmembers) (break `/coatofarms/Assets/FactionsDataStruct` (`BlueprintMapLibrary.Map_Find` _factions FactionOldName)))
  ;[1 1 1] Faction Create Rename Delete
  (`BlueprintMapLibrary.Map_Add` _factions FactionNewName (make `/coatofarms/Assets/FactionsDataStruct` FactionNewName _factionleaderid _allmembers))
  (`BlueprintMapLibrary.Map_Remove` _factions FactionOldName)
  (`self.ChangeAllFactionPlayersNamePrefix` FactionNewName))

(event `DeleteFaction`
  (params (FactionName :type String))
  ;[1 1 1] Faction Create Rename Delete
  (`self.ChangeAllFactionPlayersNamePrefix` FactionName true)
  (`BlueprintMapLibrary.Map_Remove` (`self.Factions`) FactionName))

(event `AddMemberFaction`
  (params (`Faction Name` :type String) (NewMemberID :type String) (NewMemberName :type String))
  (bind _factions (`self.Factions`))
  (bind (_factionname _factionleaderid _allmembers) (break `/coatofarms/Assets/FactionsDataStruct` (`BlueprintMapLibrary.Map_Find` _factions `Faction Name`)))
  ;[1 1 1] Faction Add/Remove Member
  (bind _output_get (set `self.TemporaryOldMembers` _allmembers))
  (`BlueprintMapLibrary.Map_Add` _output_get NewMemberID NewMemberName)
  (`BlueprintMapLibrary.Map_Add` _factions `Faction Name` (make `/coatofarms/Assets/FactionsDataStruct` _factionname _factionleaderid (`self.TemporaryOldMembers`)))
  (`self.ChangePlayerNamePrefix` NewMemberID))

(event `RemoveMemberFaction`
  (params (FactionName :type String) (MemberID :type String))
  (bind _factions (`self.Factions`))
  (bind (_factionname _factionleaderid _allmembers) (break `/coatofarms/Assets/FactionsDataStruct` (`BlueprintMapLibrary.Map_Find` _factions FactionName)))
  ;[1 1 1] Faction Add/Remove Member
  (bind _output_get (set `self.TemporaryOldMembers` _allmembers))
  (`BlueprintMapLibrary.Map_Remove` _output_get MemberID)
  (`BlueprintMapLibrary.Map_Add` _factions FactionName (make `/coatofarms/Assets/FactionsDataStruct` _factionname _factionleaderid (`self.TemporaryOldMembers`)))
  (`self.ChangePlayerNamePrefix` MemberID))

(event `self.ReceiveBeginPlay`
  (`parent.ReceiveBeginPlay`)
  (`self.LoadData`)
  ;[1 1 1] Save data
  (`KismetSystemLibrary.Delay` 10.0 :!label _label)
  (bind _returnvalue (`GameplayStatics.CreateSaveGameObject` "/coatofarms/Assets/coatsavegame.coatsavegame_C"))
  (bind _playerdataout (`self.NewPlayerData`))
  (set `/coatofarms/Assets/coatsavegame.playerdata` _playerdataout _returnvalue)
  (set `self.PlayerData` _playerdataout)
  (set `/coatofarms/Assets/coatsavegame.Factions` (`self.Factions`) _returnvalue)
  (`GameplayStatics.SaveGameToSlot` _returnvalue "CoAData")
  (goto _label))

(fn `NewPlayerData`
  (returns (PlayerDataOut :type "Map of String to /coatofarms/Assets/playerdatastruct Structure"))
  (locals (TempData :type "Map of String to /coatofarms/Assets/playerdatastruct Structure"))
  (bind _playerdata (`self.PlayerData`))
  (bind _outactors (`GameplayStatics.GetAllActorsOfClass` "/coatofarms/Assets/PC_coatofarms.PC_coatofarms_C"))
  (for _array_element _outactors
    (bind _hasvaliddata (`/coatofarms/Assets/PC_coatofarms.HasValidData` _array_element))
    (bind _returnvalue (`MordhauPlayerController.GetPlayFabID` _array_element))
    (bind (_value _returnvalue_2) (`BlueprintMapLibrary.Map_Find` (`self.PlayerData`) _returnvalue))
    (if (or _hasvaliddata _returnvalue_2)
      (`BlueprintMapLibrary.Map_Add` (`local.TempData`) _returnvalue (select `bool` _hasvaliddata :`false` _value :`true` (make `/coatofarms/Assets/playerdatastruct` (`/coatofarms/Assets/PC_coatofarms.Inventory` _array_element))))))
  (bind _keys (`BlueprintMapLibrary.Map_Keys` _playerdata))
  (for _array_element_2 _keys
    (if (not (`.ReturnValue` (`BlueprintMapLibrary.Map_Find` (`local.TempData`) _array_element_2)))
      (`BlueprintMapLibrary.Map_Add` (`local.TempData`) _array_element_2 (`BlueprintMapLibrary.Map_Find` _playerdata _array_element_2))))
  (return (`local.TempData`)))

(fn `UserConstructionScript`
  (`parent.UserConstructionScript`))