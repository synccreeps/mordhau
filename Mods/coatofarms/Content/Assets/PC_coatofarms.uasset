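; Player controller for the Coat of Arms Mordhau mod, handling player inventory, faction name tags, overhead chat and an emblem toggle.
; On join, the server loads inventory from game mode PlayerData by PlayFab ID and syncs it to the client as key/value arrays.
; Later changes are mirrored client-side, updating lockpicks and pickup widgets.
; On possess, rank items in the inventory gate tiered armour and crowns, overriding disallowed wearables.
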(event `SyncInventoryClient`
  (params (ItemTypes :type "Array of String") (ItemAmounts :type "Array of Integer"))
  ;[1 1 1] Set whole inventory on client
  (for (_array_element _array_index) ItemTypes
    (`BlueprintMapLibrary.Map_Add` (`self.Inventory`) _array_element (`|GetArrayItem` ItemAmounts _array_index))))

(event `InventoryUpdate`
  (params (ItemType :type String) (ItemAmount :type Integer))
  (bind _inventory (`self.Inventory`))
  (bind (_value _returnvalue) (`BlueprintMapLibrary.Map_Find` _inventory ItemType))
  ;[1 1 1] Update Inventory on Server
  (`KismetSystemLibrary.PrintString` "InventoryUpdate" true true (struct :`R` 0.5625 :`B` 0.024648 :`A` 1.0) 5.0)
  (if _returnvalue
    (`BlueprintMapLibrary.Map_Add` _inventory ItemType (+ _value ItemAmount))
    (else
      (`BlueprintMapLibrary.Map_Add` _inventory ItemType ItemAmount)))
  (if (< _value 0)
    (`BlueprintMapLibrary.Map_Add` _inventory ItemType 0))
  (`self.InventoryUpdateClient` ItemType ItemAmount))

(event `InventoryUpdateClient`
  (params (ItemType :type String) (ItemAmount :type Integer))
  (bind _inventory (`self.Inventory`))
  (bind (_value _returnvalue) (`BlueprintMapLibrary.Map_Find` _inventory ItemType))
  (bind (_value_2 _returnvalue_2) (`BlueprintMapLibrary.Map_Find` _inventory "Lockpick"))
  ;[1 1 1] Update Inventory on Client
  (`|ExecutionSequence`
    (:`then_0`
      (if _returnvalue
        (`BlueprintMapLibrary.Map_Add` _inventory ItemType (+ _value ItemAmount))
        (else
          (`BlueprintMapLibrary.Map_Add` _inventory ItemType ItemAmount)))
      (if (< _value 0)
        (`BlueprintMapLibrary.Map_Add` _inventory ItemType 0)))
    (:`then_1`
      (if _returnvalue_2
        (bind _asmc_coatofarms (cast `/coatofarms/Assets/MC_coatofarms` (`self.K2_GetPawn`)))
        (set `/coatofarms/Assets/coat/LockPicking/Blueprints/BP_LockPickingComponent.LockPicks` _value_2 (`/coatofarms/Assets/MC_coatofarms.BP_LockPickingComponent` _asmc_coatofarms))))
    (:`then_2`
      (if (> ItemAmount 0)
        (bind _returnvalue_3 (`|CreateWidget` "/coatofarms/Assets/InventoryUpdateWidget.InventoryUpdateWidget_C"))
        (`UserWidget.AddToViewport` _returnvalue_3 0)
        (`/coatofarms/Assets/InventoryUpdateWidget.ReceivedItems` _returnvalue_3 ItemType ItemAmount)))))

(event `BuildingInventoryUpdate`
  (params (Item :type String) (ItemAmount :type Integer))
  (`self.InventoryUpdate` Item ItemAmount))

(event `self.ReceiveBeginPlay`
  (bind _returnvalue (`self.GetPlayFabID`))
  ;[1 1 1] Load inventory on join
  (`parent.ReceiveBeginPlay`)
  (`KismetSystemLibrary.Delay` 5.0)
  (`/Engine/EditorBlueprintResources/ActorMacros.Switch Has Authority`
    (:`Authority`
      (`|ExecutionSequence`
        (:`then_0`
          (bind _asgm_coatofarms (cast `/coatofarms/Assets/GM_coatofarms` (`GameplayStatics.GetGameMode`))
            (:`then`
              (bind _playerdata (`/coatofarms/Assets/GM_coatofarms.PlayerData` _asgm_coatofarms))
              (bind (_value _returnvalue_2) (`BlueprintMapLibrary.Map_Find` _playerdata _returnvalue))
              (if _returnvalue_2
                (bind _inventory (break `/coatofarms/Assets/playerdatastruct` _value))
                (set `self.Inventory` _inventory)
                (set `self.HasValidData` true)
                (bind _keys (`BlueprintMapLibrary.Map_Keys` _inventory))
                (bind _output (`self.Get Inventory Amounts` _inventory _keys))
                (`self.SyncInventoryClient` _keys _output)
                (`self.DebugShowMessage` "loaded")
                (else
                  (set `self.HasValidData` true)
                  (`self.DebugShowMessage` (`KismetTextLibrary.Conv_StringToText` (`KismetStringLibrary.Concat_StrStr` (`KismetStringLibrary.Conv_IntToString` (`BlueprintMapLibrary.Map_Length` _playerdata)) "  " _returnvalue))))))
            (:`CastFailed`
              (`self.DebugShowMessage` "failed"))))
        (:`then_1`
          (set `self.OriginalName` (`PlayerState.GetPlayerName` (`self.PlayerState`)))
          (`self.ChangeNameFactionPrefix` false))))))

(event `DebugShowMessage`
  (params (Message :type Text))
  (bind _asbp_mordhau_hud (cast `/Game/Mordhau/Blueprints/BP_MordhauHUD` (`self.GetHUD`)))
  (`/Game/Mordhau/Blueprints/BP_MordhauHUD.SendMessageToChatbox` _asbp_mordhau_hud "DEBUG" Message))

(event `ChangeNameFactionPrefix`
  (params (ClearName :type Boolean))
  (bind _originalname (`self.OriginalName`))
  (bind _asmc_coatofarms (cast `/coatofarms/Assets/MC_coatofarms` (`self.K2_GetPawn`) :!label _label)
    (:`then`
      (bind (_factionname _found) (`/coatofarms/Assets/MC_coatofarms.GetFaction` _asmc_coatofarms))
      (bind _asbp_mordhau_player_state (cast `/Game/Mordhau/Blueprints/BP_MordhauPlayerState` (`self.PlayerState`)))
      (if ClearName
        (`MordhauPlayerState.SetPlayerName` _asbp_mordhau_player_state _originalname :!label _label_2)
        (elif _found
          (`MordhauPlayerState.SetPlayerName` _asbp_mordhau_player_state (`KismetStringLibrary.Concat_StrStr` "[" (`.FactionName_2_9D2643A241E4BE6CFEE14C94850AB4A7` (break `/coatofarms/Assets/FactionsDataStruct` _factionname)) "]" _originalname))
          (else
            (goto _label_2)))))
    (:`CastFailed`
      (`KismetSystemLibrary.Delay` 1.0)
      (goto _label))))

(event `self.RequestChatMessage`
  (params (Message :type String) (Team :type Boolean))
  (bind _returnvalue (`self.K2_GetPawn`))
  (`parent.RequestChatMessage` Message Team)
  (bind _asmc_coatofarms (cast `/coatofarms/Assets/MC_coatofarms` _returnvalue)
    (:`then`
      (`|ExecutionSequence`
        (:`then_0`
          (`/coatofarms/Assets/MC_coatofarms.TextAboveHeadClient` _asmc_coatofarms Message))
        (:`then_1`
          (bind _asmordhau_game_mode (cast `MordhauGameMode` (`GameplayStatics.GetGameMode`)))
          (add `MordhauGameMode.OnMessageBroadcasted` _asmordhau_game_mode (delegate `Commands`)))))
    (:`CastFailed`
      (bind _asbp_coat_horse (cast `/coatofarms/Assets/BP_CoatHorse` _returnvalue))
      (`/coatofarms/Assets/BP_CoatHorse.TextAboveHeadClient` _asbp_coat_horse Message))))

(event `Commands`
  (params (Sender :type "Actor Object Reference") (Msg :type String) (Type :type Name)))

(event `EmblemActivate`
  (bind _asmc_coatofarms (cast `/coatofarms/Assets/MC_coatofarms` (`self.GetControlledMordhauCharacter` true)))
  (set `/coatofarms/Assets/MC_coatofarms.Emblem` (select `bool` (`/coatofarms/Assets/MC_coatofarms.Emblem` _asmc_coatofarms) :`false` true) _asmc_coatofarms))

(event `Key|NumPadNine`
  (params (Key :type "Key Structure"))
  (:`Pressed`
    (`self.EmblemActivate`)))

(event `self.OnAfterPossess`
  (params (aPawn :type "Pawn Object Reference"))
  (bind _inventory (`self.Inventory`))
  (bind _inventory_2 (`self.Inventory`))
  (bind (_name _gearcustomization _appearancecustomization _facecustomization _skillscustomization _category) (break `CharacterProfile` (`self.CharacterProfile`)))
  (bind (_name_2 _gearcustomization_2 _appearancecustomization_2 _facecustomization_2 _skillscustomization_2 _category_2) (break `CharacterProfile` (`self.CharacterProfile`)))
  (bind (_name_3 _gearcustomization_3 _appearancecustomization_3 _facecustomization_3 _skillscustomization_3 _category_3) (break `CharacterProfile` (`self.CharacterProfile`)))
  (bind (_wearables _equipment) (break `CharacterGearCustomization` _gearcustomization_2))
  (bind (_wearables_2 _equipment_2) (break `CharacterGearCustomization` _gearcustomization_3))
  (bind (_wearables_3 _equipment_3) (break `CharacterGearCustomization` _gearcustomization))
  (`parent.OnAfterPossess` aPawn)
  (`|ExecutionSequence`
    (:`then_0`
      (if (or (>= (`BlueprintMapLibrary.Map_Find` _inventory_2 "Noble") 1) (>= (`BlueprintMapLibrary.Map_Find` _inventory_2 "Lord") 1) (>= (`BlueprintMapLibrary.Map_Find` _inventory_2 "Bishop") 1) (>= (`BlueprintMapLibrary.Map_Find` _inventory_2 "King") 1) (>= (`BlueprintMapLibrary.Map_Find` _inventory_2 "Knight") 1))
        _
        (elif (>= (`BlueprintMapLibrary.Map_Find` (`self.Inventory`) "Squire") 1)
          (for (_array_element _array_index) _wearables_2
            (bind _id (break `WearableCustomization` _array_element))
            (if (or (and (`KismetArrayLibrary.Array_Contains` (`self.Tier3Head`) _id) (`KismetArrayLibrary.Array_Contains` (`self.Head`) _array_index)) (and (`KismetArrayLibrary.Array_Contains` (`self.Tier3Upperchest`) _id) (`KismetArrayLibrary.Array_Contains` (`self.UpperChest`) _array_index)) (and (`KismetArrayLibrary.Array_Contains` (`self.Tier3Legs`) _id) (`KismetArrayLibrary.Array_Contains` (`self.Legs`) _array_index)))
              (`CustomizationReplicationActor.AssignDataFromProfile` (`self.CustomizationReplicationActor`) (make `CharacterProfile` _name_3 (make `CharacterGearCustomization` (`self.Wearables`) _equipment_2) _appearancecustomization_3 _facecustomization_3 _skillscustomization_3 _category_3))
              (bind _asmc_coatofarms (cast `/coatofarms/Assets/MC_coatofarms` (`self.K2_GetPawn`) :!label _label_3))
              (`/coatofarms/Assets/MC_coatofarms.CallThemPeasant` _asmc_coatofarms)))
          (else
            (for (_array_element_2 _array_index_2) _wearables
              (bind _id_2 (break `WearableCustomization` _array_element_2))
              (if (or (and (`KismetArrayLibrary.Array_Contains` (`self.Tier2Head`) _id_2) (`KismetArrayLibrary.Array_Contains` (`self.Head`) _array_index_2)) (and (`KismetArrayLibrary.Array_Contains` (`self.UpperChest`) _array_index_2) (`KismetArrayLibrary.Array_Contains` (`self.Tier2Upperchest`) _id_2)) (and (`KismetArrayLibrary.Array_Contains` (`self.Legs`) _array_index_2) (`KismetArrayLibrary.Array_Contains` (`self.Tier2Legs`) _id_2)))
                (`CustomizationReplicationActor.AssignDataFromProfile` (`self.CustomizationReplicationActor`) (make `CharacterProfile` _name_2 (make `CharacterGearCustomization` (`self.Wearables`) _equipment) _appearancecustomization_2 _facecustomization_2 _skillscustomization_2 _category_2) :!label _label_4)
                (goto _label_3)
                (elif (or (and (`KismetArrayLibrary.Array_Contains` (`self.Tier3Head`) _id_2) (`KismetArrayLibrary.Array_Contains` (`self.Head`) _array_index_2)) (and (`KismetArrayLibrary.Array_Contains` (`self.Tier3Upperchest`) _id_2) (`KismetArrayLibrary.Array_Contains` (`self.UpperChest`) _array_index_2)) (and (`KismetArrayLibrary.Array_Contains` (`self.Tier3Legs`) _id_2) (`KismetArrayLibrary.Array_Contains` (`self.Legs`) _array_index_2)))
                  (goto _label_4))))))))
    (:`then_1`
      (bind _asmc_coatofarms_2 (cast `/coatofarms/Assets/MC_coatofarms` aPawn))
      (set `/coatofarms/Assets/MC_coatofarms.Emblem` (`self.DefaultEmblemView`) _asmc_coatofarms_2))
    (:`then_2`
      (if (not (or (>= (`BlueprintMapLibrary.Map_Find` _inventory "Noble") 1) (>= (`BlueprintMapLibrary.Map_Find` _inventory "Lord") 1) (>= (`BlueprintMapLibrary.Map_Find` _inventory "Bishop") 1) (>= (`BlueprintMapLibrary.Map_Find` _inventory "King") 1)))
        (for (_array_element_3 _array_index_3) _wearables_3
          (if (and (`KismetArrayLibrary.Array_Contains` (`self.CrownHead`) (`.Id` (break `WearableCustomization` _array_element_3))) (`KismetArrayLibrary.Array_Contains` (`self.Head`) _array_index_3))
            (`CustomizationReplicationActor.AssignDataFromProfile` (`self.CustomizationReplicationActor`) (make `CharacterProfile` _name (make `CharacterGearCustomization` (`self.Wearables`) _equipment_3) _appearancecustomization _facecustomization _skillscustomization _category))))))))

(fn `Get Inventory Amounts`
  (params (Inventory :type "Map of String to Integer (by ref)") (Keys :type "Array of String"))
  (returns (Output :type "Array of Integer"))
  (locals (InventoryValues :type "Array of Integer"))
  (for _array_element Keys
    (`KismetArrayLibrary.Array_Add` (`local.InventoryValues`) (`BlueprintMapLibrary.Map_Find` Inventory _array_element)))
  (return (`local.InventoryValues`)))

(fn `UserConstructionScript`
  (`parent.UserConstructionScript`))