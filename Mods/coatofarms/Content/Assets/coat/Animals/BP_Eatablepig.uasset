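; BP_Eatablepig is an edible pig animal that drops meat when killed.
; It overrides OnKilled, calls the parent handler, then spawns several BP_Meat actors at the transform of its Scene component.
; BeginPlay, overlap and Tick are unused stubs, and the construction script only calls its parent.
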(event `self.OnKilled`
  (params (EventInstigator :type "Controller Object Reference"))
  (bind _returnvalue (`SceneComponent.K2_GetComponentToWorld` (`self.Scene`)))
  (`parent.OnKilled` EventInstigator)
  (`|SpawnActorFromClass` "/coatofarms/Assets/coat/MineableItems/BP_Meat.BP_Meat_C" _returnvalue "Undefined" "OverrideRootScale" null null)
  (`|SpawnActorFromClass` "/coatofarms/Assets/coat/MineableItems/BP_Meat.BP_Meat_C" _returnvalue "Undefined" "OverrideRootScale" null null)
  (`|SpawnActorFromClass` "/coatofarms/Assets/coat/MineableItems/BP_Meat.BP_Meat_C" _returnvalue "Undefined" "OverrideRootScale" null null)
  (`|SpawnActorFromClass` "/coatofarms/Assets/coat/MineableItems/BP_Meat.BP_Meat_C" _returnvalue "Undefined" "OverrideRootScale" null null))

(fn `UserConstructionScript`
  (`parent.UserConstructionScript`))