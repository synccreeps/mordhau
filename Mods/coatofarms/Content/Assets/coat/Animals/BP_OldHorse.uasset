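; BP_OldHorse is an old horse animal Blueprint that drops meat when it dies.
; Its OnDied override runs the parent death handling, then spawns two BP_HorseMeat actors at the horse's transform.
; It adds no other logic, leaving all remaining behavior to its parent class.
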(event `self.OnDied`
  (params (Angle :type "Float (single-precision)") (Type :type "EMordhauDamageType Enum" :default "Generic") (SubType :type Byte) (Bone :type Name) (Point :type "Vector Structure") (Source :type "Actor Object Reference") (Agent :type "Actor Object Reference"))
  (bind _returnvalue (`self.GetTransform`))
  (`parent.OnDied` Angle Type SubType Bone Point Source Agent)
  (`|SpawnActorFromClass` "/coatofarms/Assets/coat/MineableItems/BP_HorseMeat.BP_HorseMeat_C" _returnvalue "Undefined" "OverrideRootScale" null null)
  (`|SpawnActorFromClass` "/coatofarms/Assets/coat/MineableItems/BP_HorseMeat.BP_HorseMeat_C" _returnvalue "Undefined" "OverrideRootScale" null null))

(fn `UserConstructionScript`
  (`parent.UserConstructionScript`))