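; BP_Bartender is an interactable bartender who opens the bartender widget and buys wine barrels from the player.
; On InteractionStart it calls BartenderWidget on the MC_coatofarms character.
; It then checks that character's right hand for a BP_WineBarrel, which it drops and destroys before crediting Copper Coins through InventoryUpdate on PC_coatofarms.
; The sale runs automatically on interaction, with no confirmation from the widget.
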(event `self.InteractionStart`
  (params (Character :type "MordhauCharacter Object Reference"))
  (`|ExecutionSequence`
    (:`then_0`
      (bind _asmc_coatofarms (cast `/coatofarms/Assets/MC_coatofarms` Character))
      (`/coatofarms/Assets/MC_coatofarms.BartenderWidget` _asmc_coatofarms))
    (:`then_1`
      (bind _asmc_coatofarms_2 (cast `/coatofarms/Assets/MC_coatofarms` Character))
      (bind _aspc_coatofarms (cast `/coatofarms/Assets/PC_coatofarms` (`Pawn.GetController` Character)))
      (bind _righthandequipment (`MordhauCharacter.RightHandEquipment` _asmc_coatofarms_2))
      (if (== (`GameplayStatics.GetObjectClass` _righthandequipment) "/coatofarms/Assets/coat/CraftableItems/BP_WineBarrel.BP_WineBarrel_C")
        (bind _returnvalue (`MordhauCharacter.DropEquipment` Character _righthandequipment false))
        (`self.K2_DestroyActor` _returnvalue)
        (`/coatofarms/Assets/PC_coatofarms.InventoryUpdate` _aspc_coatofarms "Copper Coin" 20)))))

(fn `UserConstructionScript`
  (`parent.UserConstructionScript`))