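; Cart actor that receives a delivery crate, weapon bundle or wine barrel carried in the player's right hand.
; On InteractionStart it casts to MC_coatofarms and checks the held item's exact class.
; It spawns a replacement at the Scene component's transform, attaches it to the cart, then drops and destroys the held original.
; Crates and barrels respawn as the same class, while weapon bundles become the blue deliverable variant.
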(event `self.InteractionStart`
  (params (Character :type "MordhauCharacter Object Reference"))
  (bind _scene (`self.Scene`))
  (bind _asmc_coatofarms (cast `/coatofarms/Assets/MC_coatofarms` Character))
  (bind _righthandequipment (`MordhauCharacter.RightHandEquipment` _asmc_coatofarms))
  (if (== (`GameplayStatics.GetObjectClass` _righthandequipment) "/coatofarms/Assets/coat/CraftableItems/BP_DeliverCrate.BP_DeliverCrate_C")
    (bind _returnvalue (`|SpawnActorFromClass` "/coatofarms/Assets/coat/CraftableItems/BP_DeliverCrate.BP_DeliverCrate_C" (`SceneComponent.K2_GetComponentToWorld` _scene) "Undefined" "OverrideRootScale" null null))
    (`self.K2_AttachToActor` _returnvalue self (`SceneComponent.GetAttachSocketName` _scene) "SnapToTarget" "SnapToTarget" "SnapToTarget" false)
    (bind _returnvalue_2 (`MordhauCharacter.DropEquipment` _asmc_coatofarms _righthandequipment false))
    (`self.K2_DestroyActor` _returnvalue_2)
    (else
      (bind _righthandequipment_2 (`MordhauCharacter.RightHandEquipment` _asmc_coatofarms))
      (if (== (`GameplayStatics.GetObjectClass` _righthandequipment_2) "/coatofarms/Assets/coat/CraftableItems/BP_WeaponBundle.BP_WeaponBundle_C")
        (bind _returnvalue_3 (`|SpawnActorFromClass` "/Game/Mordhau/Blueprints/GameModes/Battle/Deliverables/BP_DeliverableWeaponBundle_Blue.BP_DeliverableWeaponBundle_Blue_C" (`SceneComponent.K2_GetComponentToWorld` _scene) "Undefined" "OverrideRootScale" null null))
        (`self.K2_AttachToActor` _returnvalue_3 self (`SceneComponent.GetAttachSocketName` _scene) "SnapToTarget" "SnapToTarget" "SnapToTarget" false)
        (bind _returnvalue_4 (`MordhauCharacter.DropEquipment` _asmc_coatofarms _righthandequipment_2 false))
        (`self.K2_DestroyActor` _returnvalue_4)
        (else
          (bind _righthandequipment_3 (`MordhauCharacter.RightHandEquipment` _asmc_coatofarms))
          (if (== (`GameplayStatics.GetObjectClass` _righthandequipment_3) "/coatofarms/Assets/coat/CraftableItems/BP_WineBarrel.BP_WineBarrel_C")
            (bind _returnvalue_5 (`|SpawnActorFromClass` "/coatofarms/Assets/coat/CraftableItems/BP_WineBarrel.BP_WineBarrel_C" (`SceneComponent.K2_GetComponentToWorld` _scene) "Undefined" "OverrideRootScale" null null))
            (`self.K2_AttachToActor` _returnvalue_5 self (`SceneComponent.GetAttachSocketName` _scene) "SnapToTarget" "SnapToTarget" "SnapToTarget" false)
            (bind _returnvalue_6 (`MordhauCharacter.DropEquipment` _asmc_coatofarms _righthandequipment_3 false))
            (`self.K2_DestroyActor` _returnvalue_6)))))))

(fn `UserConstructionScript`
  (`parent.UserConstructionScript`))