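; BP_Flagholdable is an actor, apparently a holdable flag by its name, that displays an image fetched from a URL.
; On BeginPlay it downloads the image asynchronously, then creates a dynamic material instance from CustomImage on the Plane component.
; The downloaded texture is set on that material, though the parameter name is left as None.
; Plane1 is not updated, and a failed download has no handling.
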(event `self.ReceiveBeginPlay`
  (bind _texture (`AsyncTaskDownloadImage.DownloadImage` (`self.Url`))
    (:`then`
      (bind _returnvalue (`PrimitiveComponent.CreateDynamicMaterialInstance` (`self.Plane`) 0 "/coatofarms/Assets/coat/CustomImage.CustomImage" "None"))
      (`MaterialInstanceDynamic.SetTextureParameterValue` _returnvalue "None" _texture))))

(fn `UserConstructionScript`
  (`parent.UserConstructionScript`))