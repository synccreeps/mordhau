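; Gold trader actor that opens a trading UI when a player character interacts with it.
; InteractionStart casts the character to MC_coatofarms and calls its GoldTraderWidget.
; Tick rotates the TextRender along the vector from the player camera to the text, billboard-style.
; An unconnected leftover graph converts silver, iron and gold ore into ingots through the PC_coatofarms inventory, but never runs.
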(event `self.InteractionStart`
  (params (Character :type "MordhauCharacter Object Reference"))
  (bind _asmc_coatofarms (cast `/coatofarms/Assets/MC_coatofarms` Character))
  (`/coatofarms/Assets/MC_coatofarms.GoldTraderWidget` _asmc_coatofarms))

(event `self.ReceiveTick`
  (params (DeltaSeconds :type "Float (single-precision)"))
  (bind _returnvalue (`GameplayStatics.GetPlayerCameraManager` 0))
  (bind _textrender (`self.TextRender`))
  (`/Engine/EditorBlueprintResources/StandardMacros.IsValid` _returnvalue
    (:`Is Valid`
      (`SceneComponent.K2_SetWorldRotation` _textrender (`KismetMathLibrary.MakeRotFromX` (- (`SceneComponent.K2_GetComponentLocation` _textrender) (`self.K2_GetActorLocation` _returnvalue))) false false))))

(fn `UserConstructionScript`
  (`parent.UserConstructionScript`))