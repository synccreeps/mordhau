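; Pickup bag actor that holds an item type and amount, with a text label showing the type.
; On interaction, it passes both values to InventoryUpdate on the character's PC_coatofarms controller, then destroys itself.
; Each Tick billboards the label by aligning its X axis with the vector from the player camera to the text, so it points away from the camera.
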(event `self.ReceiveBeginPlay`
  (`TextRenderComponent.K2_SetText` (`self.TextRender`) (`KismetTextLibrary.Conv_StringToText` (`self.Item Type`))))

(event `self.InteractionStart`
  (params (Character :type "MordhauCharacter Object Reference"))
  (bind _aspc_coatofarms (cast `/coatofarms/Assets/PC_coatofarms` (`Pawn.GetController` Character)))
  (`/coatofarms/Assets/PC_coatofarms.InventoryUpdate` _aspc_coatofarms (`self.Item Type`) (`self.Item Amount`))
  (`self.K2_DestroyActor`))

(event `self.ReceiveTick`
  (params (DeltaSeconds :type "Float (single-precision)"))
  (bind _returnvalue (`GameplayStatics.GetPlayerCameraManager` 0))
  (bind _textrender (`self.TextRender`))
  (`/Engine/EditorBlueprintResources/StandardMacros.IsValid` _returnvalue
    (:`Is Valid`
      (`SceneComponent.K2_SetWorldRotation` _textrender (`KismetMathLibrary.MakeRotFromX` (- (`SceneComponent.K2_GetComponentLocation` _textrender) (`self.K2_GetActorLocation` _returnvalue))) false false))))

(fn `UserConstructionScript`
  (`parent.UserConstructionScript`))