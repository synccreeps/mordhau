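; BP_NoBuildingZone is a zone actor that blocks building placement when the player enters it holding a building toolbox.
; On begin overlap with MC_coatofarms, it checks that the right-hand equipment class is BP_BuildingToolbox.
; It then calls ValidateSpot with ForceFail on the BuildingSystem of every toolbox in the level.
; End overlap is empty, and the revalidation logic is disconnected, so leaving triggers no recheck.
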(event `self.ReceiveActorBeginOverlap`
  (params (OtherActor :type "Actor Object Reference"))
  (bind _asmc_coatofarms (cast `/coatofarms/Assets/MC_coatofarms` OtherActor))
  (if (`self.IsOverlappingActor` _asmc_coatofarms self)
    (if (== (`GameplayStatics.GetObjectClass` (`MordhauCharacter.RightHandEquipment` _asmc_coatofarms)) "/coatofarms/Assets/coat/Building/BP_BuildingToolbox.BP_BuildingToolbox_C")
      (bind _outactors (`GameplayStatics.GetAllActorsOfClass` "/coatofarms/Assets/coat/Building/BP_BuildingToolbox.BP_BuildingToolbox_C"))
      (for _array_element _outactors
        (`BuildingSystemComponent.ValidateSpot` (`/Game/Mordhau/Blueprints/Equipment/Misc/BP_ToolBox.BuildingSystem` _array_element) (0.0 0.0 0.0) 0 false true)))))

(event `self.ReceiveActorEndOverlap`
  (params (OtherActor :type "Actor Object Reference")))

(fn `UserConstructionScript`
  (`parent.UserConstructionScript`))