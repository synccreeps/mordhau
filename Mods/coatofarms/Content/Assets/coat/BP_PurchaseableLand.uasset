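; BP_PurchaseableLand is a land plot that keeps players who do not own it from bringing building tools inside.
; When a character enters its Box, it looks up the Land entry in the player controller's Inventory.
; Without at least one, a character holding a BP_BuildingToolbox or BP_ToolBox in either hand is told to drop both hands' equipment.
; Safe-zone logic is left disconnected, and Tick does nothing beyond the parent call.
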(event `self.Box.OnComponentBeginOverlap`
  (params (OverlappedComponent :type "PrimitiveComponent Object Reference") (OtherActor :type "Actor Object Reference") (OtherComp :type "PrimitiveComponent Object Reference") (OtherBodyIndex :type Integer) (bFromSweep :type Boolean) (SweepResult :type "HitResult Structure (by ref)"))
  (bind _asmc_coatofarms (cast `/coatofarms/Assets/MC_coatofarms` OtherActor))
  (bind _aspc_coatofarms (cast `/coatofarms/Assets/PC_coatofarms` (`self.GetInstigatorController` OtherActor)))
  (if (not (>= (`BlueprintMapLibrary.Map_Find` (`/coatofarms/Assets/PC_coatofarms.Inventory` _aspc_coatofarms) (`self.Land`)) 1))
    (bind _lefthandequipment (`MordhauCharacter.LeftHandEquipment` _asmc_coatofarms))
    (bind _returnvalue (`GameplayStatics.GetObjectClass` _lefthandequipment))
    (bind _righthandequipment (`MordhauCharacter.RightHandEquipment` _asmc_coatofarms))
    (bind _returnvalue_2 (`GameplayStatics.GetObjectClass` _righthandequipment))
    (if (or (== _returnvalue "/coatofarms/Assets/coat/Building/BP_BuildingToolbox.BP_BuildingToolbox_C") (== _returnvalue_2 "/coatofarms/Assets/coat/Building/BP_BuildingToolbox.BP_BuildingToolbox_C"))
      (`MordhauCharacter.DropEquipment` _asmc_coatofarms _lefthandequipment false :!label _label)
      (`MordhauCharacter.DropEquipment` _asmc_coatofarms _righthandequipment false)
      (elif (or (== _returnvalue "/Game/Mordhau/Blueprints/Equipment/Misc/BP_ToolBox.BP_ToolBox_C") (== _returnvalue_2 "/Game/Mordhau/Blueprints/Equipment/Misc/BP_ToolBox.BP_ToolBox_C"))
        (goto _label)))))

(event `self.ReceiveTick`
  (params (DeltaSeconds :type "Float (single-precision)"))
  (`parent.ReceiveTick` DeltaSeconds)
  (if (== (`self.IsSafe`) true)
    _))

(event `self.ReceiveActorEndOverlap`
  (params (OtherActor :type "Actor Object Reference")))

(fn `UserConstructionScript`
  (`parent.UserConstructionScript`))