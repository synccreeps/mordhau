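; Placeable building object that previews whether its current spot is valid and becomes solid when placed.
; CheckSpawn treats any overlapping actor as blocking, setting the CanSpawn flag and swapping the mesh between the blocked and green preview materials.
; Place acts only when CanSpawn is true, applying the stored material and switching the mesh collision profile to BlockAllDynamic.
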(fn `CheckSpawn`
  (bind _mesh (`self.Mesh`))
  (if (> (`KismetArrayLibrary.Array_Length` (`self.GetOverlappingActors` null)) 0)
    (`PrimitiveComponent.SetMaterial` _mesh 0 "/Game/Mordhau/Assets/Materials/M_PreviewMesh.M_PreviewMesh")
    (set `self.CanSpawn` false)
    (else
      (`PrimitiveComponent.SetMaterial` _mesh 0 "/coatofarms/Assets/coat/Building/M_PreviewMeshGreen.M_PreviewMeshGreen")
      (set `self.CanSpawn` true))))

(fn `Place`
  (bind _mesh (`self.Mesh`))
  (if (`self.CanSpawn`)
    (`PrimitiveComponent.SetMaterial` _mesh 0 (`self.Material`))
    (`PrimitiveComponent.SetCollisionProfileName` _mesh "BlockAllDynamic" true)))

(fn `UserConstructionScript`
  (`parent.UserConstructionScript`))