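; BP_WoodRoof1 is a buildable wooden roof that a player completes piece by piece with Planks from their inventory.
; Each InteractionStart consumes one Plank via PC_coatofarms, and every second one reveals the next static mesh in a fixed array.
; After ten reveal steps WeDone blocks further interaction.
; The array lists StaticMesh8 twice and omits StaticMesh7, so one step reveals nothing new.
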(event `self.InteractionStart`
  (params (Character :type "MordhauCharacter Object Reference"))
  (bind _hitindex (`self.HitIndex`))
  (if (not (>= (`self.WeDone`) 1))
    (bind _aspc_coatofarms (cast `/coatofarms/Assets/PC_coatofarms` (`Pawn.GetController` Character)))
    (if (>= (`BlueprintMapLibrary.Map_Find` (`/coatofarms/Assets/PC_coatofarms.Inventory` _aspc_coatofarms) "Plank") 1)
      (`/coatofarms/Assets/PC_coatofarms.InventoryUpdate` _aspc_coatofarms "Plank" -1)
      (bind _output_get (set `self.Total Hits` (+ (`self.Total Hits`) 1)))
      (if (>= _output_get 2)
        (`SceneComponent.SetVisibility` (`|GetArrayItem` (`|MakeArray` (`self.StaticMesh1`) (`self.StaticMesh2`) (`self.StaticMesh3`) (`self.StaticMesh4`) (`self.StaticMesh5`) (`self.StaticMesh8`) (`self.StaticMesh8`) (`self.StaticMesh9`) (`self.StaticMesh10`) (`self.StaticMesh6`)) _hitindex) true false)
        (bind _output_get_2 (set `self.HitIndex` (+ _hitindex 1)))
        (if (`KismetMathLibrary.Conv_IntToBool` _output_get_2)
          (set `self.Total Hits` 0)
          (if (>= (`KismetMathLibrary.Conv_IntToByte` _hitindex) 10)
            (set `self.WeDone` 1)))))))

(fn `UserConstructionScript`
  (`parent.UserConstructionScript`))