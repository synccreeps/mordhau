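; BP_WoodWallThin1 is a buildable thin wooden wall for Mordhau that players raise piece by piece by hitting it.
; AnyDamage takes a Plank from the attacking PC_coatofarms inventory, even before checking for a left or right strike with BP_SmithHammer or BP_Warhammer.
; Each valid hit unhides the next mesh in an ordered array, which repeats two meshes, until WeDone locks it at index 16, before the last entry.
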(event `self.ReceiveAnyDamage`
  (params (Damage :type "Float (single-precision)") (DamageType :type "DamageType Object Reference") (InstigatedBy :type "Controller Object Reference") (DamageCauser :type "Actor Object Reference"))
  (bind _hitindex (`self.HitIndex`))
  (if (not (>= (`self.WeDone`) 1))
    (bind _aspc_coatofarms (cast `/coatofarms/Assets/PC_coatofarms` InstigatedBy))
    (if (>= (`BlueprintMapLibrary.Map_Find` (`/coatofarms/Assets/PC_coatofarms.Inventory` _aspc_coatofarms) "Plank") 1)
      (`/coatofarms/Assets/PC_coatofarms.InventoryUpdate` _aspc_coatofarms "Plank" -1)
      (bind _asmordhau_character (cast `MordhauCharacter` DamageCauser))
      (bind _asattack_motion (cast `AttackMotion` (`MordhauCharacter.Motion` _asmordhau_character)))
      (bind _move (`AttackMotion.Move` _asattack_motion))
      (if (or (`|EnumEquality` _move "RightStrike") (`|EnumEquality` _move "LeftStrike"))
        (bind _weapon (`AttackMotion.Weapon` _asattack_motion))
        (if (== (`GameplayStatics.GetObjectClass` _weapon) "/Game/Mordhau/Blueprints/Equipment/Weapons/Specific/OneHanded/BP_SmithHammer.BP_SmithHammer_C")
          (bind _output_get (set `self.Total Hits` (+ (`self.Total Hits`) 1)))
          (if (>= _output_get 1)
            (`SceneComponent.SetVisibility` (`|GetArrayItem` (`|MakeArray` (`self.StaticMesh`) (`self.StaticMesh1`) (`self.StaticMesh2`) (`self.StaticMesh3`) (`self.StaticMesh4`) (`self.StaticMesh5`) (`self.StaticMesh8`) (`self.StaticMesh8`) (`self.StaticMesh9`) (`self.StaticMesh9`) (`self.StaticMesh10`) (`self.StaticMesh11`) (`self.StaticMesh12`) (`self.StaticMesh13`) (`self.StaticMesh14`) (`self.StaticMesh15`) (`self.StaticMesh16`)) _hitindex) true false :!label _label)
            (bind _output_get_2 (set `self.HitIndex` (+ _hitindex 1)))
            (if (`KismetMathLibrary.Conv_IntToBool` _output_get_2)
              (set `self.Total Hits` 0)
              (if (>= (`KismetMathLibrary.Conv_IntToByte` _hitindex) 16)
                (set `self.WeDone` 1))))
          (elif (== (`GameplayStatics.GetObjectClass` _weapon) "/Game/Mordhau/Blueprints/Equipment/Weapons/Specific/OneHanded/BP_Warhammer.BP_Warhammer_C")
            (bind _output_get_3 (set `self.Total Hits` (+ (`self.Total Hits`) 1)))
            (if (>= _output_get_3 1)
              (goto _label))))))))

(fn `UserConstructionScript`
  (`parent.UserConstructionScript`))