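; BP_BagSwords is an interactable crafting object that turns three Smith Swords from a player's inventory into a weapon bundle.
; Interaction calls BagServer, which passes straight to BagClient.
; BagClient casts the interacting Character's controller to PC_coatofarms and checks its inventory for at least three swords.
; It then removes three through InventoryUpdate and spawns a BP_WeaponBundle at the Scene component's world transform.
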(event `self.InteractionStart`
  (params (Character :type "MordhauCharacter Object Reference"))
  (`self.BagServer`))

(event `BagClient`
  (bind _aspc_coatofarms (cast `/coatofarms/Assets/PC_coatofarms` (`Pawn.GetController` (stale `self.InteractionStart` Character))))
  (if (>= (`BlueprintMapLibrary.Map_Find` (`/coatofarms/Assets/PC_coatofarms.Inventory` _aspc_coatofarms) "Smith Sword") 3)
    (`/coatofarms/Assets/PC_coatofarms.InventoryUpdate` _aspc_coatofarms "Smith Sword" -3)
    (`|SpawnActorFromClass` "/coatofarms/Assets/coat/CraftableItems/BP_WeaponBundle.BP_WeaponBundle_C" (`SceneComponent.K2_GetComponentToWorld` (`self.Scene`)) "Undefined" "OverrideRootScale" null null)))

(event `BagServer`
  (`self.BagClient`))

(fn `UserConstructionScript`
  (`parent.UserConstructionScript`))