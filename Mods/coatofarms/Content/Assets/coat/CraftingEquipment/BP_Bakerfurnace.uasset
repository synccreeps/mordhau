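; Baker's furnace crafting station that opens the interacting character's baking widget, passing the furnace's first tag.
; An AnyDamage path marked OldWay counts left or right strikes while the Bread component is visible, then spawns BP_Bread on the second hit and hides it.
; BakerComponentVisiblity, marked Old, calls BakerComponentVisiblityMulti to show the bread.
; Unreachable leftovers hold ore-to-ingot smelting and a hammer-type check.
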(event `self.InteractionStart`
  (params (Character :type "MordhauCharacter Object Reference"))
  (bind _asmc_coatofarms (cast `/coatofarms/Assets/MC_coatofarms` Character))
  (`/coatofarms/Assets/MC_coatofarms.BakingWidget` _asmc_coatofarms (`|GetArrayItem` (`self.Tag`))))

(event `self.ReceiveAnyDamage`
  (params (Damage :type "Float (single-precision)") (DamageType :type "DamageType Object Reference") (InstigatedBy :type "Controller Object Reference") (DamageCauser :type "Actor Object Reference"))
  (bind _bread (`self.Bread`))
  ;[1 1 1] OldWay
  (if (`SceneComponent.IsVisible` _bread)
    (bind _asmc_coatofarms (cast `/coatofarms/Assets/MC_coatofarms` DamageCauser))
    (bind _asattack_motion (cast `AttackMotion` (`MordhauCharacter.Motion` _asmc_coatofarms)))
    (bind _move (`AttackMotion.Move` _asattack_motion))
    (if (or (`|EnumEquality` _move "RightStrike") (`|EnumEquality` _move "LeftStrike"))
      (bind _output_get (set `self.Total Hits` (+ (`self.Total Hits`) 1)))
      (if (>= _output_get 2)
        (`|SpawnActorFromClass` "/coatofarms/Assets/coat/MineableItems/BP_Bread.BP_Bread_C" (`SceneComponent.K2_GetComponentToWorld` (`self.Scene`)) "Undefined" "OverrideRootScale" null null)
        (set `self.Total Hits` 0)
        (`SceneComponent.SetVisibility` _bread false false)))))

(event `BakerComponentVisiblity`
  ;[1 1 1] Old
  (`self.BakerComponentVisiblityMulti`))

(event `BakerComponentVisiblityMulti`
  ;[1 1 1] Old
  (`SceneComponent.SetVisibility` (`self.Bread`) true false))

(fn `UserConstructionScript`
  (`parent.UserConstructionScript`))