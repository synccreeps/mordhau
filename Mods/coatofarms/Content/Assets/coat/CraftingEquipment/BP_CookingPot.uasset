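; BP_CookingPot is a crafting station Blueprint for a cooking pot.
; On interaction, it casts the character to MC_coatofarms and opens its crafting table widget, passing the actor's first tag.
; The older flow is disconnected and never runs: spending silver and gold ingots to show an ingot, then hammering it twice to spawn jewelry.
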(event `self.ReceiveBeginPlay`
  (`parent.ReceiveBeginPlay`))

(event `self.InteractionStart`
  (params (Character :type "MordhauCharacter Object Reference"))
  (bind _asmc_coatofarms (cast `/coatofarms/Assets/MC_coatofarms` Character))
  (`/coatofarms/Assets/MC_coatofarms.CraftingTableWidget` _asmc_coatofarms (`|GetArrayItem` (`self.Tags`))))

(event `self.ReceiveAnyDamage`
  (params (Damage :type "Float (single-precision)") (DamageType :type "DamageType Object Reference") (InstigatedBy :type "Controller Object Reference") (DamageCauser :type "Actor Object Reference"))
  ;[1 1 1] OldWay
)

(event `CraftingTableComponentVisiblity`
  ;[1 1 1] Old
)

(event `CraftingTableComponentVisiblityMulti`
  ;[1 1 1] Old
)

(fn `UserConstructionScript`
  (`parent.UserConstructionScript`))