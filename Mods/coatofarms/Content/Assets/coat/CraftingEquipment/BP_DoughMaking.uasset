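; BP_DoughMaking is a crafting equipment actor that turns into dough after repeated player interaction.
; Each InteractionStart from an MC_coatofarms character increments a press counter.
; Once the counter reaches its threshold, it spawns BP_Dough at its Scene component's location and destroys itself.
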(event `self.InteractionStart`
  (params (Character :type "MordhauCharacter Object Reference"))
  (cast `/coatofarms/Assets/MC_coatofarms` Character)
  (set `self.PressTime` (+ (`self.PressTime`) 1))
  (if (>= (`self.PressTime`) 5)
    (`|SpawnActorFromClass` "/coatofarms/Assets/coat/CraftableItems/BP_Dough.BP_Dough_C" (`KismetMathLibrary.Conv_VectorToTransform` (`SceneComponent.K2_GetComponentLocation` (`self.Scene`))) "Undefined" "OverrideRootScale" null null)
    (`self.K2_DestroyActor`)))

(fn `UserConstructionScript`
  (`parent.UserConstructionScript`))