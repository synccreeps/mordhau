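; BP_Export is an interactable export point where a player turns in a carried delivery crate for Copper Coins.
; On InteractionStart it checks the character's right-hand equipment for BP_DeliverCrate, drops and destroys it, then credits a fixed payout through the player controller's InventoryUpdate.
; The crate check tests the right hand twice, so the left hand is never considered.
; BagServer and BagClient are empty.
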(event `self.InteractionStart`
  (params (Character :type "MordhauCharacter Object Reference"))
  (bind _asmc_coatofarms (cast `/coatofarms/Assets/MC_coatofarms` Character))
  (bind _aspc_coatofarms (cast `/coatofarms/Assets/PC_coatofarms` (`Pawn.GetController` Character)))
  (bind _righthandequipment (`MordhauCharacter.RightHandEquipment` _asmc_coatofarms))
  (bind _righthandequipment_2 (`MordhauCharacter.RightHandEquipment` _asmc_coatofarms))
  (if (or (== (`GameplayStatics.GetObjectClass` _righthandequipment) "/coatofarms/Assets/coat/CraftableItems/BP_DeliverCrate.BP_DeliverCrate_C") (== (`GameplayStatics.GetObjectClass` _righthandequipment_2) "/coatofarms/Assets/coat/CraftableItems/BP_DeliverCrate.BP_DeliverCrate_C"))
    (bind _returnvalue (`MordhauCharacter.DropEquipment` Character _righthandequipment false))
    (bind _returnvalue_2 (`MordhauCharacter.DropEquipment` _asmc_coatofarms _righthandequipment_2 false))
    (`self.K2_DestroyActor` _returnvalue)
    (`self.K2_DestroyActor` _returnvalue_2)
    (`/coatofarms/Assets/PC_coatofarms.InventoryUpdate` _aspc_coatofarms "Copper Coin" 20)))

(event `BagServer`)

(fn `BagClient`)

(fn `UserConstructionScript`
  (`parent.UserConstructionScript`))