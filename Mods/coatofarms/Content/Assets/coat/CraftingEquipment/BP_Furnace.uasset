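; Furnace crafting actor that smelts silver, iron and gold ore from the player's inventory into ingots.
; InteractionStart casts the interacting character's controller to PC_coatofarms, then checks each ore type in sequence in its Inventory map.
; Each ore with at least five units is traded through InventoryUpdate for one ingot, so one interaction yields up to one ingot per metal.
; Conversion is instant, with recipes hardcoded as repeated branches.
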(event `self.InteractionStart`
  (params (Character :type "MordhauCharacter Object Reference"))
  (bind _aspc_coatofarms (cast `/coatofarms/Assets/PC_coatofarms` (`Pawn.GetController` Character)))
  (`|ExecutionSequence`
    (:`then_0`
      (bind _inventory (`/coatofarms/Assets/PC_coatofarms.Inventory` _aspc_coatofarms))
      (bind (_value _returnvalue) (`BlueprintMapLibrary.Map_Find` _inventory "Silverore"))
      (if _returnvalue
        (if (>= _value 5)
          (`/coatofarms/Assets/PC_coatofarms.InventoryUpdate` _aspc_coatofarms "Silverore" -5)
          (`/coatofarms/Assets/PC_coatofarms.InventoryUpdate` _aspc_coatofarms "Silveringot" 1))))
    (:`then_1`
      (bind (_value_2 _returnvalue_2) (`BlueprintMapLibrary.Map_Find` _inventory "Ironore"))
      (if _returnvalue_2
        (if (>= _value_2 5)
          (`/coatofarms/Assets/PC_coatofarms.InventoryUpdate` _aspc_coatofarms "Ironore" -5)
          (`/coatofarms/Assets/PC_coatofarms.InventoryUpdate` _aspc_coatofarms "Ironingot" 1))))
    (:`then_2`
      (bind (_value_3 _returnvalue_3) (`BlueprintMapLibrary.Map_Find` _inventory "Goldore"))
      (if _returnvalue_3
        (if (>= _value_3 5)
          (`/coatofarms/Assets/PC_coatofarms.InventoryUpdate` _aspc_coatofarms "Goldore" -5)
          (`/coatofarms/Assets/PC_coatofarms.InventoryUpdate` _aspc_coatofarms "Goldingot" 1))))))

(fn `UserConstructionScript`
  (`parent.UserConstructionScript`))