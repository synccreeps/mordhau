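; Interactable crafting station that washes silver or gold ore from the player's inventory into dust.
; InteractionStart checks the controller's inventory for each ore's required amount, deducts it, sets that ore's flag and calls ServerEverything.
; ServerEverything shows the water and particle effect, waits on a fixed delay, then spawns the flagged dust actors at the Scene transform and clears the flags.
; Nothing here hides the effects again.
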(event `ServerEverything`
  (bind _returnvalue (`SceneComponent.K2_GetComponentToWorld` (`self.Scene`)))
  (`SceneComponent.SetVisibility` (`self.Water`) true false)
  (`SceneComponent.SetVisibility` (`self.ParticleSystem`) true false)
  (`KismetSystemLibrary.Delay` 10.0)
  (`|ExecutionSequence`
    (:`then_0`
      (if (`self.Silverore`)
        (`|SpawnActorFromClass` "/coatofarms/Assets/coat/MineableItems/BP_Silverdust.BP_Silverdust_C" _returnvalue "Undefined" "OverrideRootScale" null null)
        (if (`self.Silverore`)
          (set `self.Silverore` false))))
    (:`then_1`
      (if (`self.Goldore`)
        (`|SpawnActorFromClass` "/coatofarms/Assets/coat/MineableItems/BP_Golddust.BP_Golddust_C" _returnvalue "Undefined" "OverrideRootScale" null null)
        (if (`self.Goldore`)
          (set `self.Goldore` false))))))

(event `self.InteractionStart`
  (params (Character :type "MordhauCharacter Object Reference"))
  (bind _aspc_coatofarms (cast `/coatofarms/Assets/PC_coatofarms` (`Pawn.GetController` Character)))
  (`|ExecutionSequence`
    (:`then_0`
      (bind _inventory (`/coatofarms/Assets/PC_coatofarms.Inventory` _aspc_coatofarms))
      (bind (_value _returnvalue) (`BlueprintMapLibrary.Map_Find` _inventory "Silverore"))
      (if _returnvalue
        (if (>= _value 5)
          (`/coatofarms/Assets/PC_coatofarms.InventoryUpdate` _aspc_coatofarms "Silverore" -5)
          (set `self.Silverore` true)
          (`self.ServerEverything` :!label _label))))
    (:`then_2`
      (bind (_value_2 _returnvalue_2) (`BlueprintMapLibrary.Map_Find` _inventory "Goldore"))
      (if _returnvalue_2
        (if (>= _value_2 100)
          (`/coatofarms/Assets/PC_coatofarms.InventoryUpdate` _aspc_coatofarms "Goldore" -100)
          (set `self.Goldore` true)
          (goto _label))))))

(fn `UserConstructionScript`
  (`parent.UserConstructionScript`))