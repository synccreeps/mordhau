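; BP_SmithWheel is an interactable smithing wheel that turns a Blunt Sword into a Smith Sword.
; Interaction calls SpinServer, which forwards to SpinClient to show particles and set a spin flag that Tick uses to roll the mesh by a fixed per-frame step.
; After a delay it stops the effects, then swaps one sword in the player controller's inventory if a Blunt Sword is present.
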(event `self.ReceiveTick`
  (params (DeltaSeconds :type "Float (single-precision)"))
  (if (`self.IsSpin`)
    (bind _output_get (set `self.X (Roll)` (+ (`self.X (Roll)`) 8.0)))
    (`SceneComponent.K2_SetRelativeLocationAndRotation` (`self.StaticMesh`) (0.0 0.0 0.0) (`KismetMathLibrary.MakeRotator` _output_get) false false)))

(event `self.InteractionStart`
  (params (Character :type "MordhauCharacter Object Reference"))
  (`self.SpinServer`))

(event `SpinClient`
  (bind _particlesystem (`self.ParticleSystem`))
  (`SceneComponent.SetVisibility` _particlesystem true false)
  (set `self.IsSpin` true)
  (`KismetSystemLibrary.Delay` 5.0)
  (set `self.IsSpin` false)
  (`SceneComponent.SetVisibility` _particlesystem false false)
  (bind _aspc_coatofarms (cast `/coatofarms/Assets/PC_coatofarms` (`Pawn.GetController` (stale `self.InteractionStart` Character))))
  (if (>= (`BlueprintMapLibrary.Map_Find` (`/coatofarms/Assets/PC_coatofarms.Inventory` _aspc_coatofarms) "Blunt Sword") 1)
    (`/coatofarms/Assets/PC_coatofarms.InventoryUpdate` _aspc_coatofarms "Blunt Sword" -1)
    (`/coatofarms/Assets/PC_coatofarms.InventoryUpdate` _aspc_coatofarms "Smith Sword" 1)))

(event `SpinServer`
  (`self.SpinClient`))

(fn `UserConstructionScript`
  (`parent.UserConstructionScript`))