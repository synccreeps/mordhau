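; BP_SwordTable is a crafting station that assembles a smith sword from blade and handle items.
; On interaction, if the player controller's inventory holds a Blade or a Handle, it deducts one of each and shows the ingot meshes.
; While visible, damage from left or right strikes with a smith hammer or mallet counts as hits.
; The second hit spawns BP_Smithsword, resets the count and hides the meshes.
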(event `self.ReceiveBeginPlay`
  (`parent.ReceiveBeginPlay`))

(event `self.InteractionStart`
  (params (Character :type "MordhauCharacter Object Reference"))
  (bind _aspc_coatofarms (cast `/coatofarms/Assets/PC_coatofarms` (`Pawn.GetController` Character)))
  (bind _inventory (`/coatofarms/Assets/PC_coatofarms.Inventory` _aspc_coatofarms))
  (if (or (>= (`BlueprintMapLibrary.Map_Find` _inventory "Blade") 1) (>= (`BlueprintMapLibrary.Map_Find` _inventory "Handle") 1))
    (`/coatofarms/Assets/PC_coatofarms.InventoryUpdate` _aspc_coatofarms "Blade" -1)
    (`/coatofarms/Assets/PC_coatofarms.InventoryUpdate` _aspc_coatofarms "Handle" -1)
    (`SceneComponent.SetVisibility` (`self.Ingot`) true false)
    (`SceneComponent.SetVisibility` (`self.Ingot1`) true false)))

(event `self.ReceiveAnyDamage`
  (params (Damage :type "Float (single-precision)") (DamageType :type "DamageType Object Reference") (InstigatedBy :type "Controller Object Reference") (DamageCauser :type "Actor Object Reference"))
  (bind _ingot (`self.Ingot`))
  (if (`SceneComponent.IsVisible` _ingot)
    (bind _asmc_coatofarms (cast `/coatofarms/Assets/MC_coatofarms` DamageCauser))
    (bind _asattack_motion (cast `AttackMotion` (`MordhauCharacter.Motion` _asmc_coatofarms)))
    (bind _move (`AttackMotion.Move` _asattack_motion))
    (if (or (`|EnumEquality` _move "RightStrike") (`|EnumEquality` _move "LeftStrike"))
      (bind _weapon (`AttackMotion.Weapon` _asattack_motion))
      (if (or (== (`GameplayStatics.GetObjectClass` _weapon) "/Game/Mordhau/Blueprints/Equipment/Weapons/Specific/OneHanded/BP_SmithHammer.BP_SmithHammer_C") (== (`GameplayStatics.GetObjectClass` _weapon) "/Game/Mordhau/Blueprints/Equipment/Weapons/Specific/OneHanded/BP_Mallet.BP_Mallet_C"))
        (bind _output_get (set `self.Total Hits` (+ (`self.Total Hits`) 1)))
        (if (>= _output_get 2)
          (`|SpawnActorFromClass` "/coatofarms/Assets/coat/CraftableItems/BP_Smithsword.BP_Smithsword_C" (`SceneComponent.K2_GetComponentToWorld` (`self.Scene`)) "Undefined" "OverrideRootScale" null null)
          (set `self.Total Hits` 0)
          (`SceneComponent.SetVisibility` _ingot false false)
          (`SceneComponent.SetVisibility` (`self.Ingot1`) false false))))))

(fn `UserConstructionScript`
  (`parent.UserConstructionScript`))