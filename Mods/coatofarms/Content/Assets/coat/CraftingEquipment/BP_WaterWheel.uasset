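; BP_WaterWheel is an interactable piece of crafting equipment that produces water buckets.
; Starting an interaction calls the parent handler, waits briefly, then spawns a BP_Waterbucket at the Scene component's transform.
; After spawning, it disables interaction for a cooldown, with a DoOnce blocking further spawns until interaction is restored and the gate resets.
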(event `self.InteractionStart`
  (params (Character :type "MordhauCharacter Object Reference"))
  (`parent.InteractionStart` Character)
  (`KismetSystemLibrary.Delay` 3.0)
  (`/Engine/EditorBlueprintResources/StandardMacros.DoOnce` false :!label _label
    (:`Completed`
      (`|SpawnActorFromClass` "/coatofarms/Assets/coat/MineableItems/BP_Waterbucket.BP_Waterbucket_C" (`SceneComponent.K2_GetComponentToWorld` (`self.Scene`)) "Undefined" "OverrideRootScale" null null)
      (set `self.bIsInteractable` false)
      (`KismetSystemLibrary.Delay` 10.0)
      (set `self.bIsInteractable` true)
      (goto _label :!via `Reset`))))

(fn `UserConstructionScript`
  (`parent.UserConstructionScript`))