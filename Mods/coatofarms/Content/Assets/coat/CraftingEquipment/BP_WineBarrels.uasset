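; BP_WineBarrels is an interactable crafting station that turns Grapejuice into a wine barrel.
; InteractionStart calls ServerBarrel, which relays to ClientBarrel.
; ClientBarrel checks the interacting character's PC_coatofarms inventory for at least one Grapejuice, deducts one and spawns a BP_WineBarrel at the Scene component's transform.
; The BagServer event and BagClient function are empty.
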(event `self.InteractionStart`
  (params (Character :type "MordhauCharacter Object Reference"))
  (`self.ServerBarrel`))

(event `ClientBarrel`
  (bind _aspc_coatofarms (cast `/coatofarms/Assets/PC_coatofarms` (`Pawn.GetController` (stale `self.InteractionStart` Character))))
  (if (>= (`BlueprintMapLibrary.Map_Find` (`/coatofarms/Assets/PC_coatofarms.Inventory` _aspc_coatofarms) "Grapejuice") 1)
    (`/coatofarms/Assets/PC_coatofarms.InventoryUpdate` _aspc_coatofarms "Grapejuice" -1)
    (`|SpawnActorFromClass` "/coatofarms/Assets/coat/CraftableItems/BP_WineBarrel.BP_WineBarrel_C" (`SceneComponent.K2_GetComponentToWorld` (`self.Scene`)) "Undefined" "OverrideRootScale" null null)))

(event `ServerBarrel`
  (`self.ClientBarrel`))

(event `BagServer`)

(fn `BagClient`)

(fn `UserConstructionScript`
  (`parent.UserConstructionScript`))