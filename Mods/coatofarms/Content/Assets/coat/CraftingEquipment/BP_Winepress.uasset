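; BP_Winepress is a crafting station that presses grapes into grape juice when a character interacts with it.
; On interaction start it casts the character's controller to PC_coatofarms and looks up Grape in that controller's inventory.
; With at least twenty grapes, it removes twenty and adds one Grapejuice through InventoryUpdate, with no delay or feedback in this graph.
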(event `self.InteractionStart`
  (params (Character :type "MordhauCharacter Object Reference"))
  (bind _aspc_coatofarms (cast `/coatofarms/Assets/PC_coatofarms` (`Pawn.GetController` Character)))
  (bind (_value _returnvalue) (`BlueprintMapLibrary.Map_Find` (`/coatofarms/Assets/PC_coatofarms.Inventory` _aspc_coatofarms) "Grape"))
  (if _returnvalue
    (if (>= _value 20)
      (`/coatofarms/Assets/PC_coatofarms.InventoryUpdate` _aspc_coatofarms "Grape" -20)
      (`/coatofarms/Assets/PC_coatofarms.InventoryUpdate` _aspc_coatofarms "Grapejuice" 1))))

(fn `UserConstructionScript`
  (`parent.UserConstructionScript`))