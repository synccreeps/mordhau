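; BP_Woodcutter is a crafting station that turns a Log from the player's inventory into planks.
; InteractionStart deducts one Log from the inventory and shows the Log component, whose visibility also marks the station as loaded.
; AnyDamage counts left or right strikes from axe, hand axe or battle axe weapons while loaded.
; At the hit threshold it spawns three BP_Plank actors at scene component transforms, resets the count and hides the log.
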(event `self.InteractionStart`
  (params (Character :type "MordhauCharacter Object Reference"))
  (if (not (`SceneComponent.IsVisible` (`self.Log`)))
    (bind _aspc_coatofarms (cast `/coatofarms/Assets/PC_coatofarms` (`Pawn.GetController` Character)))
    (bind (_value _returnvalue) (`BlueprintMapLibrary.Map_Find` (`/coatofarms/Assets/PC_coatofarms.Inventory` _aspc_coatofarms) "Log"))
    (if _returnvalue
      (if (>= _value 1)
        (`/coatofarms/Assets/PC_coatofarms.InventoryUpdate` _aspc_coatofarms "Log" -1)
        (`SceneComponent.SetVisibility` (`self.Log`) true false)))))

(event `self.ReceiveAnyDamage`
  (params (Damage :type "Float (single-precision)") (DamageType :type "DamageType Object Reference") (InstigatedBy :type "Controller Object Reference") (DamageCauser :type "Actor Object Reference"))
  (bind _log (`self.Log`))
  (if (`SceneComponent.IsVisible` _log)
    (bind _asmc_coatofarms (cast `/coatofarms/Assets/MC_coatofarms` DamageCauser))
    (bind _asattack_motion (cast `AttackMotion` (`MordhauCharacter.Motion` _asmc_coatofarms)))
    (bind _move (`AttackMotion.Move` _asattack_motion))
    (if (or (`|EnumEquality` _move "RightStrike") (`|EnumEquality` _move "LeftStrike"))
      (bind _weapon (`AttackMotion.Weapon` _asattack_motion))
      (if (== (`GameplayStatics.GetObjectClass` _weapon) "/Game/Mordhau/Blueprints/Equipment/Weapons/Specific/OneHanded/BP_Axe.BP_Axe_C")
        (bind _output_get (set `self.Total Hits` (+ (`self.Total Hits`) 1)))
        (if (>= _output_get 2)
          (`|SpawnActorFromClass` "/coatofarms/Assets/coat/CraftableItems/BP_Plank.BP_Plank_C" (`SceneComponent.K2_GetComponentToWorld` (`self.Scene`)) "Undefined" "OverrideRootScale" null null :!label _label)
          (`|SpawnActorFromClass` "/coatofarms/Assets/coat/CraftableItems/BP_Plank.BP_Plank_C" (`SceneComponent.K2_GetComponentToWorld` (`self.Scene1`)) "Undefined" "OverrideRootScale" null null)
          (`|SpawnActorFromClass` "/coatofarms/Assets/coat/CraftableItems/BP_Plank.BP_Plank_C" (`SceneComponent.K2_GetComponentToWorld` (`self.Scene2`)) "Undefined" "OverrideRootScale" null null)
          (set `self.Total Hits` 0)
          (`SceneComponent.SetVisibility` _log false false))
        (elif (or (== (`GameplayStatics.GetObjectClass` _weapon) "/Game/Mordhau/Blueprints/Equipment/Weapons/Specific/OneHanded/BP_HandAxe.BP_HandAxe_C") (== (`GameplayStatics.GetObjectClass` _weapon) "/Game/Mordhau/Blueprints/Equipment/Weapons/Specific/Polearms/BP_BattleAxe.BP_BattleAxe_C"))
          (bind _output_get_2 (set `self.Total Hits` (+ (`self.Total Hits`) 1)))
          (if (>= _output_get_2 2)
            (goto _label)))))))

(fn `UserConstructionScript`
  (`parent.UserConstructionScript`))