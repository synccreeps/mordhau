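; BP_RemovedHelmetComponent undoes helmet removal when a character dies, so the player does not respawn without a helmet.
; AssignCharacterAndProfile caches the assigned character's current Profile (ignoring its Profile parameter) and binds to that character's death event.
; On death, RestoreOriginalProfile casts to MordhauCharacter and reapplies the cached profile through its customization replication actor.
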(event `AssignCharacterAndProfile`
  (params (AssignedCharacter :type "MordhauCharacter Object Reference") (Profile :type "CharacterProfile Structure"))
  (`/Engine/EditorBlueprintResources/StandardMacros.IsValid` AssignedCharacter
    (:`Is Valid`
      (set `self.OriginalProfile` (`MordhauCharacter.Profile` AssignedCharacter))
      (add `AdvancedCharacter.OnCharacterDied` AssignedCharacter (delegate `RestoreOriginalProfile`)))))

(event `RestoreOriginalProfile`
  (params (Character :type "AdvancedCharacter Object Reference"))
  (`/Engine/EditorBlueprintResources/StandardMacros.IsValid` Character
    (:`Is Valid`
      (bind _asmordhau_character (cast `MordhauCharacter` Character))
      (bind _returnvalue (`MordhauCharacter.GetCustomizationReplicationActor` _asmordhau_character))
      (`/Engine/EditorBlueprintResources/StandardMacros.IsValid` _returnvalue
        (:`Is Valid`
          (`CustomizationReplicationActor.AssignDataFromProfile` _returnvalue (`self.OriginalProfile`)))))))