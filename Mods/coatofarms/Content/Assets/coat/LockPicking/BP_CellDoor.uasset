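; BP_CellDoor is a cell door with a lock component that automatically relocks some time after being unlocked.
; Each Tick runs the parent logic, then checks whether both the door and BPLockComponent are unlocked.
; If so, a 20-second Delay leads to resetting DoorState and setting both locks again, with debug prints along the way.
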(event `self.ReceiveTick`
  (params (DeltaSeconds :type "Float (single-precision)"))
  (bind _bp_lockcomponent (`self.BP_LockComponent`))
  (`parent.ReceiveTick` DeltaSeconds)
  (if (`self.IsLocked`)
    _
    (elif (not (`/coatofarms/Assets/coat/LockPicking/Blueprints/BP_LockComponent.Locked?` _bp_lockcomponent))
      (`KismetSystemLibrary.PrintString` "Unlocked")
      (`KismetSystemLibrary.Delay` 20.0)
      (set `self.DoorState` 0)
      (set `self.IsLocked` true)
      (`KismetSystemLibrary.PrintString` "Locking")
      (set `/coatofarms/Assets/coat/LockPicking/Blueprints/BP_LockComponent.Locked?` true _bp_lockcomponent))))

(fn `UserConstructionScript`
  (`parent.UserConstructionScript`))