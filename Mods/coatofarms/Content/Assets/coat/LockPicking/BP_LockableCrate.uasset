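; BP_LockableCrate is a crate actor in the LockPicking folder that spawns loot when play begins; it contains no lock logic in its own graphs.
; BeginPlay passes through a DoOnce into the SpawnActorServer event, which spawns a BP_ItemBag at the Scene component's location, preset with a small stack of Copper Coin.
; The parent BeginPlay call is disconnected, and the overlap and tick events are disabled.
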(event `SpawnActorServer`
  (`|SpawnActorFromClass` "/coatofarms/Assets/coat/BP_ItemBag.BP_ItemBag_C" (`KismetMathLibrary.Conv_VectorToTransform` (`SceneComponent.K2_GetComponentLocation` (`self.Scene`))) "Undefined" "OverrideRootScale" null "Copper Coin" 5 null))

(event `self.ReceiveBeginPlay`
  (`/Engine/EditorBlueprintResources/StandardMacros.DoOnce` false
    (:`Completed`
      (`self.SpawnActorServer`))))

(fn `UserConstructionScript`
  (`parent.UserConstructionScript`))