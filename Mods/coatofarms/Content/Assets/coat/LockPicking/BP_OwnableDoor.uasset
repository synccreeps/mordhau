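; BP_OwnableDoor is a door variant that a player holding Land can lock with a held interaction.
; When the held interaction starts, it runs the parent logic, then looks up Land in the PC_coatofarms controller's inventory.
; With at least one, it sets both its own IsLocked flag and BPLockComponent's Locked flag to true.
; It has no unlock logic of its own.
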(event `self.HeldInteractionStart`
  (params (Character :type "MordhauCharacter Object Reference"))
  (`parent.HeldInteractionStart` Character)
  (bind _aspc_coatofarms (cast `/coatofarms/Assets/PC_coatofarms` (`self.GetInstigatorController` Character)))
  (if (>= (`BlueprintMapLibrary.Map_Find` (`/coatofarms/Assets/PC_coatofarms.Inventory` _aspc_coatofarms) (`self.Land`)) 1)
    (set `self.IsLocked` true)
    (set `/coatofarms/Assets/coat/LockPicking/Blueprints/BP_LockComponent.Locked?` true (`self.BP_LockComponent`))))

(fn `UserConstructionScript`
  (`parent.UserConstructionScript`))