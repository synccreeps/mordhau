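; Player character component that detects lockable objects and launches the lockpicking minigame.
; For the locally controlled player it creates a HUD and runs a looping timer trace from the camera, normally only while stationary, caching the hit lock component and updating the info box.
; CheckForLock reports unlocked objects or calls PickLock, which requires lockpicks, disables input, then spawns and configures a BP_Lockpicking actor in front of the camera.
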(event `self.ReceiveBeginPlay`
  (bind _asmc_coatofarms (cast `/coatofarms/Assets/MC_coatofarms` (`self.GetOwner`)))
  ;[0.02315 0.2918 0.0137] Begin Play - Create HUD and Set Instance
  (if (`Pawn.IsLocallyControlled` _asmc_coatofarms)
    (bind _returnvalue (`|CreateWidget` "/coatofarms/Assets/coat/LockPicking/UserInterface/UI_LockpickingHUD.UI_LockpickingHUD_C"))
    (bind _output_get (set `self.LockInfoHUD` _returnvalue))
    (`UserWidget.AddToViewport` _output_get 0)
    (`KismetSystemLibrary.K2_SetTimerDelegate` (delegate `TraceForLock`) (`.TraceInterval_8_3019EE3249C2B2498BDADDBD4955AB28` (break `/coatofarms/Assets/coat/LockPicking/Blueprints/Core/Lockpicking_Settings` (`self.Settings`))) true)))

(event `TraceForLock`
  (bind _lockinfohud (`self.LockInfoHUD`))
  (bind _lockinfohud_2 (`self.LockInfoHUD`))
  (bind _asmc_coatofarms (cast `/coatofarms/Assets/MC_coatofarms` (`self.GetOwner`) :!pure true))
  ;[0.02315 0.2918 0.0137] Trace for a locked object
  (bind _aspc_coatofarms (cast `/coatofarms/Assets/PC_coatofarms` (`Pawn.GetController` _asmc_coatofarms)))
  (if (and (or (`KismetMathLibrary.NearlyEqual_FloatFloat` (`KismetMathLibrary.VSize` (`Actor.GetVelocity` (`self.GetOwner`))) 0.0 1.0) (`.TraceWhileMoving_5_6BC6CD0140C89C0A35B0A4B74214AD26` (break `/coatofarms/Assets/coat/LockPicking/Blueprints/Core/Lockpicking_Settings` (`self.Settings`)))) (not (`self.Busy`)))
    (bind _playercameramanager (`PlayerController.PlayerCameraManager` _aspc_coatofarms))
    (bind _returnvalue (`PlayerCameraManager.GetCameraLocation` _playercameramanager))
    (bind (_outhit _returnvalue_2) (`KismetSystemLibrary.LineTraceSingle` _returnvalue (+ _returnvalue (* (`Actor.GetActorForwardVector` _playercameramanager) (`.TraceDistance_2_EB4AF29C4724A149589B738D7BAD972B` (break `/coatofarms/Assets/coat/LockPicking/Blueprints/Core/Lockpicking_Settings` (`self.Settings`))))) "TraceTypeQuery1" false (`|MakeArray` _asmc_coatofarms :!type "Actor Object Reference")))
    (if _returnvalue_2
      (bind (_bblockinghit _binitialoverlap _time _distance _location _impactpoint _normal _impactnormal _physmat _hitactor) (`GameplayStatics.BreakHitResult` _outhit))
      (`/Engine/EditorBlueprintResources/StandardMacros.IsValid` _hitactor
        (:`Is Valid`
          (set `self.FocusedActor` _hitactor)
          (bind _returnvalue_3 (`Actor.GetComponentByClass` _hitactor "/coatofarms/Assets/coat/LockPicking/Blueprints/BP_LockComponent.BP_LockComponent_C"))
          (`/Engine/EditorBlueprintResources/StandardMacros.IsValid` _returnvalue_3
            (:`Is Valid`
              (bind _output_get (set `self.Lock` _returnvalue_3))
              (`/coatofarms/Assets/coat/LockPicking/Blueprints/BP_LockComponent.SetHUDInfo` _output_get (`self.LockInfoHUD`))
              (set `/coatofarms/Assets/coat/LockPicking/UserInterface/UI_LockpickingHUD.Lockpicks` (`KismetTextLibrary.Conv_IntToText` (`self.LockPicks`)) _lockinfohud_2)
              (set `/coatofarms/Assets/coat/LockPicking/UserInterface/UI_LockpickingHUD.InfoBoxVisible?` true _lockinfohud_2))
            (:`Is Not Valid`
              (if (`Actor.ActorHasTag` _hitactor "LockpickBox")
                (set `/coatofarms/Assets/coat/LockPicking/UserInterface/UI_LockpickingHUD.IsLocked?` false _lockinfohud)
                (set `/coatofarms/Assets/coat/LockPicking/UserInterface/UI_LockpickingHUD.ObjectNameText` "LockpickBox" _lockinfohud)
                (set `/coatofarms/Assets/coat/LockPicking/UserInterface/UI_LockpickingHUD.InfoBoxVisible?` true _lockinfohud)
                (else
                  (set `self.Lock` null :!label _label)
                  (set `/coatofarms/Assets/coat/LockPicking/UserInterface/UI_LockpickingHUD.InfoBoxVisible?` false (`self.LockInfoHUD`)))))))
        (:`Is Not Valid`
          (set `self.FocusedActor` null :!label _label_2)
          (goto _label)))
      (else
        (goto _label_2)))
    (else
      (goto _label_2))))

(event `PickLock`
  (bind _returnvalue (`self.GetOwner`))
  (bind _lockinfohud (`self.LockInfoHUD`))
  (bind _lock (`self.Lock`))
  (bind _asmc_coatofarms (cast `/coatofarms/Assets/MC_coatofarms` _returnvalue :!pure true))
  ;[0.02315 0.2918 0.0137] Pick Lock
  ;[0.02315 0.2918 0.0137] Has enough lockpicks?
  (if (>= (`self.LockPicks`) 1)
    ;[0.02315 0.2918 0.0137] Disable Input and wait until player stands still
    ;;[1 1 1] Added by US
    (bind _aspc_coatofarms (cast `/coatofarms/Assets/PC_coatofarms` (`Pawn.GetController` _asmc_coatofarms)))
    (`Actor.DisableInput` (`Actor.GetInstigator` _returnvalue) _aspc_coatofarms)
    (`KismetSystemLibrary.Delay` 0.5) ; Make sure Character is not moving anymore
    (bind _playercameramanager (`PlayerController.PlayerCameraManager` _aspc_coatofarms))
    ;[0.02315 0.2918 0.0137] Spawn Lock in front of Character, set difficulty and object information
    (bind _returnvalue_2 (`|SpawnActorFromClass` "/coatofarms/Assets/coat/LockPicking/Blueprints/Core/BP_Lockpicking.BP_Lockpicking_C" (`KismetMathLibrary.MakeTransform` (+ (`PlayerCameraManager.GetCameraLocation` _playercameramanager) (* (`Actor.GetActorForwardVector` _playercameramanager) 40.0)) (`PlayerCameraManager.GetCameraRotation` _playercameramanager)) "AlwaysSpawn" "OverrideRootScale" null _asmc_coatofarms null))
    (set `/coatofarms/Assets/coat/LockPicking/Blueprints/Core/BP_Lockpicking.LockPickingComponent` self _returnvalue_2)
    (set `/coatofarms/Assets/coat/LockPicking/Blueprints/Core/BP_Lockpicking.LockedObject` _lock _returnvalue_2)
    (`/coatofarms/Assets/coat/LockPicking/Blueprints/Core/BP_Lockpicking.LockSetup` _returnvalue_2 (`/coatofarms/Assets/coat/LockPicking/Blueprints/BP_LockComponent.LockDifficulty` _lock))
    (set `self.Busy` true)
    (else
      ;[0.02315 0.2918 0.0137] Show no lockpicks notification
      (`TextBlock.SetText` (`/coatofarms/Assets/coat/LockPicking/UserInterface/UI_LockpickingHUD.NotificationText` (`self.LockInfoHUD`)) "You don't have lockpicks left.")
      (`UserWidget.PlayAnimation` _lockinfohud (`/coatofarms/Assets/coat/LockPicking/UserInterface/UI_LockpickingHUD.Notification` _lockinfohud) 0.0 1 "Forward" 1.0 false))))

(fn `CheckForLock`
  (returns (Unlocked :type Boolean) (LockedActor :type "Actor Object Reference"))
  (bind _lock (`self.Lock`))
  (`self.Lock`
    (:`then`
      (if (`/coatofarms/Assets/coat/LockPicking/Blueprints/BP_LockComponent.Locked?` _lock)
        (`self.PickLock`)
        (return false null)
        (else
          (return true (`self.GetOwner` _lock)))))
    (:`else`
      (return false null))))