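; BP_LockpickBox is a pickup that grants lockpicks to the player and then destroys itself.
; Its construction script can randomize the box's lockpick count within a set range.
; Pressing E adds that count once if the pawn's BP_LockPickingComponent is below its maximum, without clamping the total.
; It then shows an animated, string-table-based notification on UI_LockpickingHUD and plays a pickup sound.
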(event `Key|E`
  (params (Key :type "Key Structure"))
  (bind _lockpicksinbox (`self.LockpicksInBox`))
  (bind _returnvalue (`self.GetComponentByClass` (`GameplayStatics.GetPlayerPawn` 0) "/coatofarms/Assets/coat/LockPicking/Blueprints/BP_LockPickingComponent.BP_LockPickingComponent_C"))
  ;[0.02315 0.2918 0.0137] Check if lockpicks are full
  (:`Pressed`
    (if (< (`/coatofarms/Assets/coat/LockPicking/Blueprints/BP_LockPickingComponent.LockPicks` _returnvalue) (`/coatofarms/Assets/coat/LockPicking/Blueprints/BP_LockPickingComponent.MaxLockpicks` _returnvalue))
      ;[0.02315 0.2918 0.0137] Add amount of lockpicks, then destroy box
      (`/Engine/EditorBlueprintResources/StandardMacros.DoOnce` false
        (:`Completed`
          (set `/coatofarms/Assets/coat/LockPicking/Blueprints/BP_LockPickingComponent.LockPicks` (+ (`/coatofarms/Assets/coat/LockPicking/Blueprints/BP_LockPickingComponent.LockPicks` _returnvalue) (`self.LockpicksInBox`)) _returnvalue)
          (bind _foundwidgets (`WidgetBlueprintLibrary.GetAllWidgetsOfClass` "/coatofarms/Assets/coat/LockPicking/UserInterface/UI_LockpickingHUD.UI_LockpickingHUD_C"))
          (bind _output (`|GetArrayItem` _foundwidgets))
          (`TextBlock.SetText` (`/coatofarms/Assets/coat/LockPicking/UserInterface/UI_LockpickingHUD.NotificationText` _output) (`KismetTextLibrary.Conv_StringToText` (`KismetStringLibrary.Concat_StrStr` (`.OutKey` (`KismetTextLibrary.StringTableIdAndKeyFromText` "Collected")) " " (`KismetStringLibrary.Conv_IntToString` _lockpicksinbox) (select `bool` (> _lockpicksinbox 1) :`false` (`.OutKey` (`KismetTextLibrary.StringTableIdAndKeyFromText` "Lockpick")) :`true` (`.OutKey` (`KismetTextLibrary.StringTableIdAndKeyFromText` "Lockpicks"))) ".")))
          (`UserWidget.PlayAnimation` _output (`/coatofarms/Assets/coat/LockPicking/UserInterface/UI_LockpickingHUD.Notification` _output) 0.0 1 "Forward" 1.0 false)
          (`GameplayStatics.PlaySound2D` "/coatofarms/Assets/coat/LockPicking/Sound/Cues/SC_TakeLockpicks.SC_TakeLockpicks" 1.0 1.0 0.0 null null)
          (`self.K2_DestroyActor`))))))

(fn `UserConstructionScript`
  (if (`self.RandomInRange?`)
    (set `self.LockpicksInBox` (`KismetMathLibrary.RandomIntegerInRange` (`self.RangeMin`) (`self.RangeMax`)))))