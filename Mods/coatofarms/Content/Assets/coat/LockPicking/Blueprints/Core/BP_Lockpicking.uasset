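; Lockpicking minigame actor: mouse X rotates the pick toward a random target angle, and the Move Right axis turns the lock.
; Difficulty sets tolerance and pick damage, and tolerance tightens as the cylinder turns.
; Forcing a misaligned lock wiggles it and damages the pick until it breaks, consuming one from LockPickingComponent.
; A full turn unlocks LockedObject; success, quitting or running out of picks updates the HUD and destroys the actor.
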(event `ClientOpenLock`
  (bind _widgetinstance (`self.WidgetInstance`))
  ;[0.02315 0.2918 0.0137] Open Lock
  (`/Engine/EditorBlueprintResources/StandardMacros.DoOnce` false
    (:`Completed`
      (`GameplayStatics.PlaySound2D` "/coatofarms/Assets/coat/LockPicking/Sound/Cues/SC_OpenLock.SC_OpenLock" 1.0 1.0 0.0 null null)
      (`self.DisableInput` (`GameplayStatics.GetPlayerController` 0))
      (`KismetSystemLibrary.Delay` 0.5)
      (`self.EnableInput` (`self.GetInstigator` (`GameplayStatics.GetPlayerPawn` 0)) (`GameplayStatics.GetPlayerController` 0))
      (set `/coatofarms/Assets/coat/LockPicking/Blueprints/BP_LockPickingComponent.Busy` false (`self.LockPickingComponent`))
      ;[0.9131 0.6867 0] User Interface changes - Give your UI information about the lock status here
      (set `/coatofarms/Assets/coat/LockPicking/Blueprints/BP_LockComponent.Locked?` false (`self.LockedObject`))
      (set `/coatofarms/Assets/coat/LockPicking/UserInterface/UI_LockpickingHUD.IsLocked?` false _widgetinstance)
      (set `/coatofarms/Assets/coat/LockPicking/UserInterface/UI_LockpickingHUD.InfoBoxVisible?` true _widgetinstance)
      (set `/coatofarms/Assets/coat/LockPicking/UserInterface/UI_LockpickingHUD.LockPickingInfoVisible?` false _widgetinstance)
      ;[0.02315 0.2918 0.0137] Destroy the lock
      (`self.K2_DestroyActor`))))

(event `OpenLock`
  (`self.ClientOpenLock`))

(event `LockSetup`
  (params (Difficulty :type Integer))
  (bind _widgetinstance (`self.WidgetInstance`))
  (bind ((`Lock_3_PickDamage_39_BF03744443CCCE676200DEBA4F9D4A56` _lock_3_pickdamage) (`Lock_2_PickDamage_42_5E86BABE49780E90669EB39BD08C2F12` _lock_2_pickdamage) (`Lock_1_PickDamage_43_28FF2D0A4E74D7C89F8E2D93383EB0EB` _lock_1_pickdamage) (`Lock_3_Tolerance_29_5D0109AA4D676FD568DEB1A5AEF94ABD` _lock_3_tolerance) (`Lock_2_Tolerance_31_3DAF3D1D45B345DA32CEA9BD6AC32296` _lock_2_tolerance) (`Lock_1_Tolerance_33_D237C14A45178F970E51ADB5086DAE1A` _lock_1_tolerance)) (break `/coatofarms/Assets/coat/LockPicking/Blueprints/Core/Lockpicking_Settings` (`self.Settings`)))
  ;[0.02315 0.2918 0.0137] Setup lock information
  (`/Engine/EditorBlueprintResources/StandardMacros.CompareInt` Difficulty 2
    (:`>`
      ;;[0.02315 0.2918 0.0137 1 12] Tolerance to hit the correct spot
      (set `self.ToleranceMultiplier` _lock_3_tolerance)
      ;;[0.02315 0.2918 0.0137 1 12] Set Damage Multiplier
      (set `self.DamageMultiplier` _lock_3_pickdamage)
      ;;[0.02315 0.2918 0.0137 1 12] Set Lock Type (Visual)
      (set `self.LockType` "MasterLock"))
    (:`==`
      (set `self.ToleranceMultiplier` _lock_2_tolerance)
      (set `self.DamageMultiplier` _lock_2_pickdamage)
      (set `self.LockType` "IntermediateLock"))
    (:`<`
      (set `self.ToleranceMultiplier` _lock_1_tolerance)
      (set `self.DamageMultiplier` _lock_1_pickdamage)
      (set `self.LockType` "BeginnerLock")))
  ;[0.02315 0.2918 0.0137] Set Random Target Rotation On Spawn
  (set `self.PickTarget` (`KismetMathLibrary.Conv_IntToDouble` (`KismetMathLibrary.FFloor` (`KismetMathLibrary.RandomFloatInRange` -90.0 90.0))))
  ;[0.02315 0.2918 0.0137] Create an Instance to HUD
  (set `self.WidgetInstance` (`/coatofarms/Assets/coat/LockPicking/Blueprints/BP_LockPickingComponent.LockInfoHUD` (`self.LockPickingComponent`)))
  ;[0.9131 0.6867 0] Give information to HUD
  (set `/coatofarms/Assets/coat/LockPicking/UserInterface/UI_LockpickingHUD.LockTypeText` (`self.LockType`) _widgetinstance)
  (set `/coatofarms/Assets/coat/LockPicking/UserInterface/UI_LockpickingHUD.InfoBoxVisible?` false _widgetinstance)
  (set `/coatofarms/Assets/coat/LockPicking/UserInterface/UI_LockpickingHUD.LockPickingInfoVisible?` true _widgetinstance))

(event `Key|Q`
  (params (Key :type "Key Structure"))
  ;[0.02315 0.2918 0.0137] Quit Picking on Input (Back)
  (:`Pressed`
    (`self.QuitPicking`)))

(event `InputAxisKey|MouseX`
  (params (AxisValue :type "Float (single-precision)"))
  ;[0.02315 0.2918 0.0137] PickTurn Input
  ;[0.02315 0.2918 0.0137] Rotate Pick
  (if (not (`self.MovingLock`))
    (`SceneComponent.K2_SetRelativeRotation` (`self.Pick`) (`KismetMathLibrary.MakeRotator` (`KismetMathLibrary.ClampAngle` (+ (* (`KismetMathLibrary.GridSnap_Float` AxisValue 0.2) 2.0) (.roll (`SceneComponent.RelativeRotation` (`self.Pick`)))) -90.0 90.0) (.pitch (`SceneComponent.RelativeRotation` (`self.Pick`))) (.yaw (`SceneComponent.RelativeRotation` (`self.Pick`)))) false false)))

(event `TurnLockBackToOrigin`
  (bind _innerlock (`self.InnerLock`))
  ;[0.02315 0.2918 0.0137] Automatically Turn Lock Back To Origin
  (if (not (`self.MovingLock`))
    (`SceneComponent.K2_SetRelativeRotation` _innerlock (`KismetMathLibrary.MakeRotator` -90.0 (`KismetMathLibrary.FClamp` (- (.pitch (`SceneComponent.RelativeRotation` _innerlock)) (* (`self.DeltaMultiplier`) 1.3)) 0.0 90.0) -90.0) false false)))

(event `QuitPicking`
  (bind _widgetinstance (`self.WidgetInstance`))
  ;[0.02315 0.2918 0.0137] Quit Picking and Resume to game
  (`self.DisableInput` (`GameplayStatics.GetPlayerController` 0))
  (`KismetSystemLibrary.Delay` 0.5)
  (`self.EnableInput` (`self.GetInstigator` (`GameplayStatics.GetPlayerPawn` 0)) (`GameplayStatics.GetPlayerController` 0))
  (set `/coatofarms/Assets/coat/LockPicking/Blueprints/BP_LockPickingComponent.Busy` false (`self.LockPickingComponent`))
  ;[0.9131 0.6867 0] Change Information on HUD
  (set `/coatofarms/Assets/coat/LockPicking/UserInterface/UI_LockpickingHUD.InfoBoxVisible?` true _widgetinstance)
  (set `/coatofarms/Assets/coat/LockPicking/UserInterface/UI_LockpickingHUD.LockPickingInfoVisible?` false _widgetinstance)
  ;[0.02315 0.2918 0.0137] Destroy lock
  (`self.K2_DestroyActor`))

(event `self.ReceiveTick`
  (params (DeltaSeconds :type "Float (single-precision)"))
  (bind _relativerotation (`SceneComponent.RelativeRotation` (`self.InnerLock`)))
  ;[0.02315 0.2918 0.0137] Tick
  ;[0.02315 0.2918 0.0137] Set multiplier for rotation translation depending on tickrate
  (set `self.DeltaMultiplier` (`KismetMathLibrary.Conv_IntToDouble` (`KismetMathLibrary.FCeil` (* DeltaSeconds 100.0))))
  ;[0.02315 0.2918 0.0137] Check if lock is openend, set target tolerance, turn lock back to origin
  (if (== _relativerotation (`KismetMathLibrary.MakeRotator` (.roll _relativerotation) 90.0 (.yaw _relativerotation)))
    (`self.OpenLock`)
    (else
      (set `self.DynaimcTolerance` (+ (/ (- 90.0 (.pitch (`SceneComponent.RelativeRotation` (`self.InnerLock`)))) 3.0) 2.0))
      (`self.TurnLockBackToOrigin`)
      ;[0.02315 0.2918 0.0137] Move Pick with Lock
      (`self.MovePickWithLock`))))

(event `MovePickWithLock`
  ;[0.02315 0.2918 0.0137] Move Pick with Lock (PickPosition)
  (`SceneComponent.K2_SetWorldLocation` (`self.Pick`) (`SceneComponent.K2_GetComponentLocation` (`self.PickPosition`)) false false))

(event `Wiggle`
  (bind _innerlock (`self.InnerLock`))
  (bind _pick (`self.Pick`))
  ;[0.02315 0.2918 0.0137] Wiggle Event
  (if (`self.ApplyDamage?`)
    (`self.AddPickDamage`)
    (`|MultiGate` false true
      (:`Out 0`
        ;[0.02315 0.2918 0.0137] Lock Wiggle
        (`SceneComponent.K2_SetRelativeRotation` _innerlock (`KismetMathLibrary.MakeRotator` (.roll (`SceneComponent.RelativeRotation` (`self.InnerLock`))) (+ (.pitch (`SceneComponent.RelativeRotation` (`self.InnerLock`))) 1.0) (.yaw (`SceneComponent.RelativeRotation` (`self.InnerLock`)))) false false)
        ;[0.02315 0.2918 0.0137] Pick Wiggle
        (`SceneComponent.K2_SetRelativeRotation` _pick (`KismetMathLibrary.MakeRotator` (+ (.roll (`SceneComponent.RelativeRotation` (`self.Pick`))) 0.5) (.pitch (`SceneComponent.RelativeRotation` (`self.Pick`))) (.yaw (`SceneComponent.RelativeRotation` (`self.Pick`)))) false false))
      (:`Out 11`
        (`SceneComponent.K2_SetRelativeRotation` _innerlock (`KismetMathLibrary.MakeRotator` (.roll (`SceneComponent.RelativeRotation` (`self.InnerLock`))) (- (.pitch (`SceneComponent.RelativeRotation` (`self.InnerLock`))) 1.0) (.yaw (`SceneComponent.RelativeRotation` (`self.InnerLock`)))) false false)
        (`SceneComponent.K2_SetRelativeRotation` _pick (`KismetMathLibrary.MakeRotator` (- (.roll (`SceneComponent.RelativeRotation` (`self.Pick`))) 0.5) (.pitch (`SceneComponent.RelativeRotation` (`self.Pick`))) (.yaw (`SceneComponent.RelativeRotation` (`self.Pick`)))) false false)))
    (`GameplayStatics.PlaySound2D` "/coatofarms/Assets/coat/LockPicking/Sound/Cues/SC_LockStuck.SC_LockStuck" 1.0 1.0 0.0 null null)))

(event `InputAxis|Move Right`
  (params (AxisValue :type "Float (single-precision)"))
  ;[0.02315 0.2918 0.0137] Turn Lock Input
  ;[0.02315 0.2918 0.0137] Set LockMoving to block PickTurn Input
  (bind _output_get (set `self.TurnValue` AxisValue))
  (if (> _output_get 0.0)
    (set `self.MovingLock` true)
    (else
      (set `self.MovingLock` false)
      (set `self.PickDamage` (`KismetMathLibrary.FInterpTo` (`self.PickDamage`) 0.0 (`GameplayStatics.GetWorldDeltaSeconds`) 1.0))
      (bind _rotationsound (`self.RotationSound`)
        (:`then`
          (`AudioComponent.Stop` _rotationsound))
        (:`else`
          _))))
  ;[0.02315 0.2918 0.0137] Pick at correct spot? Turn the lock
  (`self.IsPickAtRightPosition?`
    (:`No`
      ;[0.02315 0.2918 0.0137] Turn the lock a few degrees if not the correct spot, then wiggle
      (if (< (.pitch (`SceneComponent.RelativeRotation` (`self.InnerLock`))) 5.0)
        (`SceneComponent.K2_SetRelativeRotation` (`self.InnerLock`) (`KismetMathLibrary.MakeRotator` (.roll (`SceneComponent.RelativeRotation` (`self.InnerLock`))) (`KismetMathLibrary.FClamp` (+ (* _output_get (`.LockTurnSpeed_47_1E6BB1CA4565DC4EE069ABBF7EAA4AB2` (break `/coatofarms/Assets/coat/LockPicking/Blueprints/Core/Lockpicking_Settings` (`self.Settings`))) (`self.DeltaMultiplier`)) (.pitch (`SceneComponent.RelativeRotation` (`self.InnerLock`)))) 0.0 4.0) (.yaw (`SceneComponent.RelativeRotation` (`self.InnerLock`)))) false false)
        ;[0.02315 0.2918 0.0137] Apply damage to pick if still trying to turn the lock
        (if (>= (.pitch (`SceneComponent.RelativeRotation` (`self.InnerLock`))) 3.0)
          (`self.Wiggle`) ; Wiggle Fires ApplyDamage
          (bind _rotationsound_2 (`self.RotationSound`)
            (:`then`
              (`AudioComponent.Stop` _rotationsound_2))
            (:`else`)))
        (else
          (`self.Wiggle`)
          (bind _rotationsound_3 (`self.RotationSound`)
            (:`then`
              (`AudioComponent.Stop` _rotationsound_3))
            (:`else`)))))
    (:`Yes`
      (`SceneComponent.K2_SetRelativeRotation` (`self.InnerLock`) (`KismetMathLibrary.MakeRotator` (.roll (`SceneComponent.RelativeRotation` (`self.InnerLock`))) (`KismetMathLibrary.ClampAngle` (+ (* _output_get (`.LockTurnSpeed_47_1E6BB1CA4565DC4EE069ABBF7EAA4AB2` (break `/coatofarms/Assets/coat/LockPicking/Blueprints/Core/Lockpicking_Settings` (`self.Settings`))) (`self.DeltaMultiplier`)) (.pitch (`SceneComponent.RelativeRotation` (`self.InnerLock`)))) 0.0 90.0) (.yaw (`SceneComponent.RelativeRotation` (`self.InnerLock`)))) false false)
      (bind _rotationsound_4 (`self.RotationSound`)
        (:`then`
          (if (not (`AudioComponent.IsPlaying` _rotationsound_4))
            (`AudioComponent.Play` _rotationsound_4 0.0)))
        (:`else`
          (bind _returnvalue (`GameplayStatics.SpawnSound2D` "/coatofarms/Assets/coat/LockPicking/Sound/Cues/SC_LockRotation.SC_LockRotation" 1.0 1.0 0.0 null))
          (bind _output_get_2 (set `self.RotationSound` _returnvalue))
          (`AudioComponent.Play` _output_get_2 0.0))))))

(event `AddPickDamage`
  (bind _lockpickingcomponent (`self.LockPickingComponent`))
  (bind _pick (`self.Pick`))
  ;[0.02315 0.2918 0.0137] Add Pick Damage
  (if (`self.ApplyDamage?`)
    (`ForceFeedbackComponent.Play` (`self.ForceFeedback`) 0.0)
    (bind _output_get (set `self.PickDamage` (`KismetMathLibrary.FClamp` (+ (`self.PickDamage`) (* (+ (`GameplayStatics.GetWorldDeltaSeconds`) 0.2) (`self.DamageMultiplier`))) 0.0 11.0)))
    (if (>= _output_get 10.0)
      ;[0.02315 0.2918 0.0137] Break Pick
      (`self.DisableInput` (`GameplayStatics.GetPlayerController` 0))
      (`GameplayStatics.PlaySound2D` "/coatofarms/Assets/coat/LockPicking/Sound/Cues/SC_LockPickBreak.SC_LockPickBreak" 1.0 1.0 0.0 null null)
      (`SceneComponent.K2_SetRelativeRotation` _pick (`KismetMathLibrary.MakeRotator` (.roll (`SceneComponent.RelativeRotation` _pick)) 25.0 -25.0) false false)
      (`SceneComponent.K2_SetRelativeLocation` (`self.PickPosition`) (`KismetMathLibrary.MakeVector` (.x (`SceneComponent.RelativeLocation` (`self.PickPosition`))) (- (.y (`SceneComponent.RelativeLocation` (`self.PickPosition`))) 1.0) (+ (.z (`SceneComponent.RelativeLocation` (`self.PickPosition`))) 10.0)) false false)
      (`KismetSystemLibrary.Delay` 1.0)
      (`SceneComponent.SetVisibility` _pick false false)
      (`SceneComponent.K2_SetRelativeRotation` _pick (`self.OriginRotation`) false false)
      (`SceneComponent.K2_SetRelativeLocation` (`self.PickPosition`) (`KismetMathLibrary.MakeVector` (.x (`SceneComponent.RelativeLocation` (`self.PickPosition`))) (+ (.y (`SceneComponent.RelativeLocation` (`self.PickPosition`))) 1.0) (- (.z (`SceneComponent.RelativeLocation` (`self.PickPosition`))) 10.0)) false false)
      (`KismetSystemLibrary.Delay` 0.4)
      (set `self.ApplyDamage?` false)
      ;[0.02315 0.2918 0.0137] Remove one Lockpick from Player or Inventory Instance
      (bind _output_get_2 (set `/coatofarms/Assets/coat/LockPicking/Blueprints/BP_LockPickingComponent.LockPicks` (- (`/coatofarms/Assets/coat/LockPicking/Blueprints/BP_LockPickingComponent.LockPicks` _lockpickingcomponent) 1) _lockpickingcomponent))
      (set `/coatofarms/Assets/coat/LockPicking/UserInterface/UI_LockpickingHUD.Lockpicks` (`KismetTextLibrary.Conv_IntToText` _output_get_2) (`self.WidgetInstance`))
      (if (< _output_get_2 1)
        (`self.QuitPicking`)
        (else
          ;[0.02315 0.2918 0.0137] Make pick visible and enable input again
          (`SceneComponent.SetVisibility` _pick true false)
          (set `self.PickDamage` 0.0)
          (`self.EnableInput` (`GameplayStatics.GetPlayerController` 0))
          (`KismetSystemLibrary.Delay` 0.5)
          (set `self.ApplyDamage?` true))))))

(fn `UserConstructionScript`
  (set `self.OriginRotation` (`SceneComponent.RelativeRotation` (`self.Pick`))))