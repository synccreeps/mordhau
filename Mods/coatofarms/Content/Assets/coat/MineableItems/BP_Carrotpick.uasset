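; BP_Carrotpick is a carrot pickup that a character collects by interacting with it.
; On InteractionStart it casts the character's controller to PC_coatofarms and calls InventoryUpdate to add one Carrot.
; It then plays a 2D grass footstep sound and destroys itself; if the cast fails, nothing happens.
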(event `self.InteractionStart`
  (params (Character :type "MordhauCharacter Object Reference"))
  (bind _aspc_coatofarms (cast `/coatofarms/Assets/PC_coatofarms` (`Pawn.GetController` Character)))
  (`/coatofarms/Assets/PC_coatofarms.InventoryUpdate` _aspc_coatofarms "Carrot" 1)
  (`GameplayStatics.PlaySound2D` "/Game/Mordhau/Audio/Raw/Footsteps/Grass/SW_Footstep_Grass06.SW_Footstep_Grass06" 1.0 1.0 0.0 null null)
  (`self.K2_DestroyActor`))

(fn `UserConstructionScript`
  (`parent.UserConstructionScript`))