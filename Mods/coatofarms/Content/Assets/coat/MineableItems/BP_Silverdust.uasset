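; BP_Silverdust is an interactable Silverdust pickup among the mineable items.
; On InteractionStart it casts the interacting character's controller to PC_coatofarms, adds one Silverdust through InventoryUpdate, then destroys itself.
; If the cast fails, nothing happens and the actor stays in the world.
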(event `self.InteractionStart`
  (params (Character :type "MordhauCharacter Object Reference"))
  (bind _aspc_coatofarms (cast `/coatofarms/Assets/PC_coatofarms` (`Pawn.GetController` Character)))
  (`/coatofarms/Assets/PC_coatofarms.InventoryUpdate` _aspc_coatofarms "Silverdust" 1)
  (`self.K2_DestroyActor`))

(fn `UserConstructionScript`
  (`parent.UserConstructionScript`))