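; BP_Wheat is a harvestable wheat actor that a character cuts with a scythe.
; Box overlap requires an MC_coatofarms in a RightStrike attack with BP_Scythe; the condition tests RightStrike twice, so LeftStrike never qualifies.
; After a short delay it plays a random sound, and the authority spawns BP_Wheatpackaged and destroys the wheat.
; An older damage-causer version accepting both strikes is left disconnected, and AnyDamage is empty.
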(event `self.ReceiveAnyDamage`
  (params (Damage :type "Float (single-precision)") (DamageType :type "DamageType Object Reference") (InstigatedBy :type "Controller Object Reference") (DamageCauser :type "Actor Object Reference")))

(event `self.Box.OnComponentBeginOverlap`
  (params (OverlappedComponent :type "PrimitiveComponent Object Reference") (OtherActor :type "Actor Object Reference") (OtherComp :type "PrimitiveComponent Object Reference") (OtherBodyIndex :type Integer) (bFromSweep :type Boolean) (SweepResult :type "HitResult Structure (by ref)"))
  (bind _scene1 (`self.Scene1`))
  (bind _asmc_coatofarms (cast `/coatofarms/Assets/MC_coatofarms` OtherActor))
  (bind _asattack_motion (cast `AttackMotion` (`MordhauCharacter.Motion` _asmc_coatofarms)))
  (bind _move (`AttackMotion.Move` _asattack_motion))
  (if (and (or (`|EnumEquality` _move "RightStrike") (`|EnumEquality` _move "RightStrike")) (== (`GameplayStatics.GetObjectClass` (`AttackMotion.Weapon` _asattack_motion)) "/Game/Mordhau/Blueprints/Equipment/Weapons/Specific/Makeshift/BP_Scythe.BP_Scythe_C"))
    (`KismetSystemLibrary.Delay` 0.2)
    (`GameplayStatics.PlaySoundAtLocation` (`KismetArrayLibrary.Array_Random` (`self.Sound`)) (`SceneComponent.K2_GetComponentLocation` _scene1) (struct) 1.0 1.0 0.0 null null null)
    (`/Engine/EditorBlueprintResources/ActorMacros.Switch Has Authority`
      (:`Authority`
        (`|SpawnActorFromClass` "/coatofarms/Assets/coat/MineableItems/BP_Wheatpackaged.BP_Wheatpackaged_C" (`SceneComponent.K2_GetComponentToWorld` _scene1) "Undefined" "OverrideRootScale" null null)
        (`self.K2_DestroyActor`)))))

(fn `UserConstructionScript`
  (`parent.UserConstructionScript`))