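; Apple tree actor that spawns a batch of BP_Apple actors at BeginPlay.
; Each of the seven spawns independently picks a random transform from twelve Scene components, so apples can share a spot.
; A trailing DoOnce waits on a delay and resets itself but triggers no further spawning, so apples never regrow here.
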(event `self.ReceiveBeginPlay`
  (bind _outitem (`KismetArrayLibrary.Array_Random` (`|MakeArray` (`SceneComponent.K2_GetComponentToWorld` (`self.Scene`)) (`SceneComponent.K2_GetComponentToWorld` (`self.scene1`)) (`SceneComponent.K2_GetComponentToWorld` (`self.Scene2`)) (`SceneComponent.K2_GetComponentToWorld` (`self.Scene3`)) (`SceneComponent.K2_GetComponentToWorld` (`self.Scene4`)) (`SceneComponent.K2_GetComponentToWorld` (`self.Scene5`)) (`SceneComponent.K2_GetComponentToWorld` (`self.Scene6`)) (`SceneComponent.K2_GetComponentToWorld` (`self.Scene7`)) (`SceneComponent.K2_GetComponentToWorld` (`self.Scene8`)) (`SceneComponent.K2_GetComponentToWorld` (`self.Scene9`)) (`SceneComponent.K2_GetComponentToWorld` (`self.Scene10`)) (`SceneComponent.K2_GetComponentToWorld` (`self.Scene11`)))))
  (`|SpawnActorFromClass` "/coatofarms/Assets/coat/MineableItems/BP_Apple.BP_Apple_C" _outitem "Undefined" "OverrideRootScale" null null)
  (`|SpawnActorFromClass` "/coatofarms/Assets/coat/MineableItems/BP_Apple.BP_Apple_C" _outitem "Undefined" "OverrideRootScale" null null)
  (`|SpawnActorFromClass` "/coatofarms/Assets/coat/MineableItems/BP_Apple.BP_Apple_C" _outitem "Undefined" "OverrideRootScale" null null)
  (`|SpawnActorFromClass` "/coatofarms/Assets/coat/MineableItems/BP_Apple.BP_Apple_C" _outitem "Undefined" "OverrideRootScale" null null)
  (`|SpawnActorFromClass` "/coatofarms/Assets/coat/MineableItems/BP_Apple.BP_Apple_C" _outitem "Undefined" "OverrideRootScale" null null)
  (`|SpawnActorFromClass` "/coatofarms/Assets/coat/MineableItems/BP_Apple.BP_Apple_C" _outitem "Undefined" "OverrideRootScale" null null)
  (`|SpawnActorFromClass` "/coatofarms/Assets/coat/MineableItems/BP_Apple.BP_Apple_C" _outitem "Undefined" "OverrideRootScale" null null)
  (`/Engine/EditorBlueprintResources/StandardMacros.DoOnce` false :!label _label
    (:`Completed`
      (`KismetSystemLibrary.Delay` 5.0)
      (goto _label :!via `Reset`))))

(fn `UserConstructionScript`)