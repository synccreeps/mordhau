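; Choppable apple tree for Mordhau that drops wood when struck by axes.
; AnyDamage counts left or right strikes from three axe types, with hit threshold and wood yield varying by weapon, spawning at the Scene component.
; A completed chop hides the tree and disables mesh collision, then restores collision and most components after a delay.
; GetSpawnLocationObjects picks shuffled scene points but is not called in these graphs.
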(event `WoodDisappearMulti`
  (bind _staticmesh (`self.StaticMesh`))
  (`SceneComponent.SetVisibility` _staticmesh false false)
  (`SceneComponent.SetVisibility` (`self.Scene6`) false false)
  (`SceneComponent.SetVisibility` (`self.Scene10`) false false)
  (`SceneComponent.SetVisibility` (`self.Scene9`) false false)
  (`SceneComponent.SetVisibility` (`self.Scene8`) false false)
  (`SceneComponent.SetVisibility` (`self.Scene7`) false false)
  (`SceneComponent.SetVisibility` (`self.Scene11`) false false)
  (`SceneComponent.SetVisibility` (`self.Scene5`) false false)
  (`SceneComponent.SetVisibility` (`self.Scene4`) false false)
  (`SceneComponent.SetVisibility` (`self.Scene3`) false false)
  (`SceneComponent.SetVisibility` (`self.Scene2`) false false)
  (`SceneComponent.SetVisibility` (`self.scene1`) false false)
  (`SceneComponent.SetVisibility` (`self.Scene`) false false)
  (`PrimitiveComponent.SetCollisionEnabled` _staticmesh "NoCollision")
  (`KismetSystemLibrary.Delay` 10.0)
  (`PrimitiveComponent.SetCollisionEnabled` _staticmesh "QueryAndPhysics")
  (`SceneComponent.SetVisibility` _staticmesh true false)
  (`SceneComponent.SetVisibility` (`self.Scene6`) true false)
  (`SceneComponent.SetVisibility` (`self.Scene10`) true false)
  (`SceneComponent.SetVisibility` (`self.Scene9`) true false)
  (`SceneComponent.SetVisibility` (`self.Scene7`) true false)
  (`SceneComponent.SetVisibility` (`self.Scene11`) true false)
  (`SceneComponent.SetVisibility` (`self.Scene5`) true false)
  (`SceneComponent.SetVisibility` (`self.Scene3`) true false)
  (`SceneComponent.SetVisibility` (`self.Scene2`) true false)
  (`SceneComponent.SetVisibility` (`self.scene1`) true false)
  (`SceneComponent.SetVisibility` (`self.Scene`) true false))

(event `self.ReceiveAnyDamage`
  (params (Damage :type "Float (single-precision)") (DamageType :type "DamageType Object Reference") (InstigatedBy :type "Controller Object Reference") (DamageCauser :type "Actor Object Reference"))
  (bind _returnvalue (`SceneComponent.K2_GetComponentToWorld` (`self.Scene`)))
  (bind _asmordhau_character (cast `MordhauCharacter` DamageCauser))
  (bind _asattack_motion (cast `AttackMotion` (`MordhauCharacter.Motion` _asmordhau_character)))
  (bind _move (`AttackMotion.Move` _asattack_motion))
  (if (or (`|EnumEquality` _move "RightStrike") (`|EnumEquality` _move "LeftStrike"))
    (bind _weapon (`AttackMotion.Weapon` _asattack_motion))
    (if (== (`GameplayStatics.GetObjectClass` _weapon) "/Game/Mordhau/Blueprints/Equipment/Weapons/Specific/OneHanded/BP_Axe.BP_Axe_C")
      (bind _output_get (set `self.Total Hits` (+ (`self.Total Hits`) 1)))
      (if (>= _output_get 5)
        (`|SpawnActorFromClass` "/coatofarms/Assets/coat/MineableItems/BP_Wood.BP_Wood_C" _returnvalue "Undefined" "OverrideRootScale" null null)
        (set `self.Total Hits` 0 :!label _label)
        (`self.WoodDisappearMulti`))
      (elif (== (`GameplayStatics.GetObjectClass` _weapon) "/Game/Mordhau/Blueprints/Equipment/Weapons/Specific/Polearms/BP_BattleAxe.BP_BattleAxe_C")
        (bind _output_get_2 (set `self.Total Hits` (+ (`self.Total Hits`) 1)))
        (if (>= _output_get_2 5)
          (`|SpawnActorFromClass` "/coatofarms/Assets/coat/MineableItems/BP_Wood.BP_Wood_C" _returnvalue "Undefined" "OverrideRootScale" null null :!label _label_2)
          (`|SpawnActorFromClass` "/coatofarms/Assets/coat/MineableItems/BP_Wood.BP_Wood_C" _returnvalue "Undefined" "OverrideRootScale" null null)
          (goto _label))
        (elif (== (`GameplayStatics.GetObjectClass` _weapon) "/Game/Mordhau/Blueprints/Equipment/Weapons/Specific/OneHanded/BP_HandAxe.BP_HandAxe_C")
          (bind _output_get_3 (set `self.Total Hits` (+ (`self.Total Hits`) 1)))
          (if (>= _output_get_3 2)
            (goto _label_2)))))))

(fn `GetSpawnLocationObjects`
  (returns (NewParam :type "Array of SceneComponent Object Reference"))
  (locals (ChosenSpawns :type "Array of SceneComponent Object Reference") (RandomSpawns :type "Array of SceneComponent Object Reference"))
  (bind _output_get (set `local.RandomSpawns` (`|MakeArray` (`self.Scene`) (`self.scene1`) (`self.Scene2`) (`self.Scene4`) (`self.Scene3`) (`self.Scene5`) (`self.Scene6`) (`self.Scene7`) (`self.Scene8`) (`self.Scene9`) (`self.Scene10`) (`self.Scene11`))))
  (`KismetArrayLibrary.Array_Shuffle` _output_get)
  (for _index (range 7)
    (`KismetArrayLibrary.Array_Add` (`local.ChosenSpawns`) (`|GetArrayItem` (`local.RandomSpawns`) _index)))
  (return (`local.ChosenSpawns`)))

(fn `UserConstructionScript`)