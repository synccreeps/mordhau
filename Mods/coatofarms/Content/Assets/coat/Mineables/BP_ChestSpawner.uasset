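; BP_ChestSpawner is a Blueprint that supplies randomized spawn points, by its name for chests.
; GetSpawnLocationObjects shuffles an array of nine scene components plus three empty slots, then adds the first five to ChosenSpawns and returns it, so picks can include empty entries.
; It contains no spawning logic itself, and its events and construction script are empty.
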(fn `GetSpawnLocationObjects`
  (returns (NewParam :type "Array of SceneComponent Object Reference"))
  (locals (ChosenSpawns :type "Array of SceneComponent Object Reference") (RandomSpawns :type "Array of SceneComponent Object Reference"))
  (bind _output_get (set `local.RandomSpawns` (`|MakeArray` (`self.Scene`) (`self.scene1`) (`self.Scene2`) (`self.Scene4`) (`self.Scene3`) (`self.Scene5`) (`self.Scene6`) (`self.Scene7`) (`self.Scene8`) null null null)))
  (`KismetArrayLibrary.Array_Shuffle` _output_get)
  (for _index (range 5)
    (`KismetArrayLibrary.Array_Add` (`local.ChosenSpawns`) (`|GetArrayItem` (`local.RandomSpawns`) _index)))
  (return (`local.ChosenSpawns`)))

(fn `UserConstructionScript`)