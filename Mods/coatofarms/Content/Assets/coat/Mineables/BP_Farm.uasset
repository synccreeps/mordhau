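; BP_Farm is a mineable farm that periodically restocks its resource actors (carrots, per the function name).
; On BeginPlay, only the authority runs a loop that spawns one Resource actor at each of eight spawn location objects and tracks them in CurrentResources.
; After each RestockTime delay it destroys any still-valid tracked actors, then respawns the full set.
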(event `self.ReceiveBeginPlay`
  (`/Engine/EditorBlueprintResources/ActorMacros.Switch Has Authority`
    (:`Authority`
      (`self.SpawnCarrots` :!label _label)
      (`KismetSystemLibrary.Delay` (`self.RestockTime`))
      (bind (_arrayindex _arrayelement) (`/Engine/EditorBlueprintResources/StandardMacros.ReverseForEachLoop` (`self.CurrentResources`))
        (:`LoopBody`
          (`/Engine/EditorBlueprintResources/StandardMacros.IsValid` _arrayelement
            (:`Is Valid`
              (`self.K2_DestroyActor` _arrayelement))))
        (:`Completed`
          (goto _label))))))

(fn `GetSpawnLocationObjects`
  (returns (NewParam :type "Array of SceneComponent Object Reference"))
  (return (`|MakeArray` null null null null null null null null :!type "SceneComponent Object Reference")))

(fn `SpawnCarrots`
  (locals (CarrotSpawns :type "Array of SceneComponent Object Reference"))
  (`KismetArrayLibrary.Array_Clear` (`self.CurrentResources`))
  (bind _newparam (`self.GetSpawnLocationObjects`))
  (for _array_element _newparam
    (bind _returnvalue (`|SpawnActorFromClass` (`self.Resource`) (`SceneComponent.K2_GetComponentToWorld` _array_element) "Undefined" "OverrideRootScale" null null))
    (`KismetArrayLibrary.Array_Add` (`self.CurrentResources`) _returnvalue)))

(fn `UserConstructionScript`)