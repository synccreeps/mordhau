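; BP_GoldMine is a mineable gold node that spawns gold ore when struck by licensed players.
; AnyDamage checks the instigating controller's inventory for a Mining License, then reads the Mordhau attacker's motion to accept only left or right strikes.
; Every second qualifying hit spawns BP_Goldore at the Scene component and resets the counter, one ore for BP_Pickaxe and two for another weapon class.
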(event `self.ReceiveAnyDamage`
  (params (Damage :type "Float (single-precision)") (DamageType :type "DamageType Object Reference") (InstigatedBy :type "Controller Object Reference") (DamageCauser :type "Actor Object Reference"))
  (bind _returnvalue (`SceneComponent.K2_GetComponentToWorld` (`self.Scene`)))
  (bind _aspc_coatofarms (cast `/coatofarms/Assets/PC_coatofarms` InstigatedBy))
  (if (>= (`BlueprintMapLibrary.Map_Find` (`/coatofarms/Assets/PC_coatofarms.Inventory` _aspc_coatofarms) "Mining License") 1)
    (bind _asmordhau_character (cast `MordhauCharacter` DamageCauser))
    (bind _asattack_motion (cast `AttackMotion` (`MordhauCharacter.Motion` _asmordhau_character)))
    (bind _move (`AttackMotion.Move` _asattack_motion))
    (if (or (`|EnumEquality` _move "RightStrike") (`|EnumEquality` _move "LeftStrike"))
      (bind _weapon (`AttackMotion.Weapon` _asattack_motion))
      (if (== (`GameplayStatics.GetObjectClass` _weapon) "/Game/Mordhau/Blueprints/Equipment/Weapons/Specific/Makeshift/BP_Pickaxe.BP_Pickaxe_C")
        (bind _output_get (set `self.Total Hits` (+ (`self.Total Hits`) 1)))
        (if (>= _output_get 2)
          (`|SpawnActorFromClass` "/coatofarms/Assets/coat/MineableItems/BP_Goldore.BP_Goldore_C" _returnvalue "Undefined" "OverrideRootScale" null null)
          (set `self.Total Hits` 0 :!label _label))
        (elif (== (`GameplayStatics.GetObjectClass` _weapon) null)
          (bind _output_get_2 (set `self.Total Hits` (+ (`self.Total Hits`) 1)))
          (if (>= _output_get_2 2)
            (`|SpawnActorFromClass` "/coatofarms/Assets/coat/MineableItems/BP_Goldore.BP_Goldore_C" _returnvalue "Undefined" "OverrideRootScale" null null)
            (`|SpawnActorFromClass` "/coatofarms/Assets/coat/MineableItems/BP_Goldore.BP_Goldore_C" _returnvalue "Undefined" "OverrideRootScale" null null)
            (goto _label)))))))

(fn `UserConstructionScript`)