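; BP_Tree is a mineable tree for Mordhau that yields BP_Wood when chopped.
; BeginPlay picks a random mesh, and AnyDamage counts left or right strikes from three axe classes on a shared counter, with hit threshold and yield depending on the axe.
; At the threshold it spawns wood, resets, then WoodDisappearMulti swaps to the second mesh and disables collision for a fixed delay before restoring the tree.
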(event `WoodDisappearMulti`
  (bind _staticmesh (`self.StaticMesh`))
  (bind _staticmesh1 (`self.StaticMesh1`))
  (`SceneComponent.SetVisibility` _staticmesh false false)
  (`SceneComponent.SetVisibility` _staticmesh1 true false)
  (`PrimitiveComponent.SetCollisionEnabled` _staticmesh "NoCollision")
  (`PrimitiveComponent.SetCollisionEnabled` _staticmesh1 "NoCollision")
  (`KismetSystemLibrary.Delay` 10.0)
  (`PrimitiveComponent.SetCollisionEnabled` _staticmesh1 "QueryAndPhysics")
  (`PrimitiveComponent.SetCollisionEnabled` _staticmesh "QueryAndPhysics")
  (`SceneComponent.SetVisibility` _staticmesh true false)
  (`SceneComponent.SetVisibility` _staticmesh1 false false))

(event `self.ReceiveBeginPlay`
  (`StaticMeshComponent.SetStaticMesh` (`self.StaticMesh`) (`KismetArrayLibrary.Array_Random` (`self.ListOfMeshes`))))

(event `self.ReceiveAnyDamage`
  (params (Damage :type "Float (single-precision)") (DamageType :type "DamageType Object Reference") (InstigatedBy :type "Controller Object Reference") (DamageCauser :type "Actor Object Reference"))
  (bind _returnvalue (`SceneComponent.K2_GetComponentToWorld` (`self.Scene`)))
  (bind _asmordhau_character (cast `MordhauCharacter` DamageCauser))
  (bind _asattack_motion (cast `AttackMotion` (`MordhauCharacter.Motion` _asmordhau_character)))
  (bind _move (`AttackMotion.Move` _asattack_motion))
  (if (or (`|EnumEquality` _move "RightStrike") (`|EnumEquality` _move "LeftStrike"))
    (bind _weapon (`AttackMotion.Weapon` _asattack_motion))
    (if (== (`GameplayStatics.GetObjectClass` _weapon) "/Game/Mordhau/Blueprints/Equipment/Weapons/Specific/OneHanded/BP_Axe.BP_Axe_C")
      (bind _output_get (set `self.Total Hits` (+ (`self.Total Hits`) 1)))
      (if (>= _output_get 5)
        (`|SpawnActorFromClass` "/coatofarms/Assets/coat/MineableItems/BP_Wood.BP_Wood_C" _returnvalue "Undefined" "OverrideRootScale" null null)
        (set `self.Total Hits` 0 :!label _label)
        (`self.WoodDisappearMulti`))
      (elif (== (`GameplayStatics.GetObjectClass` _weapon) "/Game/Mordhau/Blueprints/Equipment/Weapons/Specific/Polearms/BP_BattleAxe.BP_BattleAxe_C")
        (bind _output_get_2 (set `self.Total Hits` (+ (`self.Total Hits`) 1)))
        (if (>= _output_get_2 5)
          (`|SpawnActorFromClass` "/coatofarms/Assets/coat/MineableItems/BP_Wood.BP_Wood_C" _returnvalue "Undefined" "OverrideRootScale" null null :!label _label_2)
          (`|SpawnActorFromClass` "/coatofarms/Assets/coat/MineableItems/BP_Wood.BP_Wood_C" _returnvalue "Undefined" "OverrideRootScale" null null)
          (goto _label))
        (elif (== (`GameplayStatics.GetObjectClass` _weapon) "/Game/Mordhau/Blueprints/Equipment/Weapons/Specific/OneHanded/BP_HandAxe.BP_HandAxe_C")
          (bind _output_get_3 (set `self.Total Hits` (+ (`self.Total Hits`) 1)))
          (if (>= _output_get_3 2)
            (goto _label_2)))))))

(fn `UserConstructionScript`)