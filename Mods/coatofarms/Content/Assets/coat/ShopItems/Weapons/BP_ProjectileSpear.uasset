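; Shop spear weapon that can launch its head as a projectile.
; On the first AltStab attack, it waits briefly, spawns a spearhead projectile at the W component's transform, fires it and hides the spearhead mesh.
; A counter blocks later launches, and nothing in this Blueprint resets it or restores the mesh, so the shot is single-use.
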(event `self.OnAttackStarted`
  (params (Move :type "EAttackMove Enum" :default "RightStrike") (Angle :type "Float (single-precision)"))
  (if (`|EnumEquality` Move "AltStab")
    (bind _output_get (set `self.SpearHeadShoot` (+ (`self.SpearHeadShoot`) 1)))
    (if (not (>= _output_get 2))
      (`KismetSystemLibrary.Delay` 0.5)
      (bind _returnvalue (`|SpawnActorFromClass` "/coatofarms/Assets/coat/ShopItems/Weapons/BP_SpearHeadProjectile.BP_SpearHeadProjectile_C" (`SceneComponent.K2_GetComponentToWorld` (`self.w`)) "Undefined" "OverrideRootScale" null null))
      (`MordhauProjectile.Fire` _returnvalue)
      (`SceneComponent.SetVisibility` (`self.SK_shortSpear_head_03`) false false))))

(fn `UserConstructionScript`
  (`parent.UserConstructionScript`))