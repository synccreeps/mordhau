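; BP_StaffForce is a staff weapon that fires projectiles when its owner's attack moves start.
; OnAttackStarted spawns and fires a projectile at the Scene component's transform: mortar for stabs, smoke bomb for right strikes, fire catapult for left strikes.
; Each shot increments HitLeft; from the eighth onward, CanAttack is disabled for a long delay.
; HitLeft is never reset here, so every later shot triggers that cooldown again.
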(event `self.ReceiveBeginPlay`
  (`parent.ReceiveBeginPlay`))

(event `self.OnAttackStarted`
  (params (Move :type "EAttackMove Enum" :default "RightStrike") (Angle :type "Float (single-precision)"))
  (if (or (`|EnumEquality` Move "AltStab") (`|EnumEquality` Move "Stab"))
    (bind _returnvalue (`|SpawnActorFromClass` "/Game/Mordhau/Blueprints/Interactables/SiegeEngines/BP_MortarProjectile.BP_MortarProjectile_C" (`SceneComponent.K2_GetComponentToWorld` (`self.Scene`)) "Undefined" "OverrideRootScale" null null))
    (`MordhauProjectile.Fire` _returnvalue)
    (bind _output_get (set `self.HitLeft` (+ (`self.HitLeft`) 1) :!label _label))
    (if (>= _output_get 8)
      (set `self.bCanAttack` false)
      (`KismetSystemLibrary.Delay` 200.0)
      (set `self.bCanAttack` true))
    (elif (`|EnumEquality` Move "RightStrike")
      (bind _returnvalue_2 (`|SpawnActorFromClass` "/Game/Mordhau/Blueprints/Equipment/Thrown/BP_SmokeBombProjectile.BP_SmokeBombProjectile_C" (`SceneComponent.K2_GetComponentToWorld` (`self.Scene`)) "Undefined" "OverrideRootScale" null null))
      (`MordhauProjectile.Fire` _returnvalue_2)
      (goto _label)
      (elif (`|EnumEquality` Move "LeftStrike")
        (bind _returnvalue_3 (`|SpawnActorFromClass` "/Game/Mordhau/Blueprints/Interactables/SiegeEngines/BP_CatapultProjectileFire.BP_CatapultProjectileFire_C" (`SceneComponent.K2_GetComponentToWorld` (`self.Scene`)) "Undefined" "OverrideRootScale" null null))
        (`MordhauProjectile.Fire` _returnvalue_3)
        (goto _label)))))

(fn `UserConstructionScript`
  (`parent.UserConstructionScript`))