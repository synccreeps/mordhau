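; BP_Arquebus is an arquebus weapon useable that adds a smoke puff to the projectile firing of its parent class.
; FireProjectile calls the parent implementation, then ServerSmokePuff, which relays to MultiSmokePuff, a server-to-multicast pattern judging by the names.
; MultiSmokePuff spawns the P_SmokePuff emitter at the Scene component's world transform.
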(event `self.FireProjectile`
  (params (Origin :type "Vector Structure (by ref)") (Orientation :type "Rotator Structure (by ref)") (OwningController :type "Controller Object Reference") (ExpectedDelay :type "Float (single-precision)"))
  (`parent.FireProjectile` Origin Orientation OwningController ExpectedDelay)
  (`self.ServerSmokePuff`))

(event `ServerSmokePuff`
  (`self.MultiSmokePuff`))

(event `MultiSmokePuff`
  (bind (_returnvalue_location _returnvalue_rotation _returnvalue_scale) (`KismetMathLibrary.BreakTransform` (`SceneComponent.K2_GetComponentToWorld` (`self.Scene`))))
  (`GameplayStatics.SpawnEmitterAtLocation` "/coatofarms/Assets/coat/ShopItems/Weapons/Mesh/P_SmokePuff.P_SmokePuff" _returnvalue_location _returnvalue_rotation _returnvalue_scale))

(fn `UserConstructionScript`
  (`parent.UserConstructionScript`))