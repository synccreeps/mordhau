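; Projectile Blueprint for a poison throwing knife that, despite its name, can set damaged targets burning.
; It extends the parent's damage event, running the parent logic first, then acting only on the server.
; When FireDamage is positive and the hit will not kill, it starts a brief burn on the target's BurnableComponent, if present, crediting the projectile's owning controller.
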(event `self.OnProjectileDamagedDamagable`
  (params (DamagableComp :type "DamageableComponent Object Reference") (bWillKill :type Boolean) (WorldLocation :type "Vector Structure (by ref)") (Bone :type Name))
  (bind _returnvalue (`self.GetComponentByClass` (`ActorComponent.GetOwner` DamagableComp) "/Script/Mordhau.BurnableComponent"))
  (`parent.OnProjectileDamagedDamagable` DamagableComp bWillKill WorldLocation Bone)
  (`/Engine/EditorBlueprintResources/ActorMacros.Switch Has Authority`
    (:`Authority`
      (if (and (> (`self.FireDamage`) 0.0) (not bWillKill) (`KismetSystemLibrary.IsValid` _returnvalue))
        (bind _returnvalue_2 (`self.GetProjectileOwningController`))
        (`BurnableComponent.StartBurning` _returnvalue 1.0 10.0 0.5 null _returnvalue_2)))))

(fn `UserConstructionScript`
  (`parent.UserConstructionScript`))