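; BP_WarHorn is a single-use war horn equipment item that sounds a loud horn and is then consumed.
; Its PlayTone event spawns the WarHorn sound attached to the root, using loud attenuation and music concurrency.
; It then casts the parent character to MC_coatofarms, has it drop the horn without forcing, and destroys the dropped actor.
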(event `/Game/Mordhau/Blueprints/Equipment/Weapons/Specific/Instruments/BP_Instrument.PlayTone`
  (params (Tone :type Byte))
  (`GameplayStatics.SpawnSoundAttached` "/coatofarms/Assets/coat/Audio/WarHorn.WarHorn" (`self.RootComponent`) "None" (0.0 0.0 0.0) (struct) "KeepRelativeOffset" false 1.0 1.0 0.0 "/Game/Mordhau/Audio/Attenuation/General/LoudAttenuation.LoudAttenuation" "/Game/Mordhau/Audio/Other/Concurrency/MusicConcurrency.MusicConcurrency")
  (bind _asmc_coatofarms (cast `/coatofarms/Assets/MC_coatofarms` (`self.GetParentCharacter`)))
  (bind _returnvalue (`MordhauCharacter.DropEquipment` _asmc_coatofarms self false))
  (`self.K2_DestroyActor` _returnvalue))

(fn `UserConstructionScript`
  (`parent.UserConstructionScript`))