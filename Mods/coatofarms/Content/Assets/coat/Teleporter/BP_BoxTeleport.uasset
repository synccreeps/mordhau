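; BP_BoxTeleport is an interactable teleporter that moves the MC_coatofarms character to a destination.
; On InteractionStart it casts the interacting character to MC_coatofarms and teleports it to the DestLocation variable with zero rotation, ignoring any other character type.
; It has no other active logic, as BeginPlay, overlap and Tick are disabled and the construction script only calls its parent.
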(event `self.InteractionStart`
  (params (Character :type "MordhauCharacter Object Reference"))
  (bind _asmc_coatofarms (cast `/coatofarms/Assets/MC_coatofarms` Character))
  (`self.K2_TeleportTo` :`self` _asmc_coatofarms :`DestLocation` (`self.Dest Location`)))

(fn `UserConstructionScript`
  (`parent.UserConstructionScript`))