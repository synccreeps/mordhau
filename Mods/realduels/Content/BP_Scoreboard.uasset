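; BP_Scoreboard is an in-world scoreboard that shows player display names and win counts for the DeathmatchDuels game mode.
; UpdateScoreboard walks the game mode's SortedKeys up to PlayerMaxScoreboard, looking up each entry in its Scoreboard map.
; The first seven entries build one string and the rest a second, which is not cleared between updates.
; SetScoreboardTextMulti pushes both strings to two TextRender components.
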(event `UpdateScoreboard`
  (bind _scoretext (`self.ScoreText`))
  (bind _scoretext2 (`self.ScoreText2`))
  (set `self.ScoreText` "")
  (bind _asdeathmatch_duels (cast `/realduels/DeathmatchDuels` (`GameplayStatics.GetGameMode`)))
  (for (_array_element _array_index) (`/realduels/DeathmatchDuels.SortedKeys` _asdeathmatch_duels)
    (if (< _array_index (`self.PlayerMaxScoreboard`))
      (if (< _array_index 7)
        (bind (_wins _displayname) (break `/realduels/Scoreboard` (`BlueprintMapLibrary.Map_Find` (`/realduels/DeathmatchDuels.Scoreboard` _asdeathmatch_duels) _array_element)))
        (bind _returnvalue (`KismetStringLibrary.Conv_IntToString` _wins))
        (set `self.ScoreText` (`KismetStringLibrary.Concat_StrStr` _scoretext " \n" _displayname ": " _returnvalue))
        (else
          (set `self.ScoreText2` (`KismetStringLibrary.Concat_StrStr` _scoretext2 " \n" _displayname ": " _returnvalue))))
      (else
        (break))))
  (`self.SetScoreboardTextMulti` (`KismetTextLibrary.Conv_StringToText` _scoretext) (`KismetTextLibrary.Conv_StringToText` _scoretext2)))

(event `SetScoreboardTextMulti`
  (params (Value :type Text) (Value2 :type Text))
  (`TextRenderComponent.K2_SetText` (`self.TextRender`) Value)
  (`TextRenderComponent.K2_SetText` (`self.TextRender1`) Value2))

(fn `UserConstructionScript`)